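; Projectile arrow from the Vive game that can catch fire from a Brazier and damages siege units and AI troops.
; While in flight it rotates its mesh along projectile velocity until movement stops.
; A burning arrow ignites battering rams and catapults, then destroys itself after a delay.
; Hits remove light soldiers and archers from the Overlord's unit array and destroy them, while other soldiers and landscape only trigger impact sounds.
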(event Custom|RotateToVelocity
  (bind _projectilemovement (Variables|Default|GetProjectileMovement))
  (bind _scene (Variables|Default|GetScene))
  (bind _returnvalue (Transformation|GetWorldLocation _scene))
  (bind _velocity (Variables|/Script/Engine.MovementComponent|GetVelocity _projectilemovement))
  (bind _returnvalue_2 (+ _returnvalue _velocity))
  (bind _returnvalue_3 (Math|Rotator|FindLookatRotation _returnvalue _returnvalue_2))
  (bind (_roll _pitch _yaw) (Math|Rotator|BreakRotator _returnvalue_3))
  (Transformation|SetWorldRotation (Variables|Default|GetStaticMesh) (Math|Rotator|MakeRotator _roll (+ _pitch 9e+01) _yaw) false false))

(event Collision|EventHit
  (params (MyComp :type Primitive%20Component%20Object%20Reference) (Other :type Actor%20Object%20Reference) (OtherComp :type Primitive%20Component%20Object%20Reference) (bSelfMoved :type Boolean) (HitLocation :type Vector) (HitNormal :type Vector :default "0, 0, 0") (NormalImpulse :type Vector :default "0, 0, 0") (Hit :type Hit%20Result%20Structure%20%28by%20ref%29))
  (Variables|Default|SetArrowHitLocation HitLocation)
  (bind _asbp_battering_ram_old (Utilities|Casting|CastToBP_BatteringRamOld Other)
    (:then
      (if (Variables|Default|GetOnFire)
        (Variables|/Game/Vive/Blueprints/AI/SiegeAI/BP_BatteringRamOld.BP_BatteringRamOld_C|SetIsOnFire _asbp_battering_ram_old true)
        (Utilities|FlowControl|Delay 2.0)
        (Audio|PlaySoundatLocation 0 (Variables|Default|GetArrowHitLocation))
        (Actor|DestroyActor)))
    (:CastFailed
      (bind _asbp_catapult (Utilities|Casting|CastToBP_Catapult Other)
        (:then
          (if (Variables|Default|GetOnFire)
            (Variables|/Game/Vive/Blueprints/AI/SiegeAI/BP_Catapult.BP_Catapult_C|SetIsOnFire _asbp_catapult true)
            (Utilities|FlowControl|Delay 2.0)
            (Actor|DestroyActor)))
        (:CastFailed
          (bind _asbp_light_soldier_ai (Utilities|Casting|CastToBP_LightSoldierAI Other)
            (:then
              (bind _outactors (Actor|GetAllActorsOfClass "/Game/Vive/Blueprints/Overlords/BP_Overlord_Master.BP_Overlord_Master_C"))
              (Utilities|Array|RemoveItem (Variables|/Game/Vive/Blueprints/Overlords/BP_Overlord_Master.BP_Overlord_Master_C|GetUnitArray (Utilities|Array|Get(acopy) _outactors)) _asbp_light_soldier_ai)
              (Audio|PlaySoundatLocation 0 (Variables|Default|GetArrowHitLocation))
              (Actor|DestroyActor _asbp_light_soldier_ai)
              (Actor|DestroyActor))
            (:CastFailed
              (bind _asbp_archer_ai (Utilities|Casting|CastToBP_ArcherAi Other)
                (:then
                  (bind _outactors_2 (Actor|GetAllActorsOfClass "/Game/Vive/Blueprints/Overlords/BP_Overlord_Master.BP_Overlord_Master_C"))
                  (Utilities|Array|RemoveItem (Variables|/Game/Vive/Blueprints/Overlords/BP_Overlord_Master.BP_Overlord_Master_C|GetUnitArray (Utilities|Array|Get(acopy) _outactors_2)) _asbp_archer_ai)
                  (Audio|PlaySoundatLocation 0 (Variables|Default|GetArrowHitLocation))
                  (Actor|DestroyActor _asbp_archer_ai)
                  (Actor|DestroyActor))
                (:CastFailed
                  (Utilities|Casting|CastToBP_SoldierAI Other
                    (:then
                      (Audio|PlaySoundatLocation 0 (Variables|Default|GetArrowHitLocation)))
                    (:CastFailed
                      (Utilities|Casting|CastToLandscape Other)
                      (Audio|PlaySoundatLocation 0 (Variables|Default|GetArrowHitLocation)))))))))))))

(event EventActorBeginOverlap
  (params (OtherActor :type Actor%20Object%20Reference))
  (bind _asbrazier (Utilities|Casting|CastToBrazier OtherActor))
  (if (Class|PrimitiveComponent|IsOverlappingComponent (Variables|/Game/Vive/Blueprints/Brazier.Brazier_C|GetFireCollision _asbrazier) (Variables|Default|GetStaticMesh))
    (Variables|Default|SetOnFire true)))

(event EventTick
  (params (DeltaSeconds :type Float%20%28single-precision%29))
  (Transformation|SetWorldRotation (Variables|Default|GetScene1) "0,0.000000, 0" false false)
  (if (Variables|Default|GetInFlight)
    (Variables|Default|SetInFlight (Math|Vector|NotEqual(Vector) (Variables|/Script/Engine.MovementComponent|GetVelocity (Variables|Default|GetProjectileMovement)) "0, 0, 0" 0.0001))
    (CallFunction|RotatetoVelocity)))

(event EventBeginPlay
  (Components|Movement|SetUpdatedComponent (Variables|Default|GetProjectileMovement) (Variables|Default|GetStaticMesh))
  (Variables|Default|SetInFlight false)
  (Variables|Default|SetHit false)
  (Variables|Default|SetSocketFlame "Flame")
  (Variables|Default|SetSocketTrail "Trail"))

(fn ConstructionScript)

(fn PrinttoVive
  (params (String%20In :type String))
  (Development|PrintString String%20In)
  (Development|PrintString String%20In)
  (Development|PrintString String%20In)
  (Development|PrintString String%20In)
  (Development|PrintString String%20In)
  (Development|PrintString String%20In)
  (Development|PrintString String%20In)
  (Development|PrintString String%20In)
  (Development|PrintString String%20In)
  (Development|PrintString String%20In)
  (Development|PrintString String%20In)
  (Development|PrintString String%20In)
  (Development|PrintString String%20In)
  (Development|PrintString String%20In)
  (Development|PrintString String%20In)
  (Development|PrintString String%20In))