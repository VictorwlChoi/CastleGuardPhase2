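; BP_CatapultRock is a short-lived catapult rock projectile that launches toward a test door.
; Its construction script finds the first SM_TestDoor_Blueprint actor, rotates to face that door's CurrentLocation and sets a high ProjectileMovement initial speed.
; A SetTransform function applies a supplied spawner transform.
; The rock destroys itself a few seconds after BeginPlay, with no hit handling in its graphs.
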(event EventBeginPlay
  (Utilities|FlowControl|Delay 3.0)
  (Actor|DestroyActor))

(fn ConstructionScript
  (bind _outactors (Actor|GetAllActorsOfClass "/Game/Vive/Blueprints/SM_TestDoor_Blueprint.SM_TestDoor_Blueprint_C"))
  (Transformation|SetActorRotation (Math|Rotator|FindLookatRotation (Transformation|GetWorldLocation (Variables|Default|GetSphere)) (Variables|/Game/Vive/Blueprints/SM_TestDoor_Blueprint.SM_TestDoor_Blueprint_C|GetCurrentLocation (Utilities|Array|Get(acopy) _outactors))))
  (Variables|/Script/Engine.ProjectileMovementComponent|SetInitialSpeed (Variables|Default|GetProjectileMovement) 5e+03))

(fn SetTransform
  (params (SpawnerTransform :type Transform))
  (Transformation|SetActorTransform SpawnerTransform))