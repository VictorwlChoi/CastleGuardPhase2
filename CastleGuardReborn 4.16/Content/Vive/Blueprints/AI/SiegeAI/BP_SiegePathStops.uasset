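; BP_SiegePathStops is a waypoint actor that relays AI catapults and battering rams along a chain of siege path stations.
; When a BP_Catapult or BP_BatteringRamOld enters OverlapCheck, it issues an AI move to NextStation and records that station as the vehicle's FirstPos.
; Separate end flags, CatapultLastStop and LastStation, halt each vehicle type.
; BeginPlay fills RotationToNextStop from NextStation's raw location X and Y, not a look-at rotation.
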(event OnComponentBeginOverlap(OverlapCheck)
  (params (OverlappedComponent :type Primitive%20Component%20Object%20Reference) (OtherActor :type Actor%20Object%20Reference) (OtherComp :type Primitive%20Component%20Object%20Reference) (OtherBodyIndex :type Integer) (bFromSweep :type Boolean) (SweepResult :type Hit%20Result%20Structure%20%28by%20ref%29))
  (bind _nextstation (Variables|Default|GetNextStation))
  (bind _nextstation_2 (Variables|Default|GetNextStation))
  (bind _asbp_catapult (Utilities|Casting|CastToBP_Catapult OtherActor)
    (:then
      (if (not (Variables|Default|GetCatapultLastStop))
        (AI|AIMoveTo _asbp_catapult "0, 0, 0" _nextstation_2 0.0 false
          (:then
            (Variables|/Game/Vive/Blueprints/AI/SiegeAI/BP_Catapult.BP_Catapult_C|SetFirstPos _asbp_catapult _nextstation_2)))))
    (:CastFailed
      (bind _asbp_battering_ram_old (Utilities|Casting|CastToBP_BatteringRamOld OtherActor))
      (if (not (Variables|Default|GetLastStation?))
        (AI|AIMoveTo _asbp_battering_ram_old "0, 0, 0" _nextstation 5.0 false
          (:then
            (Variables|/Game/Vive/Blueprints/AI/SiegeAI/BP_BatteringRamOld.BP_BatteringRamOld_C|SetFirstPos _asbp_battering_ram_old _nextstation)))))))

(event EventBeginPlay
  (bind _nextstation (Variables|Default|GetNextStation))
  (bind _returnvalue (Transformation|GetActorTransform _nextstation))
  (bind _location (Math|Transform|BreakTransform _returnvalue))
  (bind (_x _y) (Math|Vector|BreakVector _location))
  (if (Utilities|IsValid (Variables|Default|GetNextStation))
    (Variables|Default|SetRotationToNextStop (Math|Rotator|MakeRotator _x _y 0.0))))

(fn ConstructionScript)