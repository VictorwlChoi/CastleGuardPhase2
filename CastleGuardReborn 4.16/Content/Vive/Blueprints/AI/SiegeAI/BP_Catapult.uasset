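; AI siege catapult that soldiers crew and push to an attack position, where it stops and switches their animations.
; Overlapping soldiers snap onto two handle sockets; crew count sets speed along waypoints, skipping taken final positions.
; Tick aligns it to the traced ground, turns the health bar to the headset and applies burn damage from flaming arrows.
; At zero health it removes itself and crew from the Overlord's units; destruction frees its position.
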(event OnComponentBeginOverlap(SoldierOverlapCheck)
  (params (OverlappedComponent :type Primitive%20Component%20Object%20Reference) (OtherActor :type Actor%20Object%20Reference) (OtherComp :type Primitive%20Component%20Object%20Reference) (OtherBodyIndex :type Integer) (bFromSweep :type Boolean) (SweepResult :type Hit%20Result%20Structure%20%28by%20ref%29))
  ;[1 1 1] Checking for someone manning Catapult & Attach Soldier if there isn't
  (if (Variables|Default|GetIsActive)
    (bind _asbp_soldier_ai (Utilities|Casting|CastToBP_SoldierAI OtherActor))
    (Variables|/Game/Vive/Blueprints/AI/SoldierAI/BP_SoldierAI.BP_SoldierAI_C|SetCatapult _asbp_soldier_ai (Variables|Default|GetNextCatapult))
    (if (not (Variables|Default|GetHandleBool2))
      (if (Variables|Default|GetHandleBool1)
        (if (!= OtherActor (Variables|Default|GetSoldier1))
          (bind _asbp_soldier_ai_2 (Utilities|Casting|CastToBP_SoldierAI OtherActor))
          (Collision|SetCollisionEnabled (Variables|/Script/Engine.Character|GetMesh _asbp_soldier_ai_2) "NoCollision")
          (Variables|Default|SetHandleBool2 true)
          (Transformation|AttachComponentToComponent OtherActor (Variables|Character|GetMesh) (Utilities|String|StringToName (Variables|Default|GetHandleString2)) "SnapToTarget" "KeepWorld" "KeepWorld" false)
          (Variables|Default|SetIsFull? true)
          (Collision|SetActorEnableCollision OtherActor false)
          (bind _asbp_soldier_ai_3 (Utilities|Casting|CastToBP_SoldierAI OtherActor))
          (Variables|Default|SetSoldier2 _asbp_soldier_ai_3)
          (bind _asabp_soldier_unit (Utilities|Casting|CastToABP_SoldierUnit (Components|SkeletalMesh|GetAnimInstance (Variables|/Script/Engine.Character|GetMesh _asbp_soldier_ai_3))))
          (Variables|/Game/Vive/Blueprints/AI/SoldierAI/ABP_SoldierUnit.ABP_SoldierUnit_C|SetSiegeHandle _asabp_soldier_unit (Utilities|String|StringToName (Variables|Default|GetHandleString2))))
        (else
          (bind _asbp_soldier_ai_4 (Utilities|Casting|CastToBP_SoldierAI OtherActor))
          (Collision|SetCollisionEnabled (Variables|/Script/Engine.Character|GetMesh _asbp_soldier_ai_4) "NoCollision")
          (Variables|Default|SetHandleBool1 true)
          (Transformation|AttachComponentToComponent OtherActor (Variables|Character|GetMesh) (Utilities|String|StringToName (Variables|Default|GetHandleString1)) "SnapToTarget" "KeepWorld" "KeepWorld" false)
          (Collision|SetActorEnableCollision OtherActor false)
          (bind _asbp_soldier_ai_5 (Utilities|Casting|CastToBP_SoldierAI OtherActor))
          (Variables|Default|SetSoldier1 _asbp_soldier_ai_5)
          (bind _asabp_soldier_unit_2 (Utilities|Casting|CastToABP_SoldierUnit (Components|SkeletalMesh|GetAnimInstance (Variables|/Script/Engine.Character|GetMesh _asbp_soldier_ai_5))))
          (Variables|/Game/Vive/Blueprints/AI/SoldierAI/ABP_SoldierUnit.ABP_SoldierUnit_C|SetSiegeHandle _asabp_soldier_unit_2 (Utilities|String|StringToName (Variables|Default|GetHandleString1))))))))

(event OnComponentHit(Mesh)
  (params (HitComponent :type Primitive%20Component%20Object%20Reference) (OtherActor :type Actor%20Object%20Reference) (OtherComp :type Primitive%20Component%20Object%20Reference) (NormalImpulse :type Vector :default "0, 0, 0") (Hit :type Hit%20Result%20Structure%20%28by%20ref%29))
  (if (Variables|Default|GetIsActive)
    (bind _asbp_heavy_arrow (Utilities|Casting|CastToBP_HeavyArrow OtherActor)
      (:then
        (if (Variables|/Game/Vive/Blueprints/BP_HeavyArrow.BP_HeavyArrow_C|GetOnFire _asbp_heavy_arrow)
          (Variables|Default|SetIsOnFire true)))
      (:CastFailed
        (bind _asbp_light_arrow (Utilities|Casting|CastToBP_LightArrow OtherActor))
        (if (Variables|/Game/Vive/Blueprints/BP_LightArrow.BP_LightArrow_C|GetOnFire _asbp_light_arrow)
          (Variables|Default|SetIsOnFire true))))))

(event OnComponentBeginOverlap(CapsuleComponent)
  (params (OverlappedComponent :type Primitive%20Component%20Object%20Reference) (OtherActor :type Actor%20Object%20Reference) (OtherComp :type Primitive%20Component%20Object%20Reference) (OtherBodyIndex :type Integer) (bFromSweep :type Boolean) (SweepResult :type Hit%20Result%20Structure%20%28by%20ref%29))
  ;[1 1 1] When Catapult Has Position Update Soldier Animation State Machines
  (if (Variables|Default|GetIsActive)
    (Utilities|Casting|CastToBP_CatapultAttackPositions OtherActor)
    (Variables|Default|SetHasPosition true)
    (bind _asabp_soldier_unit (Utilities|Casting|CastToABP_SoldierUnit (Components|SkeletalMesh|GetAnimInstance (Variables|/Script/Engine.Character|GetMesh (Variables|Default|GetSoldier1)))))
    (Variables|/Game/Vive/Blueprints/AI/SoldierAI/ABP_SoldierUnit.ABP_SoldierUnit_C|SetMountHandle _asabp_soldier_unit true)
    (bind _asabp_soldier_unit_2 (Utilities|Casting|CastToABP_SoldierUnit (Components|SkeletalMesh|GetAnimInstance (Variables|/Script/Engine.Character|GetMesh (Variables|Default|GetSoldier2)))))
    (Variables|/Game/Vive/Blueprints/AI/SoldierAI/ABP_SoldierUnit.ABP_SoldierUnit_C|SetMountHandle _asabp_soldier_unit_2 true)))

(event Custom|ResetSoldierRotations
  (if (Variables|Default|GetIsFull?)
    _))

(event Custom|Tick
  ;[1 1 1] Checking for someone manning Catapult & Attach Soldier if there isn't
  (if (Variables|Default|GetIsActive)
    (if (Variables|Default|GetHandleBool1)
      (if (Variables|Default|GetHandleBool2)
        (Variables|/Script/Engine.CharacterMovementComponent|SetMaxWalkSpeed (Variables|Character|GetCharacterMovement) 4e+02)
        (AI|AIMoveTo self "0, 0, 0" (Variables|Default|GetFirstPos) 5.0 false)
        (else
          (Variables|/Script/Engine.CharacterMovementComponent|SetMaxWalkSpeed (Variables|Character|GetCharacterMovement) 2e+02)
          (AI|AIMoveTo self "0, 0, 0" (Variables|Default|GetFirstPos) 5.0 false))))))

(event EventTick
  (params (DeltaSeconds :type Float%20%28single-precision%29))
  (bind _firstpos (Variables|Default|GetFirstPos))
  (bind _firstpos_2 (Variables|Default|GetFirstPos))
  (bind _capsulecomponent (Variables|Default|GetCapsuleComponent))
  (bind _capsulecomponent_2 (Variables|Default|GetCapsuleComponent))
  (bind _returnvalue (Transformation|GetWorldLocation _capsulecomponent))
  (bind _returnvalue_2 (Transformation|GetWorldLocation _capsulecomponent_2))
  (bind _returnvalue_3 (Transformation|GetActorTransform _firstpos_2))
  (bind _location (Math|Transform|BreakTransform _returnvalue_3))
  (bind _returnvalue_4 (Math|Rotator|FindLookatRotation _returnvalue _location))
  (bind (_roll _pitch _yaw) (Math|Rotator|BreakRotator _returnvalue_4))
  (if (Variables|Default|GetIsActive)
    (CallFunction|ResetSoldierRotations)
    (bind _outhit (Collision|LineTraceByChannel _returnvalue_2 (+ _returnvalue_2 "0, 0,-100.000000") "TraceTypeQuery1" true 0 "None"))
    (if (Variables|/Game/Vive/Blueprints/AI/SiegeAI/BP_SiegePathStops.BP_SiegePathStops_C|GetCatapultLastStop _firstpos)
      (if (Utilities|IsValid _firstpos)
        _
        (else
          _))
      (Transformation|SetActorRotation (Math|Rotator|MakeRotator (.Roll (Math|Rotator|BreakRotator (Math|Rotator|FindLookatRotation (Transformation|GetWorldLocation (Variables|Default|GetCapsuleComponent)) (.Location (Math|Transform|BreakTransform (Transformation|GetActorTransform (Variables|Default|GetFinalLocation))))))) (.Pitch (Math|Rotator|BreakRotator (Math|Rotator|MakeRotfromY (.Normal (Collision|BreakHitResult _outhit))))) (.Yaw (Math|Rotator|BreakRotator (Math|Rotator|FindLookatRotation (Transformation|GetWorldLocation (Variables|Default|GetCapsuleComponent)) (.Location (Math|Transform|BreakTransform (Transformation|GetActorTransform (Variables|Default|GetFinalLocation)))))))) true)
      (else
        (Transformation|SetActorRotation (Math|Rotator|MakeRotator _roll (.Pitch (Math|Rotator|BreakRotator (Math|Rotator|MakeRotfromY (.Normal (Collision|BreakHitResult _outhit))))) _yaw) true)))
    ;[1 1 1] UpdateHealth (Using Tick Event)
    (CallFunction|Tick)
    (if (<= (Variables|Default|GetHealth) 0.0)
      (bind _outactors (Actor|GetAllActorsOfClass "/Game/Vive/Blueprints/Overlords/BP_Overlord_Master.BP_Overlord_Master_C"))
      (Utilities|Array|RemoveItem (Variables|/Game/Vive/Blueprints/Overlords/BP_Overlord_Master.BP_Overlord_Master_C|GetUnitArray (Utilities|Array|Get(acopy) _outactors)) (Variables|Default|GetSoldier1))
      (Actor|DestroyActor (Variables|Default|GetSoldier1))
      (Utilities|Array|RemoveItem (Variables|/Game/Vive/Blueprints/Overlords/BP_Overlord_Master.BP_Overlord_Master_C|GetUnitArray (Utilities|Array|Get(acopy) _outactors)) (Variables|Default|GetSoldier2))
      (Actor|DestroyActor (Variables|Default|GetSoldier2))
      (Utilities|Array|RemoveItem (Variables|/Game/Vive/Blueprints/Overlords/BP_Overlord_Master.BP_Overlord_Master_C|GetUnitArray (Utilities|Array|Get(acopy) _outactors)) self)
      (Audio|PlaySoundatLocation 0 (Transformation|GetActorLocation))
      (Actor|DestroyActor)
      (else
        (bind _ascatapult_health_bar (Utilities|Casting|CastToCatapultHealthBar (UserInterface|GetUserWidgetObject (Variables|Default|GetCatapultHealthBarComponent))))
        (Transformation|SetWorldRotation (Variables|Default|GetCatapultHealthBarComponent) (Math|Rotator|FindLookatRotation (Transformation|GetWorldLocation (Variables|Default|GetCatapultHealthBarComponent)) (.DevicePosition (Class|HeadMountedDisplayFunctionLibrary|GetOrientationandPosition))) false false)
        (Progress|SetPercent (Variables|/Game/Vive/Blueprints/WidgetUI/CatapultHealthBar.CatapultHealthBar_C|GetProgressBar_143 _ascatapult_health_bar) (/ (Variables|Default|GetHealth) 1e+02))
        (if (Variables|Default|GetIsOnFire)
          (Variables|Default|SetHealth (- (Variables|Default|GetHealth) 0.1))
          (|SetFlamesToVisible))
        ;[1 1 1] Moving AI
        (if (Variables|Default|GetIsFull?)
          (if (Variables|Default|GetHasPosition)
            (Variables|/Script/Engine.CharacterMovementComponent|SetMaxWalkSpeed (Variables|Character|GetCharacterMovement) 0.0)
            (elif (Variables|/Game/Vive/Blueprints/AI/SiegeAI/BP_SiegePathStops.BP_SiegePathStops_C|GetCatapultLastStop (Variables|Default|GetFirstPos))
              (if (Variables|/Game/Vive/Blueprints/AI/SiegeAI/BP_CatapultAttackPositions.BP_CatapultAttackPositions_C|GetPositionTaken (Variables|Default|GetFinalLocation))
                (AI|AIMoveTo self "0, 0, 0" (Variables|/Game/Vive/Blueprints/AI/SiegeAI/BP_CatapultAttackPositions.BP_CatapultAttackPositions_C|GetNextPosition (Variables|Default|GetFinalLocation)) 5.0 true
                  (:then
                    (Variables|Default|SetFinalLocation (Variables|/Game/Vive/Blueprints/AI/SiegeAI/BP_CatapultAttackPositions.BP_CatapultAttackPositions_C|GetNextPosition (Variables|Default|GetFinalLocation)))))
                (else
                  (AI|AIMoveTo self "0, 0, 0" (Variables|Default|GetFinalLocation) 5.0 true))))))))))

(event EventDestroyed
  ;[1 1 1] When Catapult Has Position Update Soldier Animation State Machines
  (if (Variables|Default|GetIsActive)
    (if (Variables|Default|GetHasPosition)
      (Variables|/Game/Vive/Blueprints/AI/SiegeAI/BP_CatapultAttackPositions.BP_CatapultAttackPositions_C|SetPositionTaken (Variables|Default|GetFinalLocation) false)
      (Variables|/Game/Vive/Blueprints/AI/SiegeAI/BP_CatapultAttackPositions.BP_CatapultAttackPositions_C|SetTimer (Variables|Default|GetFinalLocation) 0.0))))

(fn ConstructionScript
  (Variables|Default|SetHandleBool1 false)
  (Variables|Default|SetHandleString1 "CatapultLeftHandle")
  (Variables|Default|SetHandleString2 "CatapultRightHandle")
  (Variables|Default|SetHandleBool2 false))

(fn ReturnCatapultBools
  (return (Variables|Default|GetHasPosition) (Variables|Default|GetHandleBool1) (Variables|Default|GetHandleBool2)))

(fn PrinttoVive
  (params (String%20In :type String))
  (Development|PrintString String%20In)
  (Development|PrintString String%20In)
  (Development|PrintString String%20In)
  (Development|PrintString String%20In)
  (Development|PrintString String%20In)
  (Development|PrintString String%20In)
  (Development|PrintString String%20In)
  (Development|PrintString String%20In)
  (Development|PrintString String%20In)
  (Development|PrintString String%20In)
  (Development|PrintString String%20In)
  (Development|PrintString String%20In)
  (Development|PrintString String%20In)
  (Development|PrintString String%20In)
  (Development|PrintString String%20In)
  (Development|PrintString String%20In))

(fn CatapultChainAudio
  (params (CatapultPositionIn :type Vector))
  (bind _returnvalue (Math|Random|RandomInteger 0))
  (if (== _returnvalue 0)
    (Audio|SpawnSoundAttached 0 (Variables|Default|GetChainAudio1) "None" CatapultPositionIn)
    (elif (== _returnvalue 0)
      _)))