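; Arrow projectile for the archer AI that flies at the Vive VR player and damages them.
; The construction script rotates it toward a point just above the player collision capsule's center and sets a fast projectile speed.
; Both actor and arrow component overlaps with the player subtract the pawn's HealthDamageRecovery from its Health and destroy the arrow.
; It also destroys itself on a castle actor overlap or ten seconds after spawning.
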(event OnComponentBeginOverlap(Arrow)
  (params (OverlappedComponent :type Primitive%20Component%20Object%20Reference) (OtherActor :type Actor%20Object%20Reference) (OtherComp :type Primitive%20Component%20Object%20Reference) (OtherBodyIndex :type Integer) (bFromSweep :type Boolean) (SweepResult :type Hit%20Result%20Structure%20%28by%20ref%29))
  (Variables|Default|SetHitLocation (|BreakHitCollapse SweepResult))
  (Utilities|Casting|CastToBP_PlayerCollision OtherActor
    (:then
      (bind _outactors (Actor|GetAllActorsOfClass "/Game/Vive/Blueprints/BP_Vive_Pawn.BP_Vive_Pawn_C"))
      (Variables|/Game/Vive/Blueprints/BP_Vive_Pawn.BP_Vive_Pawn_C|SetHealth (Utilities|Array|Get(acopy) _outactors) (- (Variables|/Game/Vive/Blueprints/BP_Vive_Pawn.BP_Vive_Pawn_C|GetHealth (Utilities|Array|Get(acopy) _outactors)) (Variables|/Game/Vive/Blueprints/BP_Vive_Pawn.BP_Vive_Pawn_C|GetHealthDamage/Recovery (Utilities|Array|Get(acopy) _outactors))))
      (Actor|DestroyActor))
    (:CastFailed
      (Utilities|Casting|CastToBP_Castle OtherActor))))

(event EventTick
  (params (DeltaSeconds :type Float%20%28single-precision%29)))

(event Collision|EventActorBeginOverlap
  (params (OtherActor :type Actor%20Object%20Reference))
  (Utilities|Casting|CastToBP_PlayerCollision OtherActor
    (:then
      (Development|PrintString "Player Succesful")
      (bind _outactors (Actor|GetAllActorsOfClass "/Game/Vive/Blueprints/BP_Vive_Pawn.BP_Vive_Pawn_C"))
      (Variables|/Game/Vive/Blueprints/BP_Vive_Pawn.BP_Vive_Pawn_C|SetHealth (Utilities|Array|Get(acopy) _outactors) (- (Variables|/Game/Vive/Blueprints/BP_Vive_Pawn.BP_Vive_Pawn_C|GetHealth (Utilities|Array|Get(acopy) _outactors)) (Variables|/Game/Vive/Blueprints/BP_Vive_Pawn.BP_Vive_Pawn_C|GetHealthDamage/Recovery (Utilities|Array|Get(acopy) _outactors))))
      (Development|PrintString "Overlap Actor")
      (Actor|DestroyActor :!label _label))
    (:CastFailed
      (Utilities|Casting|CastToBP_Castle OtherActor
        (:then
          (Development|PrintString "Castle Succesful")
          (goto _label))
        (:CastFailed
          (Development|PrintString "Cast Failed"))))))

(event EventBeginPlay
  (Utilities|FlowControl|Delay 1e+01)
  (Actor|DestroyActor))

(fn ConstructionScript
  (bind _outactors (Actor|GetAllActorsOfClass "/Game/Vive/Blueprints/BP_PlayerCollision.BP_PlayerCollision_C"))
  (Transformation|SetActorRotation (Math|Rotator|FindLookatRotation (Transformation|GetWorldLocation (Variables|Default|GetArrow)) (+ (Transformation|GetWorldLocation (Variables|/Game/Vive/Blueprints/BP_PlayerCollision.BP_PlayerCollision_C|GetCapsule (Utilities|Array|Get(acopy) _outactors))) "0, 0,34.000000")))
  (Variables|/Script/Engine.ProjectileMovementComponent|SetInitialSpeed (Variables|Default|GetProjectileMovement) 5e+03))