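; Archer AI character that walks to an attack position and fires arrows at the player.
; While active and unpositioned, Tick moves it via FirstStop to AttackPosition, following NextPosition if taken, and destroys it after 30 accumulated seconds standing still.
; EventShootArrow spawns BP_AI_Arrows aimed at the BP_PlayerCollision capsule.
; A light or heavy arrow hit removes it from BP_Overlord_Master's UnitArray, destroys both and plays a collapse sound.
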(event Custom|EventShootArrow
  (bind _outactors (Actor|GetAllActorsOfClass "/Game/Vive/Blueprints/BP_PlayerCollision.BP_PlayerCollision_C"))
  (Game|SpawnActorfromClass "/Game/Vive/Blueprints/AI/ArcherAI/BP_AI_Arrows.BP_AI_Arrows_C" (Math|Transform|MakeTransform (Transformation|GetWorldLocation (Variables|Default|GetScene)) (Math|Rotator|MakeRotator (+ (.Roll (Math|Rotator|BreakRotator (Math|Rotator|FindLookatRotation (Transformation|GetWorldLocation (Variables|Default|GetScene)) (Transformation|GetWorldLocation (Variables|/Game/Vive/Blueprints/BP_PlayerCollision.BP_PlayerCollision_C|GetCapsule (Utilities|Array|Get(acopy) _outactors)))))) 9e+01) (.Pitch (Math|Rotator|BreakRotator (Math|Rotator|FindLookatRotation (Transformation|GetWorldLocation (Variables|Default|GetScene)) (Transformation|GetWorldLocation (Variables|/Game/Vive/Blueprints/BP_PlayerCollision.BP_PlayerCollision_C|GetCapsule (Utilities|Array|Get(acopy) _outactors)))))) (.Yaw (Math|Rotator|BreakRotator (Math|Rotator|FindLookatRotation (Transformation|GetWorldLocation (Variables|Default|GetScene)) (Transformation|GetWorldLocation (Variables|/Game/Vive/Blueprints/BP_PlayerCollision.BP_PlayerCollision_C|GetCapsule (Utilities|Array|Get(acopy) _outactors)))))))) "AlwaysSpawn" 0 0))

(event Collision|EventHit
  (params (MyComp :type Primitive%20Component%20Object%20Reference) (Other :type Actor%20Object%20Reference) (OtherComp :type Primitive%20Component%20Object%20Reference) (bSelfMoved :type Boolean) (HitLocation :type Vector :default "0, 0, 0") (HitNormal :type Vector :default "0, 0, 0") (NormalImpulse :type Vector :default "0, 0, 0") (Hit :type Hit%20Result%20Structure%20%28by%20ref%29))
  (bind _asbp_light_arrow (Utilities|Casting|CastToBP_LightArrow Other)
    (:then
      (bind _outactors (Actor|GetAllActorsOfClass "/Game/Vive/Blueprints/Overlords/BP_Overlord_Master.BP_Overlord_Master_C"))
      (Utilities|Array|RemoveItem (Variables|/Game/Vive/Blueprints/Overlords/BP_Overlord_Master.BP_Overlord_Master_C|GetUnitArray (Utilities|Array|Get(acopy) _outactors)) self)
      (Actor|DestroyActor _asbp_light_arrow)
      (Actor|DestroyActor))
    (:CastFailed
      (bind _asbp_heavy_arrow (Utilities|Casting|CastToBP_HeavyArrow Other))
      (bind _outactors_2 (Actor|GetAllActorsOfClass "/Game/Vive/Blueprints/Overlords/BP_Overlord_Master.BP_Overlord_Master_C"))
      (Utilities|Array|RemoveItem (Variables|/Game/Vive/Blueprints/Overlords/BP_Overlord_Master.BP_Overlord_Master_C|GetUnitArray (Utilities|Array|Get(acopy) _outactors_2)) self)
      (Actor|DestroyActor _asbp_heavy_arrow)
      (Actor|DestroyActor)))
  (Audio|PlaySound2D "/Game/StarterContent/Audio/Collapse_Cue.Collapse_Cue"))

(event EventTick
  (params (DeltaSeconds :type Float%20%28single-precision%29))
  (if (Variables|Default|GetIsActive)
    (bind _asabp_erika (Utilities|Casting|CastToABP_Erika (Components|SkeletalMesh|GetAnimInstance (Variables|Character|GetMesh)))
      (:then
        _)
      (:CastFailed
        _))
    (if (not (Variables|Default|GetHasPosition))
      (if (>= (Variables|Default|GetSuicideTimer) 3e+01)
        (Actor|DestroyActor)
        (else
          (if (== (Variables|/Game/Vive/Blueprints/AI/ArcherAI/ABP_Erika.ABP_Erika_C|GetSpeed _asabp_erika) 0.0)
            (Variables|Default|SetSuicideTimer (+ (Variables|Default|GetSuicideTimer) DeltaSeconds)))
          (if (Variables|Default|GetFirstStop?)
            (if (Variables|/Game/Vive/Blueprints/AI/ArcherAI/BP_ArcherPathStops.BP_ArcherPathStops_C|GetLastStation? (Variables|Default|GetFirstStop))
              (if (Variables|/Game/Vive/Blueprints/AI/ArcherAI/BP_ArcherAttackPosition.BP_ArcherAttackPosition_C|GetPositionTaken (Variables|Default|GetAttackPosition))
                (AI|AIMoveTo self "0, 0, 0" (Variables|/Game/Vive/Blueprints/AI/ArcherAI/BP_ArcherAttackPosition.BP_ArcherAttackPosition_C|GetNextPosition (Variables|Default|GetAttackPosition)) 5.0 true
                  (:then
                    (Variables|Default|SetAttackPosition (Variables|/Game/Vive/Blueprints/AI/ArcherAI/BP_ArcherAttackPosition.BP_ArcherAttackPosition_C|GetNextPosition (Variables|Default|GetAttackPosition)))))
                (else
                  (AI|AIMoveTo self "0, 0, 0" (Variables|Default|GetAttackPosition) 5.0 true))))
            (else
              (AI|AIMoveTo self "0, 0, 0" (Variables|Default|GetFirstStop) 5.0 false
                (:then
                  (Variables|Default|SetFirstStop? true))))))))))

(event Collision|EventActorBeginOverlap
  (params (OtherActor :type Actor%20Object%20Reference)))

(fn ConstructionScript)