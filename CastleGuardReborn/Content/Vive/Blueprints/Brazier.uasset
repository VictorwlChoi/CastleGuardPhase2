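; Brazier actor in the Vive game that ignites arrows passing through its fire and is destroyed when an arrow hits it.
; FireCollision overlap shows the Fire component on heavy or light arrows, setting OnFire true for heavy arrows but false for light ones.
; The Hit event destroys the brazier for either arrow type.
; A PrintToVive helper repeats PrintString many times for debug messages.
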(event OnComponentBeginOverlap(FireCollision)
  (params (OverlappedComponent :type Primitive%20Component%20Object%20Reference) (OtherActor :type Actor%20Object%20Reference) (OtherComp :type Primitive%20Component%20Object%20Reference) (OtherBodyIndex :type Integer) (bFromSweep :type Boolean) (SweepResult :type Hit%20Result%20Structure%20%28by%20ref%29))
  (bind _asbp_heavy_arrow (Utilities|Casting|CastToBP_HeavyArrow OtherActor)
    (:then
      (CallFunction|PrinttoVive "Heavy arrow on fire")
      (Variables|/Game/Vive/Blueprints/BP_HeavyArrow.BP_HeavyArrow_C|SetOnFire _asbp_heavy_arrow true)
      (Rendering|SetVisibility (Variables|/Game/Vive/Blueprints/BP_HeavyArrow.BP_HeavyArrow_C|GetFire _asbp_heavy_arrow) true false))
    (:CastFailed
      (bind _asbp_light_arrow (Utilities|Casting|CastToBP_LightArrow OtherActor))
      (CallFunction|PrinttoVive "Light arrow on fire")
      (Variables|/Game/Vive/Blueprints/BP_LightArrow.BP_LightArrow_C|SetOnFire _asbp_light_arrow false)
      (Rendering|SetVisibility (Variables|/Game/Vive/Blueprints/BP_LightArrow.BP_LightArrow_C|GetFire _asbp_light_arrow) true false))))

(event Collision|EventHit
  (params (MyComp :type Primitive%20Component%20Object%20Reference) (Other :type Actor%20Object%20Reference) (OtherComp :type Primitive%20Component%20Object%20Reference) (bSelfMoved :type Boolean) (HitLocation :type Vector :default "0, 0, 0") (HitNormal :type Vector :default "0, 0, 0") (NormalImpulse :type Vector :default "0, 0, 0") (Hit :type Hit%20Result%20Structure%20%28by%20ref%29))
  (Utilities|Casting|CastToBP_HeavyArrow Other
    (:then
      (CallFunction|PrinttoVive "Arrow Hits Brazier")
      (Actor|DestroyActor))
    (:CastFailed
      (Utilities|Casting|CastToBP_LightArrow Other)
      (CallFunction|PrinttoVive "Arrow hits Brazier")
      (Actor|DestroyActor))))

(fn ConstructionScript)

(fn PrinttoVive
  (params (String%20In :type String))
  (Development|PrintString String%20In)
  (Development|PrintString String%20In)
  (Development|PrintString String%20In)
  (Development|PrintString String%20In)
  (Development|PrintString String%20In)
  (Development|PrintString String%20In)
  (Development|PrintString String%20In)
  (Development|PrintString String%20In)
  (Development|PrintString String%20In)
  (Development|PrintString String%20In)
  (Development|PrintString String%20In)
  (Development|PrintString String%20In)
  (Development|PrintString String%20In)
  (Development|PrintString String%20In)
  (Development|PrintString String%20In)
  (Development|PrintString String%20In))