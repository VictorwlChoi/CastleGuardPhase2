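; PlayerCollision is an actor that follows the player's Vive headset, by its name serving as the player's collision body in VR.
; Every Tick it moves to the world location of the Vive headset scene component, offset slightly downward, without sweeping or teleporting.
; A PrintToVive helper repeats the same PrintString call many times for one input string.
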(event EventTick
  (params (DeltaSeconds :type Float%20%28single-precision%29))
  (Transformation|SetActorLocation (+ (Transformation|GetWorldLocation (Variables|/Game/Vive/Blueprints/Vive_Pawn.Vive_Pawn_C|GetHeadsetSceneActor (Variables|Default|GetVive))) "0, 0,-34.000000") false false))

(fn ConstructionScript)

(fn PrinttoVive
  (params (String%20In :type String))
  (Development|PrintString String%20In)
  (Development|PrintString String%20In)
  (Development|PrintString String%20In)
  (Development|PrintString String%20In)
  (Development|PrintString String%20In)
  (Development|PrintString String%20In)
  (Development|PrintString String%20In)
  (Development|PrintString String%20In)
  (Development|PrintString String%20In)
  (Development|PrintString String%20In)
  (Development|PrintString String%20In)
  (Development|PrintString String%20In)
  (Development|PrintString String%20In)
  (Development|PrintString String%20In)
  (Development|PrintString String%20In)
  (Development|PrintString String%20In))