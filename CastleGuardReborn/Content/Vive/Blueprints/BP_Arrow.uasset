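; BP_Arrow is an arrow projectile actor that uses a ProjectileMovement component to drive its static mesh.
; BeginPlay caches the Vive pawn, clears the flight and hit flags and sets flame and trail socket names.
; While InFlight, Tick prints velocity and clears the flag at zero velocity; Hit destroys the arrow when not in flight.
; Enemy-kill and trail-positioning logic is present but disconnected, and overlap does nothing.
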(event Collision|EventHit
  (params (MyComp :type Primitive%20Component%20Object%20Reference) (Other :type Actor%20Object%20Reference) (OtherComp :type Primitive%20Component%20Object%20Reference) (bSelfMoved :type Boolean) (HitLocation :type Vector) (HitNormal :type Vector :default "0, 0, 0") (NormalImpulse :type Vector :default "0, 0, 0") (Hit :type Hit%20Result%20Structure%20%28by%20ref%29))
  (if (not (Variables|Default|GetInFlight))
    (Actor|DestroyActor)))

(event EventActorBeginOverlap
  (params (OtherActor :type Actor%20Object%20Reference)))

(event EventTick
  (params (DeltaSeconds :type Float%20%28single-precision%29))
  (bind _projectilemovement (Variables|Default|GetProjectileMovement))
  (bind _velocity (Variables|/Script/Engine.MovementComponent|GetVelocity _projectilemovement))
  (if (Variables|Default|GetInFlight)
    (Development|PrintString (Utilities|String|ToString(Vector) _velocity))
    (Variables|Default|SetInFlight (Math|Vector|NotEqual(Vector) _velocity "0, 0, 0" 0.0001))))

(event EventBeginPlay
  (bind _asvive_pawn (Utilities|Casting|CastToVive_Pawn (Game|Player|GetPlayerPawn 0)))
  (Variables|Default|SetPlayerVariable _asvive_pawn)
  (Components|Movement|SetUpdatedComponent (Variables|Default|GetProjectileMovement) (Variables|Default|GetStaticMesh))
  (Variables|Default|SetInFlight false)
  (Variables|Default|SetHit false)
  (Variables|Default|SetSocketFlame "Flame")
  (Variables|Default|SetSocketTrail "Trail"))

(fn ConstructionScript)