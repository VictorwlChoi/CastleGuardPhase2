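; BP_MenuArcheryTarget is an archery target actor, named for menu use, that catches fire when shot with a burning arrow.
; Its Hit event casts the other actor to a heavy or light arrow and sets OnFire if that arrow is alight.
; While OnFire is set, Tick shows the Fire01 component and accumulates a timer, destroying the target after five seconds.
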(event OnComponentHit(StaticMeshComponent)
  (params (HitComponent :type Primitive%20Component%20Object%20Reference) (OtherActor :type Actor%20Object%20Reference) (OtherComp :type Primitive%20Component%20Object%20Reference) (NormalImpulse :type Vector :default "0, 0, 0") (Hit :type Hit%20Result%20Structure%20%28by%20ref%29)))

(event EventBeginPlay)

(event Collision|EventActorBeginOverlap
  (params (OtherActor :type Actor%20Object%20Reference)))

(event EventTick
  (params (DeltaSeconds :type Float%20%28single-precision%29))
  (if (Variables|Default|GetOnFire)
    (Rendering|SetVisibility (Variables|Default|GetFire01) true true)
    (bind _output_get (Variables|Default|SetFireTimer (+ DeltaSeconds (Variables|Default|GetFireTimer))))
    (if (>= _output_get 5.0)
      (Actor|DestroyActor))))

(event Collision|EventHit
  (params (MyComp :type Primitive%20Component%20Object%20Reference) (Other :type Actor%20Object%20Reference) (OtherComp :type Primitive%20Component%20Object%20Reference) (bSelfMoved :type Boolean) (HitLocation :type Vector :default "0, 0, 0") (HitNormal :type Vector :default "0, 0, 0") (NormalImpulse :type Vector :default "0, 0, 0") (Hit :type Hit%20Result%20Structure%20%28by%20ref%29))
  (bind _asbp_heavy_arrow (Utilities|Casting|CastToBP_HeavyArrow Other)
    (:then
      (if (Variables|/Game/Vive/Blueprints/BP_BaseArrow.BP_BaseArrow_C|GetOnFire _asbp_heavy_arrow)
        (Variables|Default|SetOnFire true)))
    (:CastFailed
      (bind _asbp_light_arrow (Utilities|Casting|CastToBP_LightArrow Other))
      (if (Variables|/Game/Vive/Blueprints/BP_BaseArrow.BP_BaseArrow_C|GetOnFire _asbp_light_arrow)
        (Variables|Default|SetOnFire true)))))

(fn ConstructionScript)