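; BP_HeavyArrowsPile is a VR world object, under the Vive content, representing a pile of heavy arrows with a quiver count.
; On BeginPlay and through an UpdateCountDisplay event, it writes QuiverCount into a CountDisplay text.
; A PrintToVive debug helper prints its input string many times, along with a hardcoded "Hello".
; The construction script is empty, and no pickup or count-changing logic appears in this Blueprint.
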(event Custom|UpdateCountDisplay
  (Rendering|Components|TextRender|SetText (Variables|Default|GetCountDisplay) (Utilities|Text|ToText(Integer) (Variables|Default|GetQuiverCount))))

(event EventBeginPlay
  (CallFunction|UpdateCountDisplay))

(fn ConstructionScript)

(fn PrinttoVive
  (params (String%20In :type String))
  (Development|PrintString String%20In)
  (Development|PrintString String%20In)
  (Development|PrintString String%20In)
  (Development|PrintString String%20In)
  (Development|PrintString String%20In)
  (Development|PrintString String%20In)
  (Development|PrintString String%20In)
  (Development|PrintString String%20In)
  (Development|PrintString String%20In)
  (Development|PrintString String%20In)
  (Development|PrintString String%20In)
  (Development|PrintString String%20In)
  (Development|PrintString String%20In)
  (Development|PrintString String%20In)
  (Development|PrintString "Hello")
  (Development|PrintString String%20In))