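; Battering ram AI pawn for a VR game that two soldiers carry along waypoints to an attack position.
; Overlapping soldiers snap to handle sockets; once full, the ram speeds up and seeks a free attack position at the last station, stopping there.
; Tick aligns it to the ground by line trace and updates a headset-facing health bar.
; Burning light arrows drain health; death removes ram and soldiers from the overlord's unit array.
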(event OnComponentBeginOverlap(SoldierOverlapCheck)
  (params (OverlappedComponent :type Primitive%20Component%20Object%20Reference) (OtherActor :type Actor%20Object%20Reference) (OtherComp :type Primitive%20Component%20Object%20Reference) (OtherBodyIndex :type Integer) (bFromSweep :type Boolean) (SweepResult :type Hit%20Result%20Structure%20%28by%20ref%29))
  (bind _handlestring2 (Variables|Default|GetHandleString2))
  (bind _handlestring1 (Variables|Default|GetHandleString1))
  ;[1 1 1] Soldiers attach themselves to Battering Ram
  (bind _asbp_soldier_ai (Utilities|Casting|CastToBP_SoldierAI OtherActor))
  (Variables|/Game/Vive/Blueprints/AI/SoldierAIHeavy/BP_SoldierAI.BP_SoldierAI_C|SetBatteringRam _asbp_soldier_ai (Variables|Default|GetNextRam))
  (if (not (Variables|Default|GetHandleBool2))
    (if (Variables|Default|GetHandleBool1)
      (Variables|Default|SetHandleBool2 true)
      (Development|PrintString _handlestring2)
      (Transformation|AttachComponentToComponent OtherActor (Variables|Default|GetStaticMesh) (Utilities|String|StringToName _handlestring2) "SnapToTarget" "SnapToTarget" "KeepWorld" false)
      (Variables|Default|SetIsFull? true)
      (Collision|SetActorEnableCollision OtherActor false)
      (bind _asbp_soldier_ai_2 (Utilities|Casting|CastToBP_SoldierAI OtherActor))
      (Variables|Default|SetSoldier2 _asbp_soldier_ai_2)
      (else
        (Variables|Default|SetHandleBool1 true)
        (Development|PrintString _handlestring1)
        (Transformation|AttachComponentToComponent OtherActor (Variables|Default|GetStaticMesh) (Utilities|String|StringToName _handlestring1) "SnapToTarget" "SnapToTarget" "KeepWorld" false)
        (Collision|SetActorEnableCollision OtherActor false)
        (bind _asbp_soldier_ai_3 (Utilities|Casting|CastToBP_SoldierAI OtherActor))
        (Variables|Default|SetSoldier1 _asbp_soldier_ai_3)))))

(event OnComponentHit(StaticMesh)
  (params (HitComponent :type Primitive%20Component%20Object%20Reference) (OtherActor :type Actor%20Object%20Reference) (OtherComp :type Primitive%20Component%20Object%20Reference) (NormalImpulse :type Vector :default "0, 0, 0") (Hit :type Hit%20Result%20Structure%20%28by%20ref%29))
  (bind _asbp_light_arrow (Utilities|Casting|CastToBP_LightArrow OtherActor))
  (if (Variables|/Game/Vive/Blueprints/BP_LightArrow.BP_LightArrow_C|GetOnFire _asbp_light_arrow)
    (Variables|Default|SetIsOnFire true)
    (CallFunction|PrinttoVive "adsafdsfdsfafasdfdsafdsafdsas")))

(event OnComponentBeginOverlap(CapsuleComponent)
  (params (OverlappedComponent :type Primitive%20Component%20Object%20Reference) (OtherActor :type Actor%20Object%20Reference) (OtherComp :type Primitive%20Component%20Object%20Reference) (OtherBodyIndex :type Integer) (bFromSweep :type Boolean) (SweepResult :type Hit%20Result%20Structure%20%28by%20ref%29))
  ;[1 1 1] Moving AI
  (Utilities|Casting|CastToBP_BatteringRamAttackPosition OtherActor)
  (Variables|Default|SetHasPosition true))

(event Custom|Tick
  ;[1 1 1] Soldiers attach themselves to Battering Ram
  (if (Variables|Default|GetHandleBool1)
    (if (Variables|Default|GetHandleBool2)
      (Variables|/Script/Engine.CharacterMovementComponent|SetMaxWalkSpeed (Variables|Character|GetCharacterMovement) 4e+02)
      (AI|AIMoveTo self "0, 0, 0" (Variables|Default|GetFirstPos) 5.0 false)
      (else
        (Variables|/Script/Engine.CharacterMovementComponent|SetMaxWalkSpeed (Variables|Character|GetCharacterMovement) 2e+02)
        (AI|AIMoveTo self "0, 0, 0" (Variables|Default|GetFirstPos) 5.0 false)))))

(event EventTick
  (params (DeltaSeconds :type Float%20%28single-precision%29))
  (bind _firstpos (Variables|Default|GetFirstPos))
  (bind _capsulecomponent (Variables|Collision|GetCapsuleComponent))
  (bind _firstpos_2 (Variables|Default|GetFirstPos))
  (bind _returnvalue (Transformation|GetActorTransform _firstpos_2))
  (bind _returnvalue_2 (Transformation|GetWorldLocation _capsulecomponent))
  (bind _location (Math|Transform|BreakTransform _returnvalue))
  (bind _returnvalue_3 (Math|Rotator|FindLookatRotation _returnvalue_2 _location))
  (bind (_roll _pitch _yaw) (Math|Rotator|BreakRotator _returnvalue_3))
  ;[1 1 1] Raycast to get correct rotation for actor
  (bind _outhit (Collision|LineTraceByChannel _returnvalue_2 (+ _returnvalue_2 "0, 0,-100.000000") "TraceTypeQuery1" true 0 "None"))
  (if (Utilities|IsValid _firstpos)
    (if (Variables|/Game/Vive/Blueprints/AI/BP_SiegePathStops.BP_SiegePathStops_C|GetLastStation? _firstpos)
      (Transformation|SetActorRotation (Math|Rotator|MakeRotator (.Roll (Math|Rotator|BreakRotator (Math|Rotator|FindLookatRotation _returnvalue_2 (.Location (Math|Transform|BreakTransform (Transformation|GetActorTransform (Variables|Default|GetAttackPos))))))) (.Pitch (Math|Rotator|BreakRotator (Math|Rotator|MakeRotfromY (.Normal (Collision|BreakHitResult _outhit))))) (.Yaw (Math|Rotator|BreakRotator (Math|Rotator|FindLookatRotation _returnvalue_2 (.Location (Math|Transform|BreakTransform (Transformation|GetActorTransform (Variables|Default|GetAttackPos)))))))) true)
      (else
        (Transformation|SetActorRotation (Math|Rotator|MakeRotator _roll (.Pitch (Math|Rotator|BreakRotator (Math|Rotator|MakeRotfromY (.Normal (Collision|BreakHitResult _outhit))))) _yaw) true)))
    ;[1 1 1] Health And Death
    (CallFunction|Tick)
    (if (<= (Variables|Default|GetHealth) 0.0)
      (bind _outactors (Actor|GetAllActorsOfClass "/Game/Vive/Blueprints/Overlords/BP_Overlord_Master.BP_Overlord_Master_C"))
      (Utilities|Array|RemoveItem (Variables|/Game/Vive/Blueprints/Overlords/BP_Overlord_Master.BP_Overlord_Master_C|GetUnitArray (Utilities|Array|Get(acopy) _outactors)) (Variables|Default|GetSoldier1))
      (Actor|DestroyActor (Variables|Default|GetSoldier1))
      (Utilities|Array|RemoveItem (Variables|/Game/Vive/Blueprints/Overlords/BP_Overlord_Master.BP_Overlord_Master_C|GetUnitArray (Utilities|Array|Get(acopy) _outactors)) (Variables|Default|GetSoldier2))
      (Actor|DestroyActor (Variables|Default|GetSoldier2))
      (Utilities|Array|RemoveItem (Variables|/Game/Vive/Blueprints/Overlords/BP_Overlord_Master.BP_Overlord_Master_C|GetUnitArray (Utilities|Array|Get(acopy) _outactors)) self)
      (Actor|DestroyActor)
      (else
        (bind _ascatapult_health_bar (Utilities|Casting|CastToCatapultHealthBar (UserInterface|GetUserWidgetObject (Variables|Default|GetRamHealthBarComponent))))
        (Transformation|SetWorldRotation (Variables|Default|GetRamHealthBarComponent) (Math|Rotator|FindLookatRotation (Transformation|GetWorldLocation (Variables|Default|GetRamHealthBarComponent)) (.DevicePosition (Class|HeadMountedDisplayFunctionLibrary|GetOrientationandPosition))) false false)
        (Progress|SetPercent (Variables|/Game/Vive/Blueprints/WidgetUI/CatapultHealthBar.CatapultHealthBar_C|GetProgressBar_143 _ascatapult_health_bar) (/ (Variables|Default|GetHealth) 1e+02))
        (if (Variables|Default|GetIsOnFire)
          (Variables|Default|SetHealth (- (Variables|Default|GetHealth) 0.1)))
        ;[1 1 1] Moving AI
        (if (Variables|Default|GetIsFull?)
          (if (Variables|Default|GetHasPosition)
            (Variables|/Script/Engine.CharacterMovementComponent|SetMaxWalkSpeed (Variables|Character|GetCharacterMovement) 0.0)
            (elif (Variables|/Game/Vive/Blueprints/AI/BP_SiegePathStops.BP_SiegePathStops_C|GetLastStation? (Variables|Default|GetFirstPos))
              (if (Variables|/Game/Vive/Blueprints/AI/BP_BatteringRamAttackPosition.BP_BatteringRamAttackPosition_C|GetPositionTaken (Variables|Default|GetAttackPos))
                (AI|AIMoveTo self "0, 0, 0" (Variables|/Game/Vive/Blueprints/AI/BP_BatteringRamAttackPosition.BP_BatteringRamAttackPosition_C|GetNextPosition (Variables|Default|GetAttackPos)) 5.0 true
                  (:then
                    (Variables|Default|SetAttackPos (Variables|/Game/Vive/Blueprints/AI/BP_BatteringRamAttackPosition.BP_BatteringRamAttackPosition_C|GetNextPosition (Variables|Default|GetAttackPos)))))
                (else
                  (AI|AIMoveTo self "0, 0, 0" (Variables|Default|GetAttackPos) 5.0 true))))))))))

(event EventDestroyed
  (bind _attackpos (Variables|Default|GetAttackPos))
  ;[1 1 1] Moving AI
  (if (Variables|Default|GetHasPosition)
    (Variables|/Game/Vive/Blueprints/AI/BP_BatteringRamAttackPosition.BP_BatteringRamAttackPosition_C|SetPositionTaken _attackpos false)
    (Variables|/Game/Vive/Blueprints/AI/BP_BatteringRamAttackPosition.BP_BatteringRamAttackPosition_C|SetTimer _attackpos 0.0)))

(fn ConstructionScript
  (Variables|Default|SetHandleBool1 false)
  (Variables|Default|SetHandleString1 "Handle1")
  (Variables|Default|SetHandleString2 "Handle2")
  (Variables|Default|SetHandleBool2 false))

(fn PrinttoVive
  (params (String :type String))
  (Development|PrintString String)
  (Development|PrintString String)
  (Development|PrintString String)
  (Development|PrintString String)
  (Development|PrintString String)
  (Development|PrintString String)
  (Development|PrintString String)
  (Development|PrintString String)
  (Development|PrintString String)
  (Development|PrintString String)
  (Development|PrintString String)
  (Development|PrintString String)
  (Development|PrintString String)
  (Development|PrintString String)
  (Development|PrintString String)
  (Development|PrintString String))