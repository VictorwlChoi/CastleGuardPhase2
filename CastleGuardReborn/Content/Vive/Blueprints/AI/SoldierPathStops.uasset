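; Path waypoint actor that relays soldier AI from one station to the next.
; When a SoldierAI or LightSoldierAI overlaps its OverlapCheck component, it sends that pawn toward NextStation with AIMoveTo, unless LastStation is set.
; A successful move updates the soldier's FirstStop to that station, so linked stops form a chain that ends at the last one.
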(event OnComponentBeginOverlap(OverlapCheck)
  (params (OverlappedComponent :type Primitive%20Component%20Object%20Reference) (OtherActor :type Actor%20Object%20Reference) (OtherComp :type Primitive%20Component%20Object%20Reference) (OtherBodyIndex :type Integer) (bFromSweep :type Boolean) (SweepResult :type Hit%20Result%20Structure%20%28by%20ref%29))
  (bind _nextstation (Variables|Default|GetNextStation))
  (bind _nextstation_2 (Variables|Default|GetNextStation))
  (bind _assoldier_ai (Utilities|Casting|CastToSoldierAI OtherActor)
    (:then
      (if (not (Variables|Default|GetLastStation?))
        (AI|AIMoveTo _assoldier_ai "0, 0, 0" _nextstation_2 1e+01 false
          (:OnSuccess
            (Variables|/Game/Vive/Blueprints/AI/SoldierAIHeavy/SoldierAI.SoldierAI_C|SetFirstStop _assoldier_ai _nextstation_2)))))
    (:CastFailed
      (bind _aslight_soldier_ai (Utilities|Casting|CastToLightSoldierAI OtherActor))
      (if (not (Variables|Default|GetLastStation?))
        (AI|AIMoveTo _aslight_soldier_ai "0, 0, 0" _nextstation 1e+01 false
          (:OnSuccess
            (Variables|/Game/Vive/Blueprints/AI/SoldierAILight/LightSoldierAI.LightSoldierAI_C|SetFirstStop _aslight_soldier_ai _nextstation)))))))

(fn ConstructionScript)