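; CatapultPathStops is a waypoint actor that moves siege units along a path of stations.
; When a Catapult or BatteringRamOld overlaps its OverlapCheck component, it issues an AI MoveTo toward NextStation, unless flagged as LastStation.
; Each move also stores NextStation as that unit's FirstPos.
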(event OnComponentBeginOverlap(OverlapCheck)
  (params (OverlappedComponent :type Primitive%20Component%20Object%20Reference) (OtherActor :type Actor%20Object%20Reference) (OtherComp :type Primitive%20Component%20Object%20Reference) (OtherBodyIndex :type Integer) (bFromSweep :type Boolean) (SweepResult :type Hit%20Result%20Structure%20%28by%20ref%29))
  (bind _nextstation (Variables|Default|GetNextStation))
  (bind _nextstation_2 (Variables|Default|GetNextStation))
  (bind _ascatapult (Utilities|Casting|CastToCatapult OtherActor)
    (:then
      (if (not (Variables|Default|GetLastStation?))
        (AI|AIMoveTo _ascatapult "0, 0, 0" _nextstation_2 1e+01 false
          (:then
            (Variables|/Game/Vive/Blueprints/AI/Catapult.Catapult_C|SetFirstPos _ascatapult _nextstation_2)))))
    (:CastFailed
      (bind _asbattering_ram_old (Utilities|Casting|CastToBatteringRamOld OtherActor))
      (if (not (Variables|Default|GetLastStation?))
        (AI|AIMoveTo _asbattering_ram_old "0, 0, 0" _nextstation 5.0 false
          (:then
            (Variables|/Game/Vive/Blueprints/AI/BatteringRamOld.BatteringRamOld_C|SetFirstPos _asbattering_ram_old _nextstation)))))))

(fn ConstructionScript)