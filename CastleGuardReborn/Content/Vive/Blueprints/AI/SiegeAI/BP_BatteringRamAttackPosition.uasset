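; BP_BatteringRamAttackPosition is a siege AI spot where a battering ram docks and damages the gate.
; The first BP_BatteringRamOld to overlap its box claims the position, is flagged as positioned, and has MountHandle set on both soldiers' animation instances.
; While claimed, Tick accumulates time and periodically subtracts health from the first SM_TestDoor_Blueprint found in the level, with no release logic.
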(event OnComponentBeginOverlap(Box)
  (params (OverlappedComponent :type Primitive%20Component%20Object%20Reference) (OtherActor :type Actor%20Object%20Reference) (OtherComp :type Primitive%20Component%20Object%20Reference) (OtherBodyIndex :type Integer) (bFromSweep :type Boolean) (SweepResult :type Hit%20Result%20Structure%20%28by%20ref%29))
  (if (not (Variables|Default|GetPositionTaken))
    (bind _asbp_battering_ram_old (Utilities|Casting|CastToBP_BatteringRamOld OtherActor))
    (Variables|/Game/Vive/Blueprints/AI/SiegeAI/BP_BatteringRamOld.BP_BatteringRamOld_C|SetHasPosition _asbp_battering_ram_old true)
    (Variables|Default|SetPositionTaken true)
    (Variables|Default|SetBatteringRam OtherActor)
    (bind _asabp_soldier_unit (Utilities|Casting|CastToABP_SoldierUnit (Components|SkeletalMesh|GetAnimInstance (Variables|/Script/Engine.Character|GetMesh (Variables|/Game/Vive/Blueprints/AI/SiegeAI/BP_BatteringRamOld.BP_BatteringRamOld_C|GetSoldier1 _asbp_battering_ram_old)))))
    (Variables|/Game/Vive/Blueprints/AI/SoldierAI/ABP_SoldierUnit.ABP_SoldierUnit_C|SetMountHandle _asabp_soldier_unit true)
    (bind _asabp_soldier_unit_2 (Utilities|Casting|CastToABP_SoldierUnit (Components|SkeletalMesh|GetAnimInstance (Variables|/Script/Engine.Character|GetMesh (Variables|/Game/Vive/Blueprints/AI/SiegeAI/BP_BatteringRamOld.BP_BatteringRamOld_C|GetSoldier2 _asbp_battering_ram_old)))))
    (Variables|/Game/Vive/Blueprints/AI/SoldierAI/ABP_SoldierUnit.ABP_SoldierUnit_C|SetMountHandle _asabp_soldier_unit_2 true)))

(event EventTick
  (params (DeltaSeconds :type Float%20%28single-precision%29))
  (if (Variables|Default|GetPositionTaken)
    (Variables|Default|SetTimer (+ DeltaSeconds (Variables|Default|GetTimer)))
    (Utilities|Casting|CastToBP_BatteringRamOld (Variables|Default|GetBatteringRam))
    ;[1 1 1] RamDamagessGate
    (if (>= (Variables|Default|GetTimer) 4.0)
      (bind _outactors (Actor|GetAllActorsOfClass "/Game/Vive/Blueprints/SM_TestDoor_Blueprint.SM_TestDoor_Blueprint_C"))
      (Variables|/Game/Vive/Blueprints/SM_TestDoor_Blueprint.SM_TestDoor_Blueprint_C|SetHealth (Utilities|Array|Get(acopy) _outactors) (- (Variables|/Game/Vive/Blueprints/SM_TestDoor_Blueprint.SM_TestDoor_Blueprint_C|GetHealth (Utilities|Array|Get(acopy) _outactors)) 1.0))
      (Variables|Default|SetTimer 0.0))))

(fn ConstructionScript)