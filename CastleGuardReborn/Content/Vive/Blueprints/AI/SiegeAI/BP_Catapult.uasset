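; BP_Catapult is a siege AI catapult for a Vive VR game, extending a parent class.
; BeginPlay caches the first BP_PlayerCollision actor, and Tick turns the catapult toward it with zero pitch while in one particular state.
; The construction script fills handle names and left/right detach points.
; Helpers repeat a debug print and play attached chain audio, whose random pick always lands on the first sound.
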(event EventBeginPlay
  (|CallParentFunction)
  (bind _outactors (Actor|GetAllActorsOfClass "/Game/Vive/Blueprints/BP_PlayerCollision.BP_PlayerCollision_C"))
  (if (> (Utilities|Array|Length _outactors) 0)
    (Variables|Default|SetPlayerRef (Utilities|Array|Get(acopy) _outactors))
    (else
      (Development|PrintString "BP_Catapult::NoPlayerCollisionInScene"))))

(event EventTick
  (params (DeltaSeconds :type Float%20%28single-precision%29))
  (bind _returnvalue (Transformation|GetActorLocation))
  (bind _playerref (Variables|Default|GetPlayerRef))
  (bind _returnvalue_2 (Transformation|GetActorLocation _playerref))
  (bind _returnvalue_3 (Math|Rotator|FindLookatRotation _returnvalue _returnvalue_2))
  (bind (_roll _pitch _yaw) (Math|Rotator|BreakRotator _returnvalue_3))
  (|CallParentFunction DeltaSeconds)
  (if (Utilities|Enum|Equal(Enum) (Variables|Default|GetCurrentState) "NewEnumerator1")
    (Transformation|SetActorRotation (Math|Rotator|MakeRotator _roll 0.0 _yaw))))

(fn ConstructionScript
  (bind _handlestrings (Variables|Default|GetHandleStrings))
  (|CallParentFunction)
  (Utilities|Array|Clear _handlestrings)
  (Utilities|Array|Add _handlestrings "CatapultLeftHandle")
  (Utilities|Array|Add _handlestrings "CatapultRightHandle")
  (Variables|Default|SetDetachPoints (Utilities|Array|MakeArray (Variables|Default|GetDetachPointLeft) (Variables|Default|GetDetachPointRight))))

(fn PrinttoVive
  (params (String%20In :type String))
  (Development|PrintString String%20In)
  (Development|PrintString String%20In)
  (Development|PrintString String%20In)
  (Development|PrintString String%20In)
  (Development|PrintString String%20In)
  (Development|PrintString String%20In)
  (Development|PrintString String%20In)
  (Development|PrintString String%20In)
  (Development|PrintString String%20In)
  (Development|PrintString String%20In)
  (Development|PrintString String%20In)
  (Development|PrintString String%20In)
  (Development|PrintString String%20In)
  (Development|PrintString String%20In)
  (Development|PrintString String%20In)
  (Development|PrintString String%20In))

(fn CatapultChainAudio
  (params (CatapultPositionIn :type Vector))
  (bind _returnvalue (Math|Random|RandomInteger 0))
  (if (== _returnvalue 0)
    (Audio|SpawnSoundAttached 0 (Variables|Default|GetChainAudio1) "None" CatapultPositionIn)
    (elif (== _returnvalue 0)
      _)))