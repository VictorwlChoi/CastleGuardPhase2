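; AI battering ram for a VR siege, crewed by up to two soldiers who snap to handle sockets on overlap.
; It moves toward its path point once crewed, faster with both, then seeks a free attack position and stops there.
; Tick yaws it toward its target, pitches it from a ground trace and turns its health bar to the headset.
; Burning arrows drain health; death destroys ram and crew and frees the position.
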(event OnComponentBeginOverlap(SoldierOverlapCheck)
  (params (OverlappedComponent :type Primitive%20Component%20Object%20Reference) (OtherActor :type Actor%20Object%20Reference) (OtherComp :type Primitive%20Component%20Object%20Reference) (OtherBodyIndex :type Integer) (bFromSweep :type Boolean) (SweepResult :type Hit%20Result%20Structure%20%28by%20ref%29))
  ;[1 1 1] Soldiers attach themselves to Battering Ram
  (if (Variables|Default|GetIsActive)
    (bind _asbp_soldier_ai (Utilities|Casting|CastToBP_SoldierAI OtherActor))
    (Variables|/Game/Vive/Blueprints/AI/SoldierAI/BP_SoldierAI.BP_SoldierAI_C|SetBatteringRam _asbp_soldier_ai (Variables|Default|GetNextRam))
    (if (not (Variables|Default|GetHandleBool2))
      (if (Variables|Default|GetHandleBool1)
        (if (!= OtherActor (Variables|Default|GetSoldier1))
          (bind _asbp_soldier_ai_2 (Utilities|Casting|CastToBP_SoldierAI OtherActor))
          (Collision|SetCollisionEnabled (Variables|/Script/Engine.Character|GetMesh _asbp_soldier_ai_2) "NoCollision")
          (Variables|Default|SetHandleBool2 true)
          (Transformation|AttachComponentToComponent OtherActor (Variables|Character|GetMesh) (Utilities|String|StringToName (Variables|Default|GetHandleString2)) "SnapToTarget" "SnapToTarget" "KeepWorld" false)
          (Variables|Default|SetIsFull? true)
          (Collision|SetActorEnableCollision OtherActor false)
          (bind _asbp_soldier_ai_3 (Utilities|Casting|CastToBP_SoldierAI OtherActor))
          (Variables|Default|SetSoldier2 _asbp_soldier_ai_3)
          (bind _asabp_soldier_unit (Utilities|Casting|CastToABP_SoldierUnit (Components|SkeletalMesh|GetAnimInstance (Variables|/Script/Engine.Character|GetMesh _asbp_soldier_ai_3))))
          (Variables|/Game/Vive/Blueprints/AI/SoldierAI/ABP_SoldierUnit.ABP_SoldierUnit_C|SetSiegeHandle _asabp_soldier_unit "RightRamHandle"))
        (else
          (bind _asbp_soldier_ai_4 (Utilities|Casting|CastToBP_SoldierAI OtherActor))
          (Collision|SetCollisionEnabled (Variables|/Script/Engine.Character|GetMesh _asbp_soldier_ai_4) "NoCollision")
          (Variables|Default|SetHandleBool1 true)
          (Transformation|AttachComponentToComponent OtherActor (Variables|Character|GetMesh) (Utilities|String|StringToName (Variables|Default|GetHandleString1)) "SnapToTarget" "SnapToTarget" "KeepWorld" false)
          (Collision|SetActorEnableCollision OtherActor false)
          (bind _asbp_soldier_ai_5 (Utilities|Casting|CastToBP_SoldierAI OtherActor))
          (Variables|Default|SetSoldier1 _asbp_soldier_ai_5)
          (bind _asabp_soldier_unit_2 (Utilities|Casting|CastToABP_SoldierUnit (Components|SkeletalMesh|GetAnimInstance (Variables|/Script/Engine.Character|GetMesh _asbp_soldier_ai_5))))
          (Variables|/Game/Vive/Blueprints/AI/SoldierAI/ABP_SoldierUnit.ABP_SoldierUnit_C|SetSiegeHandle _asabp_soldier_unit_2 "LeftRamHandle"))))))

(event OnComponentHit(Mesh)
  (params (HitComponent :type Primitive%20Component%20Object%20Reference) (OtherActor :type Actor%20Object%20Reference) (OtherComp :type Primitive%20Component%20Object%20Reference) (NormalImpulse :type Vector :default "0, 0, 0") (Hit :type Hit%20Result%20Structure%20%28by%20ref%29))
  (if (Variables|Default|GetIsActive)
    (bind _asbp_light_arrow (Utilities|Casting|CastToBP_LightArrow OtherActor)
      (:then
        (if (Variables|/Game/Vive/Blueprints/BP_LightArrow.BP_LightArrow_C|GetOnFire _asbp_light_arrow)
          (Variables|Default|SetIsOnFire true)))
      (:CastFailed
        (bind _asbp_heavy_arrow (Utilities|Casting|CastToBP_HeavyArrow OtherActor))
        (if (Variables|/Game/Vive/Blueprints/BP_HeavyArrow.BP_HeavyArrow_C|GetOnFire _asbp_heavy_arrow)
          (Variables|Default|SetIsOnFire true))))))

(event OnComponentBeginOverlap(CapsuleComponent)
  (params (OverlappedComponent :type Primitive%20Component%20Object%20Reference) (OtherActor :type Actor%20Object%20Reference) (OtherComp :type Primitive%20Component%20Object%20Reference) (OtherBodyIndex :type Integer) (bFromSweep :type Boolean) (SweepResult :type Hit%20Result%20Structure%20%28by%20ref%29))
  ;[1 1 1] Moving AI
  (if (Variables|Default|GetIsActive)
    (Utilities|Casting|CastToBP_BatteringRamAttackPosition OtherActor)
    (Variables|Default|SetHasPosition true)))

(event Custom|ResetSoldierRotations
  (if (Variables|Default|GetIsFull?)
    _))

(event Custom|Tick
  ;[1 1 1] Soldiers attach themselves to Battering Ram
  (if (Variables|Default|GetIsActive)
    (if (Variables|Default|GetHandleBool1)
      (if (Variables|Default|GetHandleBool2)
        (Variables|/Script/Engine.CharacterMovementComponent|SetMaxWalkSpeed (Variables|Character|GetCharacterMovement) 4e+02)
        (AI|AIMoveTo self "0, 0, 0" (Variables|Default|GetFirstPos) 5.0 false)
        (else
          (Variables|/Script/Engine.CharacterMovementComponent|SetMaxWalkSpeed (Variables|Character|GetCharacterMovement) 2e+02)
          (AI|AIMoveTo self "0, 0, 0" (Variables|Default|GetFirstPos) 5.0 false))))))

(event EventTick
  (params (DeltaSeconds :type Float%20%28single-precision%29))
  (bind _firstpos (Variables|Default|GetFirstPos))
  (bind _capsulecomponent (Variables|Default|GetCapsuleComponent))
  (bind _firstpos_2 (Variables|Default|GetFirstPos))
  (bind _capsulecomponent_2 (Variables|Default|GetCapsuleComponent))
  (bind _returnvalue (Transformation|GetActorTransform _firstpos_2))
  (bind _returnvalue_2 (Transformation|GetWorldLocation _capsulecomponent_2))
  (bind _returnvalue_3 (Transformation|GetWorldLocation _capsulecomponent))
  (bind _location (Math|Transform|BreakTransform _returnvalue))
  (bind _returnvalue_4 (Math|Rotator|FindLookatRotation _returnvalue_3 _location))
  (bind (_roll _pitch _yaw) (Math|Rotator|BreakRotator _returnvalue_4))
  (if (Variables|Default|GetIsActive)
    (CallFunction|ResetSoldierRotations)
    ;[1 1 1] Raycast to get correct rotation for actor
    (bind _outhit (Collision|LineTraceByChannel _returnvalue_2 (+ _returnvalue_2 "0, 0,-100.000000") "TraceTypeQuery1" true 0 "None"))
    (if (Utilities|IsValid _firstpos)
      (if (Variables|/Game/Vive/Blueprints/AI/SiegeAI/BP_SiegePathStops.BP_SiegePathStops_C|GetLastStation? _firstpos)
        (Transformation|SetActorRotation (Math|Rotator|MakeRotator (.Roll (Math|Rotator|BreakRotator (Math|Rotator|FindLookatRotation (Transformation|GetWorldLocation (Variables|Default|GetCapsuleComponent)) (.Location (Math|Transform|BreakTransform (Transformation|GetActorTransform (Variables|Default|GetAttackPos))))))) (.Pitch (Math|Rotator|BreakRotator (Math|Rotator|MakeRotfromY (.Normal (Collision|BreakHitResult _outhit))))) (.Yaw (Math|Rotator|BreakRotator (Math|Rotator|FindLookatRotation (Transformation|GetWorldLocation (Variables|Default|GetCapsuleComponent)) (.Location (Math|Transform|BreakTransform (Transformation|GetActorTransform (Variables|Default|GetAttackPos)))))))) true)
        (else
          (Transformation|SetActorRotation (Math|Rotator|MakeRotator _roll (.Pitch (Math|Rotator|BreakRotator (Math|Rotator|MakeRotfromY (.Normal (Collision|BreakHitResult _outhit))))) _yaw) true)))
      ;[1 1 1] Health And Death
      (CallFunction|Tick)
      (if (<= (Variables|Default|GetHealth) 0.0)
        (bind _outactors (Actor|GetAllActorsOfClass "/Game/Vive/Blueprints/Overlords/BP_Overlord_Master.BP_Overlord_Master_C"))
        (Utilities|Array|RemoveItem (Variables|/Game/Vive/Blueprints/Overlords/BP_Overlord_Master.BP_Overlord_Master_C|GetUnitArray (Utilities|Array|Get(acopy) _outactors)) (Variables|Default|GetSoldier1))
        (Actor|DestroyActor (Variables|Default|GetSoldier1))
        (Utilities|Array|RemoveItem (Variables|/Game/Vive/Blueprints/Overlords/BP_Overlord_Master.BP_Overlord_Master_C|GetUnitArray (Utilities|Array|Get(acopy) _outactors)) (Variables|Default|GetSoldier2))
        (Actor|DestroyActor (Variables|Default|GetSoldier2))
        (Utilities|Array|RemoveItem (Variables|/Game/Vive/Blueprints/Overlords/BP_Overlord_Master.BP_Overlord_Master_C|GetUnitArray (Utilities|Array|Get(acopy) _outactors)) self)
        (Audio|PlaySoundatLocation 0 (Transformation|GetActorLocation))
        (Actor|DestroyActor)
        (else
          (bind _ascatapult_health_bar (Utilities|Casting|CastToCatapultHealthBar (UserInterface|GetUserWidgetObject (Variables|Default|GetRamHealthBarComponent))))
          (Transformation|SetWorldRotation (Variables|Default|GetRamHealthBarComponent) (Math|Rotator|FindLookatRotation (Transformation|GetWorldLocation (Variables|Default|GetRamHealthBarComponent)) (.DevicePosition (Class|HeadMountedDisplayFunctionLibrary|GetOrientationandPosition))) false false)
          (Progress|SetPercent (Variables|/Game/Vive/Blueprints/WidgetUI/CatapultHealthBar.CatapultHealthBar_C|GetProgressBar_143 _ascatapult_health_bar) (/ (Variables|Default|GetHealth) 1e+02))
          (if (Variables|Default|GetIsOnFire)
            (Variables|Default|SetHealth (- (Variables|Default|GetHealth) 0.1))
            (Rendering|SetVisibility (Variables|Default|GetFlame1) true false))
          ;[1 1 1] Moving AI
          (if (Variables|Default|GetIsFull?)
            (if (Variables|Default|GetHasPosition)
              (Variables|/Script/Engine.CharacterMovementComponent|SetMaxWalkSpeed (Variables|Character|GetCharacterMovement) 0.0)
              (elif (Variables|/Game/Vive/Blueprints/AI/SiegeAI/BP_SiegePathStops.BP_SiegePathStops_C|GetLastStation? (Variables|Default|GetFirstPos))
                (if (Variables|/Game/Vive/Blueprints/AI/SiegeAI/BP_BatteringRamAttackPosition.BP_BatteringRamAttackPosition_C|GetPositionTaken (Variables|Default|GetAttackPos))
                  (AI|AIMoveTo self "0, 0, 0" (Variables|/Game/Vive/Blueprints/AI/SiegeAI/BP_BatteringRamAttackPosition.BP_BatteringRamAttackPosition_C|GetNextPosition (Variables|Default|GetAttackPos)) 5.0 true
                    (:then
                      (Variables|Default|SetAttackPos (Variables|/Game/Vive/Blueprints/AI/SiegeAI/BP_BatteringRamAttackPosition.BP_BatteringRamAttackPosition_C|GetNextPosition (Variables|Default|GetAttackPos)))))
                  (else
                    (AI|AIMoveTo self "0, 0, 0" (Variables|Default|GetAttackPos) 5.0 true)))))))))))

(event EventDestroyed
  (bind _attackpos (Variables|Default|GetAttackPos))
  ;[1 1 1] Moving AI
  (if (Variables|Default|GetHasPosition)
    (Variables|/Game/Vive/Blueprints/AI/SiegeAI/BP_BatteringRamAttackPosition.BP_BatteringRamAttackPosition_C|SetPositionTaken _attackpos false)
    (Variables|/Game/Vive/Blueprints/AI/SiegeAI/BP_BatteringRamAttackPosition.BP_BatteringRamAttackPosition_C|SetTimer _attackpos 0.0)))

(fn ConstructionScript
  (Variables|Default|SetHandleBool1 false)
  (Variables|Default|SetHandleString1 "LeftRamHandle")
  (Variables|Default|SetHandleString2 "RightRamHandle")
  (Variables|Default|SetHandleBool2 false))

(fn PrinttoVive
  (params (String :type String))
  (Development|PrintString String)
  (Development|PrintString String)
  (Development|PrintString String)
  (Development|PrintString String)
  (Development|PrintString String)
  (Development|PrintString String)
  (Development|PrintString String)
  (Development|PrintString String)
  (Development|PrintString String)
  (Development|PrintString String)
  (Development|PrintString String)
  (Development|PrintString String)
  (Development|PrintString String)
  (Development|PrintString String)
  (Development|PrintString String)
  (Development|PrintString String))