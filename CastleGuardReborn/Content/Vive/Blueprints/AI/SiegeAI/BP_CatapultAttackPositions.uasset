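; BP_CatapultAttackPositions is a siege AI attack spot that a catapult claims and fires rocks from.
; The first catapult to overlap its box takes the position permanently and gets HasPosition set.
; While taken, Tick runs a timer, firing every 3 seconds if both catapult handle bools are true, every 5 if only one.
; Rocks spawn above the catapult, rotated along the line from the position to the first test door found.
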(event OnComponentBeginOverlap(Box)
  (params (OverlappedComponent :type Primitive%20Component%20Object%20Reference) (OtherActor :type Actor%20Object%20Reference) (OtherComp :type Primitive%20Component%20Object%20Reference) (OtherBodyIndex :type Integer) (bFromSweep :type Boolean) (SweepResult :type Hit%20Result%20Structure%20%28by%20ref%29))
  (if (not (Variables|Default|GetPositionTaken))
    (bind _asbp_catapult (Utilities|Casting|CastToBP_Catapult OtherActor))
    (Variables|/Game/Vive/Blueprints/AI/SiegeAI/BP_Catapult.BP_Catapult_C|SetHasPosition _asbp_catapult true)
    (Variables|Default|SetPositionTaken true)
    (Variables|Default|SetCatapult _asbp_catapult)))

(event EventTick
  (params (DeltaSeconds :type Float%20%28single-precision%29))
  (if (Variables|Default|GetPositionTaken)
    (Variables|Default|SetTimer (+ DeltaSeconds (Variables|Default|GetTimer)))
    (bind (_hasposition _handlebool1 _handlebool2) (Default|ReturnCatapultBools (Variables|Default|GetCatapult)))
    (if (and _handlebool1 _handlebool2)
      (if (>= (Variables|Default|GetTimer) 3.0)
        (Variables|Default|SetTimer 0.0)
        (bind _outactors (Actor|GetAllActorsOfClass "/Game/Vive/Blueprints/SM_TestDoor_Blueprint.SM_TestDoor_Blueprint_C" :!label _label))
        (Game|SpawnActorfromClass "/Game/Vive/Blueprints/CatapultProjectiles/BP_CatapultRock.BP_CatapultRock_C" (Math|Transform|MakeTransform (+ (Transformation|GetActorLocation (stale OnComponentBeginOverlap(Box) _asbp_catapult)) "0, 0,75.000000") (Math|Rotator|FindLookatRotation (Transformation|GetActorLocation) (Transformation|GetActorLocation (Utilities|Array|Get(acopy) _outactors)))) "Undefined" 0 0))
      (elif (or _handlebool1 _handlebool2)
        (if (>= (Variables|Default|GetTimer) 5.0)
          (Variables|Default|SetTimer 0.0)
          (goto _label))))))

(fn ConstructionScript)