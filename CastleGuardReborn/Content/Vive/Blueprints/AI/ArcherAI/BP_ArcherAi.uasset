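; Archer AI that shoots arrows at the player and dies when hit by one.
; BeginPlay caches the first BP_PlayerCollision actor, which Tick faces without pitching while in one particular state.
; The shoot event, if active, spawns BP_AI_Arrows aimed at the player's capsule, rolled a quarter turn.
; Any arrow hit plays a collapse sound and calls Seppuku, as the arrow-type branches are empty.
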(event Custom|EventShootArrow
  (bind _scene (Variables|Default|GetScene))
  (bind _playerref (Variables|Default|GetPlayerRef))
  (bind _returnvalue (Transformation|GetWorldLocation _scene))
  (bind _capsule (Variables|/Game/Vive/Blueprints/BP_PlayerCollision.BP_PlayerCollision_C|GetCapsule _playerref))
  (bind _returnvalue_2 (Transformation|GetWorldLocation _capsule))
  (bind _returnvalue_3 (Math|Rotator|FindLookatRotation _returnvalue _returnvalue_2))
  (bind (_roll _pitch _yaw) (Math|Rotator|BreakRotator _returnvalue_3))
  (bind _isactive_ (CallFunction|IsActive))
  (if _isactive_
    (Development|PrintString (Utilities|String|ToString(Vector) _returnvalue_2))
    (Game|SpawnActorfromClass "/Game/Vive/Blueprints/AI/ArcherAI/BP_AI_Arrows.BP_AI_Arrows_C" (Math|Transform|MakeTransform (Transformation|GetWorldLocation (Variables|Default|GetScene)) (Math|Rotator|MakeRotator (+ _roll 9e+01) _pitch _yaw)) "AlwaysSpawn" 0 0)))

(event EventBeginPlay
  (bind _outactors (Actor|GetAllActorsOfClass "/Game/Vive/Blueprints/BP_PlayerCollision.BP_PlayerCollision_C"))
  (if (> (Utilities|Array|Length _outactors) 0)
    (Variables|Default|SetPlayerRef (Utilities|Array|Get(acopy) _outactors))
    (else
      (Development|PrintString "BP_ArcherAI::NoPlayerCollisionInScene"))))

(event EventTick
  (params (DeltaSeconds :type Float%20%28single-precision%29))
  (bind _returnvalue (Transformation|GetActorLocation))
  (bind _playerref (Variables|Default|GetPlayerRef))
  (bind _returnvalue_2 (Transformation|GetActorLocation _playerref))
  (bind _returnvalue_3 (Math|Rotator|FindLookatRotation _returnvalue _returnvalue_2))
  (bind (_roll _pitch _yaw) (Math|Rotator|BreakRotator _returnvalue_3))
  (if (Utilities|Enum|Equal(Enum) (Variables|Default|GetCurrentState) "NewEnumerator1")
    (Transformation|SetActorRotation (Math|Rotator|MakeRotator _roll 0.0 _yaw) true)))

(event EventHitUnitwithArrow
  (params (AttackingArrow :type BP%20Base%20Arrow%20Object%20Reference) (HitLocation :type Vector :default "0, 0, 0") (HitComponent :type Scene%20Component%20Object%20Reference))
  (switch Utilities|FlowControl|Switch|SwitchonArrowType (Variables|/Game/Vive/Blueprints/BP_BaseArrow.BP_BaseArrow_C|GetArrowType AttackingArrow)
    (:NewEnumerator0
      _)
    (:NewEnumerator1
      _))
  (Audio|PlaySound2D "/Game/StarterContent/Audio/Collapse_Cue.Collapse_Cue")
  (CallFunction|Seppuku))

(fn ConstructionScript)