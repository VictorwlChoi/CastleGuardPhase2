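; Archer AI arrow projectile that aims at the VR player's collision capsule when constructed and destroys itself after ten seconds.
; Mesh hits play an impact sound by target: castle hits destroy the arrow, player hits also lower the Vive pawn's Health, and landscape hits leave it in place.
; Sound helpers chain random rolls, but the castle and player ones roll with a max of zero, so always play their first sound.
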(event OnComponentHit(StaticMesh)
  (params (HitComponent :type Primitive%20Component%20Object%20Reference) (OtherActor :type Actor%20Object%20Reference) (OtherComp :type Primitive%20Component%20Object%20Reference) (NormalImpulse :type Vector :default "0, 0, 0") (Hit :type Hit%20Result%20Structure%20%28by%20ref%29))
  (Variables|Default|SetHitLocation (|StaticMesHitLocation Hit))
  (Utilities|Casting|CastToBP_Castle OtherActor
    (:then
      (CallFunction|CastleImpactSoundEffect (Variables|Default|GetHitLocation))
      (Actor|DestroyActor))
    (:CastFailed
      (Utilities|Casting|CastToBP_PlayerCollision OtherActor
        (:then
          (CallFunction|PlayerImpactSoundEffect "0, 0, 0")
          (bind _outactors (Actor|GetAllActorsOfClass "/Game/Vive/Blueprints/BP_Vive_Pawn.BP_Vive_Pawn_C"))
          (Variables|/Game/Vive/Blueprints/BP_Vive_Pawn.BP_Vive_Pawn_C|SetHealth (Utilities|Array|Get(acopy) _outactors) (- (Variables|/Game/Vive/Blueprints/BP_Vive_Pawn.BP_Vive_Pawn_C|GetHealth (Utilities|Array|Get(acopy) _outactors)) (Variables|/Game/Vive/Blueprints/BP_Vive_Pawn.BP_Vive_Pawn_C|GetHealthDamage/Recovery (Utilities|Array|Get(acopy) _outactors))))
          (Actor|DestroyActor))
        (:CastFailed
          (Utilities|Casting|CastToLandscape OtherActor)
          (CallFunction|GroundImpactSoundEffect (Variables|Default|GetHitLocation)))))))

(event EventTick
  (params (DeltaSeconds :type Float%20%28single-precision%29))
  (bind _returnvalue (Transformation|GetActorRotation))
  (bind (_roll _pitch _yaw) (Math|Rotator|BreakRotator _returnvalue))
  (Transformation|SetActorRotation (Math|Rotator|MakeRotator (.Roll (Math|Rotator|BreakRotator (Math|Rotator|MakeRotfromX (Transformation|GetVelocity)))) _pitch _yaw)))

(event EventBeginPlay
  (Utilities|FlowControl|Delay 1e+01)
  (Actor|DestroyActor))

(fn ConstructionScript
  (bind _outactors (Actor|GetAllActorsOfClass "/Game/Vive/Blueprints/BP_PlayerCollision.BP_PlayerCollision_C"))
  (Transformation|SetActorRotation (Math|Rotator|FindLookatRotation (Transformation|GetWorldLocation (Variables|Default|GetStaticMesh)) (+ (Transformation|GetWorldLocation (Variables|/Game/Vive/Blueprints/BP_PlayerCollision.BP_PlayerCollision_C|GetCapsule (Utilities|Array|Get(acopy) _outactors))) "0, 0,34.000000")))
  (Variables|/Script/Engine.ProjectileMovementComponent|SetInitialSpeed (Variables|Default|GetProjectileMovement) 5e+03))

(fn PrinttoVive
  (params (String%20Input :type String))
  (Development|PrintString String%20Input)
  (Development|PrintString String%20Input)
  (Development|PrintString String%20Input)
  (Development|PrintString String%20Input)
  (Development|PrintString String%20Input)
  (Development|PrintString String%20Input)
  (Development|PrintString String%20Input)
  (Development|PrintString String%20Input)
  (Development|PrintString String%20Input)
  (Development|PrintString String%20Input)
  (Development|PrintString String%20Input)
  (Development|PrintString "Hello")
  (Development|PrintString String%20Input)
  (Development|PrintString String%20Input)
  (Development|PrintString String%20Input)
  (Development|PrintString String%20Input))

(fn CastleImpactSoundEffect
  (params (HitVectorIn :type Vector))
  (bind _returnvalue (Math|Random|RandomInteger 0))
  (if (== _returnvalue 0)
    (Audio|PlaySoundatLocation "/Game/Audio/SFX/ArrowSounds/Arrow_Impact_Dowel_1_Cue.Arrow_Impact_Dowel_1_Cue" HitVectorIn)
    (return)
    (elif (== _returnvalue 1)
      (Audio|PlaySoundatLocation "/Game/Audio/SFX/ArrowSounds/Arrow_Impact_Dowel_2_Cue.Arrow_Impact_Dowel_2_Cue" HitVectorIn)
      (return)
      (elif (== _returnvalue 2)
        (Audio|PlaySoundatLocation "/Game/Audio/SFX/ArrowSounds/Arrow_Impact_Dowel_3_Cue.Arrow_Impact_Dowel_3_Cue" HitVectorIn)
        (return)
        (elif (== _returnvalue 3)
          (Audio|PlaySoundatLocation "/Game/Audio/SFX/ArrowSounds/Arrow_impact_dowel_4_Cue.Arrow_impact_dowel_4_Cue" HitVectorIn)
          (return))))))

(fn GroundImpactSoundEffect
  (params (HitVectorIn :type Vector))
  (bind _returnvalue (Math|Random|RandomInteger 9))
  (if (== _returnvalue 0)
    (Audio|PlaySoundatLocation "/Game/Audio/SFX/ArrowSounds/Arrow_Impact_Gravel_1_Cue.Arrow_Impact_Gravel_1_Cue" HitVectorIn)
    (return)
    (elif (== _returnvalue 1)
      (Audio|PlaySoundatLocation "/Game/Audio/SFX/ArrowSounds/Arrow_Impact_Gravel_2_Cue.Arrow_Impact_Gravel_2_Cue" HitVectorIn)
      (return)
      (elif (== _returnvalue 2)
        (Audio|PlaySoundatLocation "/Game/Audio/SFX/ArrowSounds/Arrow_Impact_Gravel_3_Cue.Arrow_Impact_Gravel_3_Cue" HitVectorIn)
        (return)
        (elif (== _returnvalue 3)
          (Audio|PlaySoundatLocation "/Game/Audio/SFX/ArrowSounds/Arrow_Impact_Gravel_4_Cue.Arrow_Impact_Gravel_4_Cue" HitVectorIn)
          (return))))))

(fn PlayerImpactSoundEffect
  (params (HitVectorIn :type Vector))
  (bind _returnvalue (Math|Random|RandomInteger 0))
  (if (== _returnvalue 0)
    (Audio|PlaySoundatLocation "/Game/Audio/SFX/ArrowSounds/Arrow_Im_pact_Gravel_7.Arrow_Im_pact_Gravel_7" HitVectorIn)
    (elif (== _returnvalue 1)
      (Audio|PlaySoundatLocation 0 HitVectorIn)
      (elif (== _returnvalue 2)
        (Audio|PlaySoundatLocation 0 HitVectorIn)
        (elif (== _returnvalue 3)
          (Audio|PlaySoundatLocation 0 HitVectorIn)
          (elif (== _returnvalue 4)
            (Audio|PlaySoundatLocation 0 HitVectorIn)
            (elif (== _returnvalue 5)
              (Audio|PlaySoundatLocation 0 HitVectorIn)
              (elif (== _returnvalue 6)
                (Audio|PlaySoundatLocation 0 "0, 0, 0")
                (elif (== _returnvalue 7)
                  (Audio|PlaySoundatLocation 0 HitVectorIn)
                  (elif (== 0 8)
                    (Audio|PlaySoundatLocation 0 "0, 0, 0")
                    (else
                      (if (== 0 9)
                        _
                        (else
                          _))
                      (Audio|PlaySoundatLocation 0 "0, 0, 0"))))))))))))