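; BP_ArcherAttackPosition is a trigger spot that an archer AI occupies as its attack position.
; Box overlap by a BP_ArcherAi marks the spot taken and registers it on that archer; end overlap frees it and resets the timer.
; Disconnected logic, which never runs, would periodically spawn arrows aimed at the player collision capsule while the spot is taken; Tick is empty.
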(event OnComponentBeginOverlap(Box)
  (params (OverlappedComponent :type Primitive%20Component%20Object%20Reference) (OtherActor :type Actor%20Object%20Reference) (OtherComp :type Primitive%20Component%20Object%20Reference) (OtherBodyIndex :type Integer) (bFromSweep :type Boolean) (SweepResult :type Hit%20Result%20Structure%20%28by%20ref%29))
  (bind _asbp_archer_ai (Utilities|Casting|CastToBP_ArcherAi OtherActor))
  (Variables|/Game/Vive/Blueprints/AI/ArcherAI/BP_ArcherAi.BP_ArcherAi_C|SetHasPosition _asbp_archer_ai true)
  (Variables|Default|SetPositionTaken true)
  (Variables|/Game/Vive/Blueprints/AI/ArcherAI/BP_ArcherAi.BP_ArcherAi_C|SetAttackPosition _asbp_archer_ai self))

(event OnComponentEndOverlap(Box)
  (params (OverlappedComponent :type Primitive%20Component%20Object%20Reference) (OtherActor :type Actor%20Object%20Reference) (OtherComp :type Primitive%20Component%20Object%20Reference) (OtherBodyIndex :type Integer))
  (Utilities|Casting|CastToBP_ArcherAi OtherActor)
  (Development|PrintString "End Overlap")
  (Variables|Default|SetPositionTaken false)
  (Variables|Default|SetTimer 0.0))

(event EventTick
  (params (DeltaSeconds :type Float%20%28single-precision%29)))

(fn ConstructionScript)