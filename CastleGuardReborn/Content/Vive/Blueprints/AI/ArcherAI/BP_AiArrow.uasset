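; Arrow projectile for the archer AI in the VR game that homes in on the player and despawns after a fixed lifetime.
; While active, Tick steers the physics capsule at the first BP_PlayerCollision, then enables gravity and stops homing at close range with a slower final push.
; Overlapping the player collision damages BP_Vive_Pawn, plays its hit sound and destroys the arrow.
; Hitting BP_Castle destroys it with a sound; SetTransform lets a spawner place it.
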(event OnComponentBeginOverlap(Sphere1)
  (params (OverlappedComponent :type Primitive%20Component%20Object%20Reference) (OtherActor :type Actor%20Object%20Reference) (OtherComp :type Primitive%20Component%20Object%20Reference) (OtherBodyIndex :type Integer) (bFromSweep :type Boolean) (SweepResult :type Hit%20Result%20Structure%20%28by%20ref%29))
  (Variables|Default|SetHitLocation (|BreakHitCollapse_2 SweepResult))
  (Utilities|Casting|CastToBP_PlayerCollision OtherActor
    (:then
      (bind _outactors (Actor|GetAllActorsOfClass "/Game/Vive/Blueprints/BP_Vive_Pawn.BP_Vive_Pawn_C"))
      (Utilities|IsValid (Utilities|Array|Get(acopy) _outactors)
        (:Is%20Valid
          (Default|PlayHitSound (Utilities|Array|Get(acopy) _outactors))
          (Variables|/Game/Vive/Blueprints/BP_Vive_Pawn.BP_Vive_Pawn_C|SetHealth (Utilities|Array|Get(acopy) _outactors) (- (Variables|/Game/Vive/Blueprints/BP_Vive_Pawn.BP_Vive_Pawn_C|GetHealth (Utilities|Array|Get(acopy) _outactors)) 1e+02))
          (Actor|DestroyActor))))
    (:CastFailed
      (Utilities|Casting|CastToBP_Castle OtherActor))))

(event Collision|EventHit
  (params (MyComp :type Primitive%20Component%20Object%20Reference) (Other :type Actor%20Object%20Reference) (OtherComp :type Primitive%20Component%20Object%20Reference) (bSelfMoved :type Boolean) (HitLocation :type Vector :default "0, 0, 0") (HitNormal :type Vector :default "0, 0, 0") (NormalImpulse :type Vector :default "0, 0, 0") (Hit :type Hit%20Result%20Structure%20%28by%20ref%29))
  (Utilities|Casting|CastToBP_Castle Other)
  (Actor|DestroyActor)
  (Audio|PlaySoundatLocation 0 HitLocation))

(event EventBeginPlay
  (Utilities|FlowControl|Delay 2e+01)
  (Actor|DestroyActor))

(event EventTick
  (params (DeltaSeconds :type Float%20%28single-precision%29))
  (bind _outactors (Actor|GetAllActorsOfClass "/Game/Vive/Blueprints/BP_PlayerCollision.BP_PlayerCollision_C"))
  (if (and (> (Utilities|Array|Length _outactors) 0) (Variables|Default|GetbActive))
    (Physics|SetPhysicsLinearVelocity (Variables|Default|GetCapsule) (* (Math|Vector|Normalize (- (Transformation|GetActorLocation (Utilities|Array|Get(acopy) _outactors)) (Transformation|GetWorldLocation (Variables|Default|GetCapsule)))) 1e+04) false "None")
    (if (< (Math|Vector|VectorLengthSquared (- (Transformation|GetActorLocation (Utilities|Array|Get(acopy) _outactors)) (Transformation|GetWorldLocation (Variables|Default|GetCapsule)))) 1.5e+05)
      (Physics|SetEnableGravity (Variables|Default|GetCapsule) true)
      (Variables|Default|SetbActive false)
      (Physics|SetPhysicsLinearVelocity (Variables|Default|GetCapsule) (* (Math|Vector|Normalize (- (Transformation|GetActorLocation (Utilities|Array|Get(acopy) _outactors)) (Transformation|GetWorldLocation (Variables|Default|GetCapsule)))) 4e+03) false "None"))))

(fn ConstructionScript)

(fn SetTransform
  (params (SpawnerTransform :type Transform))
  (Transformation|SetActorTransform SpawnerTransform))