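; AI unit character that follows assigned paths toward an attack point, delegating initialization and path switching to its BP_AiController.
; Initialize stores the path and its attack point, sets an active state and restores gravity, while SwitchPath hands a new path to the controller.
; Seppuku unregisters the unit from its attack point and the first BP_Overlord_Nathan, then destroys it.
; The old point-to-point move event is deprecated and empty.
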(event Custom|Initialize
  (params (Path :type BP%20Spline%20Path%20Object%20Reference))
  ;[1 0.8452 0] Initialize
  (bind _output_get (Variables|Default|SetPathRef Path))
  (Variables|Default|SetAttackPoint (Variables|/Game/Nathan/BP_SplinePath.BP_SplinePath_C|GetAttackPoints _output_get))
  (Variables|Default|SetCurrentState "NewEnumerator2")
  (Variables|/Script/Engine.CharacterMovementComponent|SetGravityScale (Variables|Character|GetCharacterMovement) 1.0)
  (bind _asbp_ai_controller (Utilities|Casting|CastToBP_AiController (Pawn|GetController)))
  (Default|Initialize _asbp_ai_controller))

(event Custom|SwitchPath
  (params (NewPath :type BP%20Spline%20Path%20Object%20Reference))
  ;[1 0 0.673] Switch Paths
  (bind _output_get (Variables|Default|SetPathRef NewPath))
  (Variables|Default|SetShouldSwitchPaths true)
  (bind _asbp_ai_controller (Utilities|Casting|CastToBP_AiController (Pawn|GetController)))
  (Default|SwitchPath _asbp_ai_controller _output_get))

(event Custom|Seppuku
  ;[0 1 0.9714] Sepuku
  (if (Utilities|IsValid (Variables|Default|GetAttackPoint))
    (Default|Unregister (Variables|Default|GetAttackPoint) self))
  (bind _outactors (Actor|GetAllActorsOfClass "/Game/Nathan/BP_Overlord_Nathan.BP_Overlord_Nathan_C"))
  (if (> (Utilities|Array|Length _outactors) 0)
    (Default|RemoveUnit (Utilities|Array|Get(acopy) _outactors) self))
  (Actor|DestroyActor))

(event Custom|MoveActorToNextPoint
  ;[1 0 0.8477] Move Actor To Next Point - Deprecated
)

(fn ConstructionScript)

(fn IsActive
  (return (Utilities|Enum|NotEqual(Enum) (Variables|Default|GetCurrentState) "NewEnumerator0")))