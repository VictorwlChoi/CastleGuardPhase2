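; AI battering ram character that soldiers crew and that advances toward an attack position.
; The first two overlapping soldiers snap to handle sockets; a full crew raises walk speed.
; Tick drives AIMoveTo through FirstPos and AttackPos, skipping taken positions; overlapping a CatapultFiringPosition1 halts a full ram.
; Fire arrows cause steady burn damage, shown on a headset-facing health bar; zero health destroys the ram and both soldiers.
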(event OnComponentBeginOverlap(SoldierOverlapCheck)
  (params (OverlappedComponent :type Primitive%20Component%20Object%20Reference) (OtherActor :type Actor%20Object%20Reference) (OtherComp :type Primitive%20Component%20Object%20Reference) (OtherBodyIndex :type Integer) (bFromSweep :type Boolean) (SweepResult :type Hit%20Result%20Structure%20%28by%20ref%29))
  (bind _handlestring2 (Variables|Default|GetHandleString2))
  (bind _handlestring1 (Variables|Default|GetHandleString1))
  ;[1 1 1] Soldiers attach themselves to Battering Ram
  (bind _assoldier_ai (Utilities|Casting|CastToSoldierAI OtherActor))
  (Variables|/Game/Vive/Blueprints/AI/SoldierAI.SoldierAI_C|SetBatteringRam _assoldier_ai (Variables|Default|GetNextRam))
  (if (Actor|ActorHasTag OtherActor "Soldier")
    (if (not (Variables|Default|GetHandleBool2))
      (if (Variables|Default|GetHandleBool1)
        (Variables|Default|SetHandleBool2 true)
        (Development|PrintString _handlestring2)
        (Transformation|AttachComponentToComponent OtherActor (Variables|Default|GetCube) (Utilities|String|StringToName _handlestring2) "SnapToTarget" "SnapToTarget" "KeepWorld" false)
        (Variables|Default|SetIsFull? true)
        (Collision|SetActorEnableCollision OtherActor false)
        (Variables|Default|SetSoldier2 _assoldier_ai)
        (else
          (Variables|Default|SetHandleBool1 true)
          (Development|PrintString _handlestring1)
          (Transformation|AttachComponentToComponent OtherActor (Variables|Default|GetCube) (Utilities|String|StringToName _handlestring1) "SnapToTarget" "SnapToTarget" "KeepWorld" false)
          (Collision|SetActorEnableCollision OtherActor false)
          (Variables|Default|SetSoldier1 _assoldier_ai))))))

(event OnComponentBeginOverlap(CapsuleComponent)
  (params (OverlappedComponent :type Primitive%20Component%20Object%20Reference) (OtherActor :type Actor%20Object%20Reference) (OtherComp :type Primitive%20Component%20Object%20Reference) (OtherBodyIndex :type Integer) (bFromSweep :type Boolean) (SweepResult :type Hit%20Result%20Structure%20%28by%20ref%29))
  ;[1 1 1] Moving AI
  (Utilities|Casting|CastToCatapultFiringPosition1 OtherActor)
  (Variables|Default|SetHasPosition true))

(event Custom|Tick
  ;[1 1 1] Soldiers attach themselves to Battering Ram
  (if (Variables|Default|GetHandleBool1)
    (if (Variables|Default|GetHandleBool2)
      (Variables|/Script/Engine.CharacterMovementComponent|SetMaxWalkSpeed (Variables|Character|GetCharacterMovement) 8e+02)
      (AI|AIMoveTo self "0, 0, 0" (Variables|Default|GetFirstPos) 5.0 false)
      (else
        (Variables|/Script/Engine.CharacterMovementComponent|SetMaxWalkSpeed (Variables|Character|GetCharacterMovement) 5e+01)
        (AI|AIMoveTo self "0, 0, 0" (Variables|Default|GetFirstPos) 5.0 false)))))

(event EventTick
  (params (DeltaSeconds :type Float%20%28single-precision%29))
  ;[1 1 1] Health And Death
  (CallFunction|Tick)
  (if (<= (Variables|Default|GetHealth) 0.0)
    (Actor|DestroyActor (Variables|Default|GetSoldier1))
    (Actor|DestroyActor (Variables|Default|GetSoldier2))
    (Actor|DestroyActor)
    (else
      (bind _ascatapult_health_bar (Utilities|Casting|CastToCatapultHealthBar (UserInterface|GetUserWidgetObject (Variables|Default|GetRamHealthBarComponent))))
      (Transformation|SetWorldRotation (Variables|Default|GetRamHealthBarComponent) (Math|Rotator|FindLookatRotation (Transformation|GetWorldLocation (Variables|Default|GetRamHealthBarComponent)) (.DevicePosition (Class|HeadMountedDisplayFunctionLibrary|GetOrientationandPosition))) false false)
      (Progress|SetPercent (Variables|/Game/Vive/Blueprints/WidgetUI/CatapultHealthBar.CatapultHealthBar_C|GetProgressBar_143 _ascatapult_health_bar) (/ (Variables|Default|GetHealth) 1e+02))
      (if (Variables|Default|GetIsOnFire)
        (Variables|Default|SetHealth (- (Variables|Default|GetHealth) 0.05)))
      ;[1 1 1] Moving AI
      (if (Variables|Default|GetIsFull?)
        (if (Variables|Default|GetHasPosition)
          (Variables|/Script/Engine.CharacterMovementComponent|SetMaxWalkSpeed (Variables|Character|GetCharacterMovement) 0.0)
          (elif (Variables|/Game/Vive/Blueprints/AI/CatapultPathStops.CatapultPathStops_C|GetLastStation? (Variables|Default|GetFirstPos))
            (if (Variables|/Game/Vive/Blueprints/AI/BatteringRamAttackPosition.BatteringRamAttackPosition_C|GetPositionTaken (Variables|Default|GetAttackPos))
              (AI|AIMoveTo self "0, 0, 0" (Variables|/Game/Vive/Blueprints/AI/BatteringRamAttackPosition.BatteringRamAttackPosition_C|GetNextPosition (Variables|Default|GetAttackPos)) 5.0 true
                (:then
                  (Variables|Default|SetAttackPos (Variables|/Game/Vive/Blueprints/AI/BatteringRamAttackPosition.BatteringRamAttackPosition_C|GetNextPosition (Variables|Default|GetAttackPos)))))
              (else
                (AI|AIMoveTo self "0, 0, 0" (Variables|Default|GetAttackPos) 5.0 true)))))))))

(event Collision|EventHit
  (params (MyComp :type Primitive%20Component%20Object%20Reference) (Other :type Actor%20Object%20Reference) (OtherComp :type Primitive%20Component%20Object%20Reference) (bSelfMoved :type Boolean) (HitLocation :type Vector :default "0, 0, 0") (HitNormal :type Vector :default "0, 0, 0") (NormalImpulse :type Vector :default "0, 0, 0") (Hit :type Hit%20Result%20Structure%20%28by%20ref%29))
  (if (Actor|ActorHasTag Other "FireArrow")
    (Variables|Default|SetIsOnFire true)))

(fn ConstructionScript
  (Variables|Default|SetHandleBool1 false)
  (Variables|Default|SetHandleString1 "Handle1")
  (Variables|Default|SetHandleString2 "Handle2")
  (Variables|Default|SetHandleBool2 false))