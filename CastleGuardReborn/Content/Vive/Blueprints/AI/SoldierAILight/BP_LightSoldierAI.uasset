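; BP_LightSoldierAI is a light soldier AI that walks to a first stop, then seeks a free attack position.
; While it has no position, Tick issues AI MoveTo orders, flagging the first stop once that move is issued.
; If that stop is a last station, it follows the NextPosition chain past taken attack positions and moves to the free one.
; An author note warns against spawning soldiers too close together.
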(event EventTick
  (params (DeltaSeconds :type Float%20%28single-precision%29))
  ;[1 1 1] Moving AI (Dont Spawn too close together.)
  (if (not (Variables|Default|GetHasPosition))
    (if (Variables|Default|GetFirst%20Stop)
      (if (Variables|/Game/Vive/Blueprints/AI/BP_SoldierPathStops.BP_SoldierPathStops_C|GetLastStation? (Variables|Default|GetFirstStop))
        (if (Variables|/Game/Vive/Blueprints/AI/BP_SoldierAttackPosition.BP_SoldierAttackPosition_C|GetPositionTaken (Variables|Default|GetAttackPos))
          (Variables|Default|SetAttackPos (Variables|/Game/Vive/Blueprints/AI/BP_SoldierAttackPosition.BP_SoldierAttackPosition_C|GetNextPosition (Variables|Default|GetAttackPos)))
          (else
            (AI|AIMoveTo self "0, 0, 0" (Variables|Default|GetAttackPos) 5.0 true))))
      (else
        (AI|AIMoveTo self "0, 0, 0" (Variables|Default|GetFirstStop) 1e+01 false
          (:then
            (Variables|Default|SetFirst%20Stop true)))))))

(fn ConstructionScript)