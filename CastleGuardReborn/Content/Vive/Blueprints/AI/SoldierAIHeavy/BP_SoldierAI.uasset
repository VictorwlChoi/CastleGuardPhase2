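; Heavy soldier AI that advances on an attack position or mans a nearby siege engine, shrugging off light arrows with a sound.
; Until it has a position, Tick compares path lengths to divert it to a closer catapult or battering ram with free handles.
; Otherwise it heads for a first stop, then an attack spot, following NextPosition past taken ones.
; Overlapping a non-full engine sets HasPosition, ending movement updates.
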(event EventTick
  (params (DeltaSeconds :type Float%20%28single-precision%29))
  (bind _returnvalue (Transformation|GetActorLocation))
  (bind _batteringram (Variables|Default|GetBatteringRam))
  (bind _firststop (Variables|Default|GetFirstStop))
  (bind _catapult (Variables|Default|GetCatapult))
  (bind _returnvalue_2 (Transformation|GetActorLocation _firststop))
  (bind _pathlength (Class|NavigationSystem|GetPathLength _returnvalue _returnvalue_2))
  ;[1 1 1] Moving AI (Dont Spawn too close together.)
  (if (not (Variables|Default|GetHasPosition))
    (if (Utilities|IsValid (Variables|Default|GetCatapult))
      (if (<= _pathlength (.PathLength (Class|NavigationSystem|GetPathLength _returnvalue (Transformation|GetActorLocation (Variables|Default|GetCatapult)))))
        (if (Utilities|IsValid (Variables|Default|GetBatteringRam)) :!label _label
          (if (<= _pathlength (.PathLength (Class|NavigationSystem|GetPathLength _returnvalue (Transformation|GetActorLocation (Variables|Default|GetBatteringRam)))))
            (if (Variables|Default|GetFirstStop?) :!label _label_2
              (if (Variables|/Game/Vive/Blueprints/AI/BP_SoldierPathStops.BP_SoldierPathStops_C|GetLastStation? (Variables|Default|GetFirstStop))
                (if (Variables|/Game/Vive/Blueprints/AI/BP_SoldierAttackPosition.BP_SoldierAttackPosition_C|GetPositionTaken (Variables|Default|GetAttackPos))
                  (Variables|Default|SetAttackPos (Variables|/Game/Vive/Blueprints/AI/BP_SoldierAttackPosition.BP_SoldierAttackPosition_C|GetNextPosition (Variables|Default|GetAttackPos)))
                  (else
                    (AI|AIMoveTo self "0, 0, 0" (Variables|Default|GetAttackPos) 5.0 true))))
              (else
                (AI|AIMoveTo self "0, 0, 0" (Variables|Default|GetFirstStop) 1e+01 false
                  (:then
                    (Variables|Default|SetFirstStop? true)))))
            (elif (Variables|/Game/Vive/Blueprints/AI/BP_BatteringRamOld.BP_BatteringRamOld_C|GetHandleBool1 _batteringram)
              (if (Variables|/Game/Vive/Blueprints/AI/BP_BatteringRamOld.BP_BatteringRamOld_C|GetHandleBool2 _batteringram)
                (goto _label_2)
                (else
                  (AI|AIMoveTo self "0, 0, 0" _batteringram 1e+01 false)))
              (else
                (AI|AIMoveTo self "0, 0, 0" _batteringram 1e+01 false))))
          (else
            (goto _label_2)))
        (elif (Variables|/Game/Vive/Blueprints/AI/BP_Catapult.BP_Catapult_C|GetHandleBool1 _catapult)
          (if (Variables|/Game/Vive/Blueprints/AI/BP_Catapult.BP_Catapult_C|GetHandleBool2 _catapult)
            (goto _label_2)
            (else
              (AI|AIMoveTo self "0, 0, 0" _catapult 1e+01 false)))
          (else
            (AI|AIMoveTo self "0, 0, 0" _catapult 1e+01 false))))
      (else
        (goto _label)))))

(event Collision|EventActorBeginOverlap
  (params (OtherActor :type Actor%20Object%20Reference))
  (bind _batteringram (Variables|Default|GetBatteringRam))
  (bind _catapult (Variables|Default|GetCatapult))
  ;[1 1 1] Manning Catapult
  (bind _asbp_light_arrow (Utilities|Casting|CastToBP_LightArrow OtherActor)
    (:then
      (Audio|PlaySoundatLocation 0 (Transformation|GetActorLocation _asbp_light_arrow))
      (Actor|DestroyActor _asbp_light_arrow))
    (:CastFailed
      (if (Utilities|IsValid _catapult)
        (if (Utilities|ClassIsChildOf (Utilities|GetClass OtherActor) "/Game/Vive/Blueprints/AI/BP_Catapult.BP_Catapult_C")
          (if (not (Variables|/Game/Vive/Blueprints/AI/BP_Catapult.BP_Catapult_C|GetIsFull? _catapult))
            (Variables|Default|SetHasPosition true :!label _label)))
        (elif (Utilities|ClassIsChildOf (Utilities|GetClass OtherActor) "/Game/Vive/Blueprints/AI/BP_BatteringRamOld.BP_BatteringRamOld_C")
          (if (Utilities|IsValid _batteringram)
            (if (not (Variables|/Game/Vive/Blueprints/AI/BP_BatteringRamOld.BP_BatteringRamOld_C|GetIsFull? _batteringram))
              (goto _label))))))))

(fn ConstructionScript)