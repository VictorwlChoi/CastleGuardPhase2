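; BP_LightSoldierAI is a light soldier AI pawn that carries a sword and shield.
; On BeginPlay it snaps the Sword and Shield components to their matching sockets on the Mesh.
; An unconnected movement graph would send it through a first stop to an attack position, stepping along linked positions when one is taken.
; Tick is empty, so that movement logic never runs.
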(event EventBeginPlay
  (Transformation|AttachComponentToComponent (Variables|Default|GetSword) (Variables|Character|GetMesh) "SwordSocket" "SnapToTarget" "SnapToTarget" "SnapToTarget" true)
  (Transformation|AttachComponentToComponent (Variables|Default|GetShield) (Variables|Character|GetMesh) "ShieldSocket" "SnapToTarget" "SnapToTarget" "SnapToTarget" true))

(event EventTick
  (params (DeltaSeconds :type Float%20%28single-precision%29))
  ;[1 1 1] Moving AI (Dont Spawn too close together.)
)

(fn ConstructionScript)