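; BP_LightSoldierAttackPosition is an attack slot where a light soldier AI stands to damage the gate.
; Box overlap with a BP_LightSoldierAI sets the soldier's HasPosition and the slot's PositionTaken, and end overlap clears both.
; While the slot is taken, Tick accumulates a timer and every three seconds subtracts health from the first SM_TestDoor_Blueprint found in the level, printing a debug message.
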(event OnComponentBeginOverlap(Box)
  (params (OverlappedComponent :type Primitive%20Component%20Object%20Reference) (OtherActor :type Actor%20Object%20Reference) (OtherComp :type Primitive%20Component%20Object%20Reference) (OtherBodyIndex :type Integer) (bFromSweep :type Boolean) (SweepResult :type Hit%20Result%20Structure%20%28by%20ref%29))
  (bind _asbp_light_soldier_ai (Utilities|Casting|CastToBP_LightSoldierAI OtherActor))
  (Variables|/Game/Vive/Blueprints/AI/SoldierAI/SoldierAILight/BP_LightSoldierAI.BP_LightSoldierAI_C|SetHasPosition _asbp_light_soldier_ai true)
  (Variables|Default|SetPositionTaken true))

(event OnComponentEndOverlap(Box)
  (params (OverlappedComponent :type Primitive%20Component%20Object%20Reference) (OtherActor :type Actor%20Object%20Reference) (OtherComp :type Primitive%20Component%20Object%20Reference) (OtherBodyIndex :type Integer))
  (bind _asbp_light_soldier_ai (Utilities|Casting|CastToBP_LightSoldierAI OtherActor))
  (Variables|/Game/Vive/Blueprints/AI/SoldierAI/SoldierAILight/BP_LightSoldierAI.BP_LightSoldierAI_C|SetHasPosition _asbp_light_soldier_ai false)
  (Variables|Default|SetPositionTaken false))

(event EventTick
  (params (DeltaSeconds :type Float%20%28single-precision%29))
  (if (Variables|Default|GetPositionTaken)
    (Variables|Default|SetTimer (+ DeltaSeconds (Variables|Default|GetTimer)))
    ;[1 1 1] SoldierDamagesGate
    (if (>= (Variables|Default|GetTimer) 3.0)
      (bind _outactors (Actor|GetAllActorsOfClass "/Game/Vive/Blueprints/SM_TestDoor_Blueprint.SM_TestDoor_Blueprint_C"))
      (Variables|/Game/Vive/Blueprints/SM_TestDoor_Blueprint.SM_TestDoor_Blueprint_C|SetHealth (Utilities|Array|Get(acopy) _outactors) (- (Variables|/Game/Vive/Blueprints/SM_TestDoor_Blueprint.SM_TestDoor_Blueprint_C|GetHealth (Utilities|Array|Get(acopy) _outactors)) 1.0))
      (Variables|Default|SetTimer 0.0)
      (Development|PrintString "Light Soldier Damage"))))

(fn ConstructionScript)