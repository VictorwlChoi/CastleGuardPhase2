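; BP_SoldierPathStops is a waypoint that relays soldier AI pawns along a chain of path stops.
; When a BP_SoldierAI or BP_LightSoldierAI begins overlapping its OverlapCheck component, it sends that pawn to NextStation with AI MoveTo, unless LastStation is set.
; On a successful move, it stores NextStation as the soldier's FirstStop.
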(event OnComponentBeginOverlap(OverlapCheck)
  (params (OverlappedComponent :type Primitive%20Component%20Object%20Reference) (OtherActor :type Actor%20Object%20Reference) (OtherComp :type Primitive%20Component%20Object%20Reference) (OtherBodyIndex :type Integer) (bFromSweep :type Boolean) (SweepResult :type Hit%20Result%20Structure%20%28by%20ref%29))
  (bind _nextstation (Variables|Default|GetNextStation))
  (bind _nextstation_2 (Variables|Default|GetNextStation))
  (bind _asbp_soldier_ai (Utilities|Casting|CastToBP_SoldierAI OtherActor)
    (:then
      (if (not (Variables|Default|GetLastStation?))
        (AI|AIMoveTo _asbp_soldier_ai "0, 0, 0" _nextstation_2 1e+01 false
          (:OnSuccess
            (Variables|/Game/Vive/Blueprints/AI/SoldierAI/BP_SoldierAI.BP_SoldierAI_C|SetFirstStop _asbp_soldier_ai _nextstation_2)))))
    (:CastFailed
      (bind _asbp_light_soldier_ai (Utilities|Casting|CastToBP_LightSoldierAI OtherActor))
      (if (not (Variables|Default|GetLastStation?))
        (AI|AIMoveTo _asbp_light_soldier_ai "0, 0, 0" _nextstation 1e+01 false
          (:OnSuccess
            (Variables|/Game/Vive/Blueprints/AI/SoldierAI/SoldierAILight/BP_LightSoldierAI.BP_LightSoldierAI_C|SetFirstStop _asbp_light_soldier_ai _nextstation)))))))

(fn ConstructionScript)