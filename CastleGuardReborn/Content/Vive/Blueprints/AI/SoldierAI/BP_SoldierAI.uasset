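; Soldier AI unit that carries a sword and shield, attached to its mesh sockets at BeginPlay.
; Light arrows overlapping the actor while it is active play a sound and are destroyed, while the shield's overlap destroys only flaming light or heavy arrows.
; An arrow-hit event kills the soldier through Seppuku with a collapse sound, handling only the Heavy arrow type.
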(event OnComponentBeginOverlap(Shield)
  (params (OverlappedComponent :type Primitive%20Component%20Object%20Reference) (OtherActor :type Actor%20Object%20Reference) (OtherComp :type Primitive%20Component%20Object%20Reference) (OtherBodyIndex :type Integer) (bFromSweep :type Boolean) (SweepResult :type Hit%20Result%20Structure%20%28by%20ref%29))
  (bind _asbp_heavy_arrow (Utilities|Casting|CastToBP_HeavyArrow OtherActor)
    (:then
      (if (Variables|/Game/Vive/Blueprints/BP_HeavyArrow.BP_HeavyArrow_C|GetOnFire _asbp_heavy_arrow)
        (Actor|DestroyActor _asbp_heavy_arrow)
        (Actor|DestroyActor OtherActor)))
    (:CastFailed
      (bind _asbp_light_arrow (Utilities|Casting|CastToBP_LightArrow OtherActor))
      (if (Variables|/Game/Vive/Blueprints/BP_LightArrow.BP_LightArrow_C|GetOnFire _asbp_light_arrow)
        (Actor|DestroyActor _asbp_light_arrow)
        (Actor|DestroyActor OtherActor)))))

(event EventHitUnitwithArrow
  (params (AttackingArrow :type BP%20Base%20Arrow%20Object%20Reference) (HitLocation :type Vector :default "0, 0, 0") (HitComponent :type Scene%20Component%20Object%20Reference))
  (switch Utilities|FlowControl|Switch|SwitchonArrowType (Variables|/Game/Vive/Blueprints/BP_BaseArrow.BP_BaseArrow_C|GetArrowType AttackingArrow)
    (:NewEnumerator1
      (Audio|PlaySound2D "/Game/StarterContent/Audio/Collapse_Cue.Collapse_Cue")
      (CallFunction|Seppuku))))

(event EventBeginPlay
  ;[1 1 1] Moving AI (Dont Spawn too close together.)
  (|CallParentFunction)
  (Transformation|AttachComponentToComponent (Variables|Default|GetSword) (Variables|Character|GetMesh) "SwordSocket" "SnapToTarget" "SnapToTarget" "SnapToTarget" true)
  (Transformation|AttachComponentToComponent (Variables|Default|GetShield) (Variables|Character|GetMesh) "ShieldSocket" "SnapToTarget" "SnapToTarget" "SnapToTarget" true))

(event Collision|EventActorBeginOverlap
  (params (OtherActor :type Actor%20Object%20Reference))
  ;[1 1 1] Manning Catapult
  (bind _isactive_ (CallFunction|IsActive))
  (if _isactive_
    (bind _asbp_light_arrow (Utilities|Casting|CastToBP_LightArrow OtherActor))
    (Audio|PlaySoundatLocation 0 (Transformation|GetActorLocation _asbp_light_arrow))
    (Actor|DestroyActor _asbp_light_arrow)))

(fn ConstructionScript
  (|CallParentFunction))