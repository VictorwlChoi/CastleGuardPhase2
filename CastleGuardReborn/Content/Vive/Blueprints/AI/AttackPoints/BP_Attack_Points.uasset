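; Attack point volume that builds a grid of BP_Attack_Point_Notifier actors inside SpawnBounds and allocates them to AI characters.
; AiCharacters entering the box register themselves until Unregister frees their point.
; A DoOnce-gated delay on Tick periodically walks rows front to back, collecting free points matching one occupation type.
; Units without a point or assigned farther back move into those points, keeping front rows filled first.
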(event OnComponentBeginOverlap(SpawnBounds)
  (params (OverlappedComponent :type Primitive%20Component%20Object%20Reference) (OtherActor :type Actor%20Object%20Reference) (OtherComp :type Primitive%20Component%20Object%20Reference) (OtherBodyIndex :type Integer) (bFromSweep :type Boolean) (SweepResult :type Hit%20Result%20Structure%20%28by%20ref%29))
  (bind _asai_character (Utilities|Casting|CastToAiCharacter OtherActor))
  (CallFunction|RegistertoAttackPoint _asai_character))

(event Custom|CheckRowPriority
  (Utilities|Array|Clear (Variables|Default|GetPriorityList))
  (if (> (Utilities|Array|Length (Variables|Default|GetRegisteredUnits)) 0)
    (bind (_rowindex _colindex _arrayindex) (Utilities|RowColforLoop (Variables|Default|GetRows) (Variables|Default|GetColumns) :!label _label)
      (:LoopBody
        (Utilities|IsValid (Utilities|Array|Get(acopy) (Variables|Default|GetAttackPositions) _arrayindex)
          (:Is%20Valid
            (if (not (Variables|/Game/Vive/Blueprints/AI/AttackPoints/BP_Attack_Point_Notifier.BP_Attack_Point_Notifier_C|GetIsAssigned (Utilities|Array|Get(acopy) (Variables|Default|GetAttackPositions) _arrayindex)))
              (if (Utilities|Enum|Equal(Enum) (Variables|/Game/Vive/Blueprints/AI/AttackPoints/BP_Attack_Point_Notifier.BP_Attack_Point_Notifier_C|GetEnemyTypeOccupation (Utilities|Array|Get(acopy) (Variables|Default|GetAttackPositions) _arrayindex)) "NewEnumerator6")
                (Utilities|Array|Add (Variables|Default|GetPriorityList) _arrayindex))))))
      (:RowStart
        (Utilities|FindUnassignedCount _rowindex
          (:Complete
            (Utilities|Array|Clear (Variables|Default|GetPriorityList))
            (if (== (Utilities|Array|Length (Variables|Default|GetUnassignedUnits)) 0)
              (goto _label Break)))))
      (:RowComplete
        (Variables|Default|SetCurrUnitIndex 0)
        (bind _array_element (Utilities|Array|ForEachLoopwithBreak (Variables|Default|GetPriorityList) :!label _label_2)
          (:LoopBody
            (if (< (Variables|Default|GetCurrUnitIndex) (Utilities|Array|Length (Variables|Default|GetUnassignedUnits)))
              (if (!= (Variables|/Game/Vive/Blueprints/AI/AiCharacter.AiCharacter_C|GetAttackPointIndex (Utilities|Array|Get(acopy) (Variables|Default|GetUnassignedUnits) (Variables|Default|GetCurrUnitIndex))) -1)
                (Variables|/Game/Vive/Blueprints/AI/AttackPoints/BP_Attack_Point_Notifier.BP_Attack_Point_Notifier_C|SetIsAssigned (Utilities|Array|Get(acopy) (Variables|Default|GetAttackPositions) (Variables|/Game/Vive/Blueprints/AI/AiCharacter.AiCharacter_C|GetAttackPointIndex (Utilities|Array|Get(acopy) (Variables|Default|GetUnassignedUnits) (Variables|Default|GetCurrUnitIndex)))) false))
              (Variables|/Game/Vive/Blueprints/AI/AiCharacter.AiCharacter_C|SetAttackPointIndex (Utilities|Array|Get(acopy) (Variables|Default|GetUnassignedUnits) (Variables|Default|GetCurrUnitIndex)) _array_element)
              (Math|Integer|IncrementInt (Variables|Default|GetCurrUnitIndex)
                (:%20%20
                  (Variables|/Game/Vive/Blueprints/AI/AttackPoints/BP_Attack_Point_Notifier.BP_Attack_Point_Notifier_C|SetIsAssigned (Utilities|Array|Get(acopy) (Variables|Default|GetAttackPositions) _array_element) true)))
              (else
                (goto _label_2 Break)))))))))

(event EventBeginPlay
  (CallFunction|BuildSpawnPoints))

(event Collision|EventActorBeginOverlap
  (params (OtherActor :type Actor%20Object%20Reference)))

(event EventTick
  (params (DeltaSeconds :type Float%20%28single-precision%29))
  (Utilities|FlowControl|DoOnce false :!label _label
    (:Completed
      (Utilities|FlowControl|Delay (Variables|Default|GetAttackPointDeltaTime))
      (CallFunction|CheckRowPriority)
      (goto _label Reset))))

(fn ConstructionScript)

(fn BuildSpawnPoints
  (bind _distancebetweenpoints (Variables|Default|GetDistanceBetweenPoints))
  (bind _attackpositions (Variables|Default|GetAttackPositions))
  (bind _spawnbounds (Variables|Default|GetSpawnBounds))
  (bind _spawnbounds_2 (Variables|Default|GetSpawnBounds))
  (bind _spawnbounds_3 (Variables|Default|GetSpawnBounds))
  (bind _spawnbounds_4 (Variables|Default|GetSpawnBounds))
  (bind _returnvalue (Transformation|GetWorldTransform _spawnbounds))
  (bind _boxextent (Variables|/Script/Engine.BoxComponent|GetBoxExtent _spawnbounds_2))
  (bind _boxextent_2 (Variables|/Script/Engine.BoxComponent|GetBoxExtent _spawnbounds_4))
  (bind _boxextent_3 (Variables|/Script/Engine.BoxComponent|GetBoxExtent _spawnbounds_3))
  (LocalVariables|SetHalfWidth (/ (Variables|Default|GetDistanceBetweenPoints) 2.0))
  (for _array_element _attackpositions
    (Utilities|IsValid _array_element
      (:Is%20Valid
        (Actor|DestroyActor _array_element))))
  (Utilities|Array|Clear _attackpositions)
  (bind _output_get (Variables|Default|SetRows (Math|Integer|Max(Integer) (Math|Float|Truncate (* (/ (.x _boxextent_3) _distancebetweenpoints) 2.0)) 1)))
  (bind _output_get_2 (Variables|Default|SetColumns (Math|Integer|Max(Integer) (Math|Float|Truncate (* (/ (.y _boxextent_3) _distancebetweenpoints) 2.0)) 1)))
  (Utilities|Array|Resize (Variables|Default|GetAttackPositions) (* _output_get_2 _output_get))
  (if (== (* _output_get_2 _output_get) 1)
    (bind _returnvalue_2 (Game|SpawnActorfromClass "/Game/Vive/Blueprints/AI/AttackPoints/BP_Attack_Point_Notifier.BP_Attack_Point_Notifier_C" (Transformation|GetWorldTransform (Variables|Default|GetSpawnBounds)) "Undefined" 0 0))
    (Utilities|Array|SetArrayElem (Variables|Default|GetAttackPositions) 0 _returnvalue_2)
    (return)
    (else
      (Utilities|FlowControl|Sequence
        (:then_0
          (LocalVariables|SetCurrentRowPos (Utilities|Select :Index (Math|Integer|%(Integer) (Variables|Default|GetRows) 2) :Option%200 (- (.x _boxextent_2) (LocalVariables|GetHalfWidth)) :Option%201 (- (.x _boxextent_2) (LocalVariables|GetHalfWidth))))
          (LocalVariables|SetCenterLocation (.location _returnvalue))
          (LocalVariables|SetBaseRotation (.rotation _returnvalue)))
        (:then_1
          (LocalVariables|SetColStartPoint (* (Utilities|Select :Index (Math|Integer|%(Integer) (Variables|Default|GetColumns) 2) :Option%200 (- (.y _boxextent) (LocalVariables|GetHalfWidth)) :Option%201 (- (.y _boxextent) (LocalVariables|GetHalfWidth))) -1.0)))
        (:then_2
          (for _index (range 0 (- (Variables|Default|GetRows) 1))
            (LocalVariables|SetCurrentColPos (LocalVariables|GetColStartPoint))
            (for _index_2 (range 0 (- (Variables|Default|GetColumns) 1))
              (bind _returnvalue_3 (Game|SpawnActorfromClass "/Game/Vive/Blueprints/AI/AttackPoints/BP_Attack_Point_Notifier.BP_Attack_Point_Notifier_C" (Math|Transform|MakeTransform (+ (+ (LocalVariables|GetCenterLocation) (* (Math|Vector|GetForwardVector (LocalVariables|GetBaseRotation)) (LocalVariables|GetCurrentRowPos))) (* (Math|Vector|GetRightVector (LocalVariables|GetBaseRotation)) (LocalVariables|GetCurrentColPos))) (LocalVariables|GetBaseRotation) "1,1,1") "Undefined" 0 0))
              (Utilities|Array|SetArrayElem (Variables|Default|GetAttackPositions) (+ _index_2 (* _index (Variables|Default|GetColumns))) _returnvalue_3)
              (LocalVariables|SetCurrentColPos (+ (Variables|Default|GetDistanceBetweenPoints) (LocalVariables|GetCurrentColPos))))
            (LocalVariables|SetCurrentRowPos (- (LocalVariables|GetCurrentRowPos) (Variables|Default|GetDistanceBetweenPoints)))))))))

(fn RegistertoAttackPoint
  (params (UnitToRegister :type Ai%20Character%20Object%20Reference))
  (Utilities|Array|AddUnique (Variables|Default|GetRegisteredUnits) UnitToRegister))

(fn RequestIndex)

(fn Unregister
  (params (CurrentUnit :type Ai%20Character%20Object%20Reference))
  (bind _attackpointindex (Variables|/Game/Vive/Blueprints/AI/AiCharacter.AiCharacter_C|GetAttackPointIndex CurrentUnit))
  (Utilities|Array|RemoveItem (Variables|Default|GetRegisteredUnits) CurrentUnit)
  (if (not (== _attackpointindex -1))
    (Variables|/Game/Vive/Blueprints/AI/AttackPoints/BP_Attack_Point_Notifier.BP_Attack_Point_Notifier_C|SetIsAssigned (Utilities|Array|Get(acopy) (Variables|Default|GetAttackPositions) _attackpointindex) false)))