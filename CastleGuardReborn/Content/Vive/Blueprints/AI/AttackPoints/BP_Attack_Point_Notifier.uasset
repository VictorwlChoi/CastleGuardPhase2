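; BP_Attack_Point_Notifier is an AI attack point actor that tracks which enemy type occupies it and shows that state by color.
; When an AiCharacter enters the Box with an EnemyType different from the stored occupation, it records that type and character and turns the Sphere red.
; When that recorded occupier leaves, the type resets and the Sphere returns to white through a dynamic material instance created at BeginPlay.
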(event OnComponentBeginOverlap(Box)
  (params (OverlappedComponent :type Primitive%20Component%20Object%20Reference) (OtherActor :type Actor%20Object%20Reference) (OtherComp :type Primitive%20Component%20Object%20Reference) (OtherBodyIndex :type Integer) (bFromSweep :type Boolean) (SweepResult :type Hit%20Result%20Structure%20%28by%20ref%29))
  (bind _asai_character (Utilities|Casting|CastToAiCharacter OtherActor))
  (if (Utilities|Enum|NotEqual(Enum) (Variables|Default|GetEnemyTypeOccupation) (Variables|/Game/Vive/Blueprints/AI/AiCharacter.AiCharacter_C|GetEnemyType _asai_character))
    (Variables|Default|SetEnemyTypeOccupation (Variables|/Game/Vive/Blueprints/AI/AiCharacter.AiCharacter_C|GetEnemyType _asai_character))
    (Rendering|Material|SetVectorParameterValue (Variables|Default|GetMaterialSignifier) "Color" "(R=0.692708,G=0.028495,B=0.000000,A=1.000000)" :!class /Script/Engine.MaterialInstanceDynamic)
    (Variables|Default|SetCurrentOccupier _asai_character)))

(event OnComponentEndOverlap(Box)
  (params (OverlappedComponent :type Primitive%20Component%20Object%20Reference) (OtherActor :type Actor%20Object%20Reference) (OtherComp :type Primitive%20Component%20Object%20Reference) (OtherBodyIndex :type Integer))
  (bind _asai_character (Utilities|Casting|CastToAiCharacter OtherActor))
  (if (== _asai_character (Variables|Default|GetCurrentOccupier))
    (Variables|Default|SetEnemyTypeOccupation "NewEnumerator6")
    (Rendering|Material|SetVectorParameterValue (Variables|Default|GetMaterialSignifier) "Color" "(R=1.000000,G=1.000000,B=1.000000,A=1.000000)" :!class /Script/Engine.MaterialInstanceDynamic)))

(event EventBeginPlay
  (bind _returnvalue (Rendering|Material|CreateDynamicMaterialInstance "/Game/Vive/Blueprints/AI/AttackPoints/M_ColorSignifier.M_ColorSignifier" :!class /Script/Engine.KismetMaterialLibrary))
  (Rendering|Material|SetMaterial (Variables|Default|GetSphere) 0 _returnvalue)
  (bind _output_get (Variables|Default|SetMaterialSignifier _returnvalue))
  (Rendering|Material|SetVectorParameterValue _output_get "Color" "(R=1.000000,G=1.000000,B=1.000000,A=1.000000)" :!class /Script/Engine.MaterialInstanceDynamic))

(event Collision|EventActorBeginOverlap
  (params (OtherActor :type Actor%20Object%20Reference)))

(event EventTick
  (params (DeltaSeconds :type Float%20%28single-precision%29)))

(fn ConstructionScript)