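; ArcherAI is the archer pawn logic that walks the character to a free attack position.
; Each Tick, until HasPosition is set, it moves toward a first stop and flags that stop on arrival.
; Once the stop's LastStation is true, it heads to AttackPosition, following the linked NextPosition chain whenever the current position is taken.
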(event EventTick
  (params (DeltaSeconds :type Float%20%28single-precision%29))
  (if (not (Variables|Default|GetHasPosition))
    (if (Variables|Default|GetFirstStop?)
      (if (Variables|/Game/Vive/Blueprints/AI/ArcherPathStops.ArcherPathStops_C|GetLastStation? (Variables|Default|GetFirstStop))
        (if (Variables|/Game/Vive/Blueprints/AI/ArcherAttackPosition.ArcherAttackPosition_C|GetPositionTaken (Variables|Default|GetAttackPosition))
          (AI|AIMoveTo self "0, 0, 0" (Variables|/Game/Vive/Blueprints/AI/ArcherAttackPosition.ArcherAttackPosition_C|GetNextPosition (Variables|Default|GetAttackPosition)) 5.0 true
            (:then
              (Variables|Default|SetAttackPosition (Variables|/Game/Vive/Blueprints/AI/ArcherAttackPosition.ArcherAttackPosition_C|GetNextPosition (Variables|Default|GetAttackPosition)))))
          (else
            (AI|AIMoveTo self "0, 0, 0" (Variables|Default|GetAttackPosition) 5.0 true))))
      (else
        (AI|AIMoveTo self "0, 0, 0" (Variables|Default|GetFirstStop) 5.0 false
          (:then
            (Variables|Default|SetFirstStop? true)))))))

(fn ConstructionScript)