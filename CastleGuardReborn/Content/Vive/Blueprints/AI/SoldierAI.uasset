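; Soldier AI that walks to siege engines or attack positions and is destroyed when hit by an Arrow-tagged actor.
; Each Tick, until it has a position, it compares path lengths to send itself to a Catapult or BatteringRam with an unset handle flag, otherwise toward FirstStop.
; After the last station it follows linked attack positions to find a free one.
; Overlapping a non-full Catapult marks it positioned, halting further move orders.
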(event Collision|EventHit
  (params (MyComp :type Primitive%20Component%20Object%20Reference) (Other :type Actor%20Object%20Reference) (OtherComp :type Primitive%20Component%20Object%20Reference) (bSelfMoved :type Boolean) (HitLocation :type Vector :default "0, 0, 0") (HitNormal :type Vector :default "0, 0, 0") (NormalImpulse :type Vector :default "0, 0, 0") (Hit :type Hit%20Result%20Structure%20%28by%20ref%29))
  ;[1 1 1] Death By Arrow
  (if (Actor|ActorHasTag Other "Arrow")
    (Actor|DestroyActor)))

(event EventTick
  (params (DeltaSeconds :type Float%20%28single-precision%29))
  (bind _returnvalue (Transformation|GetActorLocation))
  (bind _batteringram (Variables|Default|GetBatteringRam))
  (bind _firststop (Variables|Default|GetFirstStop))
  (bind _catapult (Variables|Default|GetCatapult))
  (bind _returnvalue_2 (Transformation|GetActorLocation _firststop))
  (bind _pathlength (Class|NavigationSystem|GetPathLength _returnvalue _returnvalue_2))
  ;[1 1 1] Moving AI (Dont Spawn too close together.)
  (if (not (Variables|Default|GetHasPosition))
    (if (Utilities|IsValid (Variables|Default|GetCatapult))
      (if (<= _pathlength (.PathLength (Class|NavigationSystem|GetPathLength _returnvalue (Transformation|GetActorLocation (Variables|Default|GetCatapult)))))
        (if (Utilities|IsValid (Variables|Default|GetBatteringRam)) :!label _label
          (if (<= _pathlength (.PathLength (Class|NavigationSystem|GetPathLength _returnvalue (Transformation|GetActorLocation (Variables|Default|GetBatteringRam)))))
            (if (Variables|Default|GetFirstStop?) :!label _label_2
              (if (Variables|/Game/Vive/Blueprints/AI/SoldierPathStops.SoldierPathStops_C|GetLastStation? (Variables|Default|GetFirstStop))
                (if (Variables|/Game/Vive/Blueprints/AI/SoldierAttackPosition.SoldierAttackPosition_C|GetPositionTaken (Variables|Default|GetAttackPos))
                  (Variables|Default|SetAttackPos (Variables|/Game/Vive/Blueprints/AI/SoldierAttackPosition.SoldierAttackPosition_C|GetNextPosition (Variables|Default|GetAttackPos)))
                  (else
                    (AI|AIMoveTo self "0, 0, 0" (Variables|Default|GetAttackPos) 5.0 true))))
              (else
                (AI|AIMoveTo self "0, 0, 0" (Variables|Default|GetFirstStop) 1e+01 false
                  (:then
                    (Variables|Default|SetFirstStop? true)))))
            (elif (Variables|/Game/Vive/Blueprints/AI/BatteringRamOld.BatteringRamOld_C|GetHandleBool1 _batteringram)
              (if (Variables|/Game/Vive/Blueprints/AI/BatteringRamOld.BatteringRamOld_C|GetHandleBool2 _batteringram)
                (goto _label_2)
                (else
                  (AI|AIMoveTo self "0, 0, 0" _batteringram 1e+01 false)))
              (else
                (AI|AIMoveTo self "0, 0, 0" _batteringram 1e+01 false))))
          (else
            (goto _label_2)))
        (elif (Variables|/Game/Vive/Blueprints/AI/Catapult.Catapult_C|GetHandleBool1 _catapult)
          (if (Variables|/Game/Vive/Blueprints/AI/Catapult.Catapult_C|GetHandleBool2 _catapult)
            (goto _label_2)
            (else
              (AI|AIMoveTo self "0, 0, 0" _catapult 1e+01 false)))
          (else
            (AI|AIMoveTo self "0, 0, 0" _catapult 1e+01 false))))
      (else
        (goto _label)))))

(event Collision|EventActorBeginOverlap
  (params (OtherActor :type Actor%20Object%20Reference))
  ;[1 1 1] Manning Catapult
  (if (Utilities|ClassIsChildOf (Utilities|GetClass OtherActor) "/Game/Vive/Blueprints/AI/Catapult.Catapult_C")
    (if (not (Variables|/Game/Vive/Blueprints/AI/Catapult.Catapult_C|GetIsFull? (Variables|Default|GetCatapult)))
      (Variables|Default|SetHasPosition true))))

(fn ConstructionScript)