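; BP_Siege is an AI siege unit, apparently a catapult, driven by BT_Siege and crewed by up to two soldiers.
; Overlapping soldiers attach to handle sockets, feed their animation Blueprints, and raise movement speed with crew size.
; Tick re-snaps the crew and updates a health bar facing the VR headset.
; Flaming arrows ignite it, draining health until it and its crew die.
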(event OnComponentHit(Mesh)
  (params (HitComponent :type Primitive%20Component%20Object%20Reference) (OtherActor :type Actor%20Object%20Reference) (OtherComp :type Primitive%20Component%20Object%20Reference) (NormalImpulse :type Vector :default "0, 0, 0") (Hit :type Hit%20Result%20Structure%20%28by%20ref%29))
  (bind _isactive_ (CallFunction|IsActive))
  (if _isactive_
    (bind _asbp_light_arrow (Utilities|Casting|CastToBP_LightArrow OtherActor))
    (if (Variables|/Game/Vive/Blueprints/BP_LightArrow.BP_LightArrow_C|GetOnFire _asbp_light_arrow)
      (Variables|Default|SetIsOnFire true))))

(event OnComponentBeginOverlap(SoldierOverlapCheck)
  (params (OverlappedComponent :type Primitive%20Component%20Object%20Reference) (OtherActor :type Actor%20Object%20Reference) (OtherComp :type Primitive%20Component%20Object%20Reference) (OtherBodyIndex :type Integer) (bFromSweep :type Boolean) (SweepResult :type Hit%20Result%20Structure%20%28by%20ref%29))
  (bind _isactive_ (CallFunction|IsActive))
  (bind _isnotfull (CallFunction|IsNotFull))
  (bind _asbp_siege_operator (Utilities|Casting|CastToBP_SiegeOperator OtherActor))
  (if (Math|Boolean|ANDBoolean _isnotfull _isactive_ (!= (Variables|/Game/Vive/Blueprints/AI/BP_SiegeOperator.BP_SiegeOperator_C|GetPreviousSiege _asbp_siege_operator) self))
    (bind _asbp_soldier_ai (Utilities|Casting|CastToBP_SoldierAI OtherActor))
    (Variables|/Game/Vive/Blueprints/AI/BP_SiegeOperator.BP_SiegeOperator_C|SetCurrentSiege _asbp_soldier_ai self)
    (Utilities|Array|AddUnique (Variables|Default|GetOperators) _asbp_soldier_ai)
    (Variables|/Game/Vive/Blueprints/AI/BP_SiegeOperator.BP_SiegeOperator_C|SetOperatorIndex _asbp_soldier_ai (Variables|Default|GetNextIndex))
    (Collision|SetCollisionEnabled (Variables|/Script/Engine.Character|GetMesh _asbp_soldier_ai) "NoCollision")
    (Transformation|AttachComponentToComponent _asbp_soldier_ai (Variables|Character|GetMesh) (Utilities|String|StringToName (Utilities|Array|Get(acopy) (Variables|Default|GetHandleStrings) (Variables|Default|GetNextIndex))) "SnapToTarget" "KeepRelative" "KeepWorld" false)
    (Collision|SetActorEnableCollision _asbp_soldier_ai false)
    (bind _asabp_soldier_unit (Utilities|Casting|CastToABP_SoldierUnit (Components|SkeletalMesh|GetAnimInstance (Variables|/Script/Engine.Character|GetMesh _asbp_soldier_ai))))
    (Variables|/Game/Vive/Blueprints/AI/SoldierAI/ABP_SoldierUnit.ABP_SoldierUnit_C|SetSiegeHandle _asabp_soldier_unit (Utilities|String|StringToName (Utilities|Array|Get(acopy) (Variables|Default|GetHandleStrings) (Variables|Default|GetNextIndex))))
    (if (== (Variables|Default|GetNextIndex) 0)
      (Variables|Default|SetNextIndex 1)
      (else
        (Variables|Default|SetNextIndex 0)))))

(event Custom|RemoveOperator
  (params (SiegeOperator :type BP%20Siege%20Operator%20Object%20Reference))
  (Utilities|Array|RemoveItem (Variables|Default|GetOperators) SiegeOperator)
  (Variables|Default|SetNextIndex (Variables|/Game/Vive/Blueprints/AI/BP_SiegeOperator.BP_SiegeOperator_C|GetOperatorIndex SiegeOperator)))

(event Custom|UpdateHealth
  (bind _healthbar (Variables|Default|GetHealthBar))
  ;[1 1 1] UpdateHealth (Using Tick Event)
  (if (<= (Variables|Default|GetHealth) 0.0)
    (for _array_element (Variables|Default|GetOperators)
      (Default|Seppuku _array_element))
    (Audio|PlaySoundatLocation "/Game/Audio/SFX/Voices/DeathVoices_Matt-25.DeathVoices_Matt-25" (Transformation|GetActorLocation))
    (CallFunction|Seppuku)
    (else
      (bind _ascatapult_health_bar (Utilities|Casting|CastToCatapultHealthBar (UserInterface|GetUserWidgetObject _healthbar)))
      (Transformation|SetWorldRotation _healthbar (Math|Rotator|FindLookatRotation (Transformation|GetWorldLocation _healthbar) (.DevicePosition (Class|HeadMountedDisplayFunctionLibrary|GetOrientationandPosition))) false false)
      (Progress|SetPercent (Variables|/Game/Vive/Blueprints/WidgetUI/CatapultHealthBar.CatapultHealthBar_C|GetProgressBar_143 _ascatapult_health_bar) (/ (Variables|Default|GetHealth) 1e+02))
      (if (Variables|Default|GetIsOnFire)
        (Variables|Default|SetHealth (- (Variables|Default|GetHealth) 0.1))
        (|SetFlamesToVisible)))))

(event Custom|UpdateSoldierAnimations
  ;[1 1 1] When Catapult Has Position Update Soldier Animation State Machines
  (if (Utilities|Enum|Equal(Enum) (Variables|Default|GetCurrentState) "NewEnumerator1")
    (for _array_element (Variables|Default|GetOperators)
      (bind _asabp_soldier_unit (Utilities|Casting|CastToABP_SoldierUnit (Components|SkeletalMesh|GetAnimInstance (Variables|/Script/Engine.Character|GetMesh _array_element))))
      (Variables|/Game/Vive/Blueprints/AI/SoldierAI/ABP_SoldierUnit.ABP_SoldierUnit_C|SetMountHandle _asabp_soldier_unit true))))

(event Custom|ResetSoldierRotations
  (for _array_element (Variables|Default|GetOperators)
    (Transformation|SetActorRotation _array_element (Transformation|GetActorRotation))))

(event Custom|ResetSoldierPositions
  (for (_array_element _array_index) (Variables|Default|GetOperators)
    (Transformation|SetActorLocation _array_element (Transformation|GetSocketLocation (Variables|Character|GetMesh) (Utilities|String|StringToName (Utilities|Array|Get(acopy) (Variables|Default|GetHandleStrings) _array_index))) false false)))

(event EventHitUnitwithArrow
  (params (AttackingArrow :type BP%20Base%20Arrow%20Object%20Reference) (HitLocation :type Vector :default "0, 0, 0") (HitComponent :type Scene%20Component%20Object%20Reference))
  (bind _onfire (Variables|/Game/Vive/Blueprints/BP_BaseArrow.BP_BaseArrow_C|GetOnFire AttackingArrow))
  (if _onfire
    (Variables|Default|SetIsOnFire _onfire)))

(event EventBeginPlay
  (|CallParentFunction)
  (bind _asbp_ai_controller (Utilities|Casting|CastToBP_AiController (Pawn|GetController)))
  (Variables|/Game/Vive/Blueprints/AI/BP_AiController.BP_AiController_C|SetBehaviourTree _asbp_ai_controller "/Game/Nathan/BT/Siege/BT_Siege.BT_Siege"))

(event EventTick
  (params (DeltaSeconds :type Float%20%28single-precision%29))
  (bind _isactive_ (CallFunction|IsActive))
  (if _isactive_
    (CallFunction|UpdateHealth)
    (CallFunction|ResetSoldierPositions)
    (CallFunction|ResetSoldierRotations)
    (switch int (Utilities|Array|Length (Variables|Default|GetOperators))
      (:1
        (Variables|/Script/Engine.CharacterMovementComponent|SetMaxWalkSpeed (Variables|Character|GetCharacterMovement) 2e+02))
      (:2
        (Variables|/Script/Engine.CharacterMovementComponent|SetMaxWalkSpeed (Variables|Character|GetCharacterMovement) 4e+02)))))

(fn ConstructionScript
  (|CallParentFunction))

(fn HasOperators
  (return (> (Utilities|Array|Length (Variables|Default|GetOperators)) 0)))

(fn IsFull
  (return (== (Utilities|Array|Length (Variables|Default|GetOperators)) 2)))

(fn IsNotFull
  (bind _isfull (CallFunction|IsFull))
  (return (not _isfull)))