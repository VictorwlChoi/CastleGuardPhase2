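; BP_SiegeOperator is an AI unit that serves as an operator of a siege.
; On BeginPlay it assigns the BT_SiegeOperator behaviour tree to its AI controller.
; LeaveSiege unregisters it, detaches the siege's mesh, teleports the operator to its detach point, and restores collision and animation flags; Seppuku also unregisters it.
; Tick copies CurrentState into the soldier anim instance, while the siege overlap handler only casts.
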(event Custom|LeaveSiege
  (Default|RemoveOperator (Variables|Default|GetCurrentSiege) self)
  (Transformation|DetachFromComponent (Variables|/Script/Engine.Character|GetMesh (Variables|Default|GetCurrentSiege)) "KeepWorld" "KeepWorld" "KeepWorld" false)
  (Transformation|SetActorLocation (Transformation|GetWorldLocation (Utilities|Array|Get(acopy) (Variables|/Game/Vive/Blueprints/AI/BP_Siege.BP_Siege_C|GetDetachPoints (Variables|Default|GetCurrentSiege)) (Variables|Default|GetOperatorIndex))) false true)
  (Collision|SetCollisionEnabled (Variables|Character|GetMesh) "QueryAndPhysics")
  (Collision|SetActorEnableCollision true)
  (bind _asabp_soldier_unit (Utilities|Casting|CastToABP_SoldierUnit (Components|SkeletalMesh|GetAnimInstance (Variables|Character|GetMesh))))
  (Variables|/Game/Vive/Blueprints/AI/SoldierAI/ABP_SoldierUnit.ABP_SoldierUnit_C|SetSiegeHandle _asabp_soldier_unit "None")
  (Variables|/Game/Vive/Blueprints/AI/SoldierAI/ABP_SoldierUnit.ABP_SoldierUnit_C|SetIsAtHandle _asabp_soldier_unit false)
  (Variables|Default|SetPreviousSiege (Variables|Default|GetCurrentSiege))
  (Variables|Default|SetCurrentSiege 0))

(event EventSeppuku
  (bind _currentsiege (Variables|Default|GetCurrentSiege))
  (Utilities|IsValid _currentsiege
    (:Is%20Valid
      (Default|RemoveOperator _currentsiege self))
    (:Is%20Not%20Valid
      _))
  (|CallParentFunction))

(event EventBeginPlay
  (|CallParentFunction)
  (bind _asbp_ai_controller (Utilities|Casting|CastToBP_AiController (Pawn|GetController)))
  (Variables|/Game/Vive/Blueprints/AI/BP_AiController.BP_AiController_C|SetBehaviourTree _asbp_ai_controller "/Game/Nathan/BT/SiegeOperator/BT_SiegeOperator.BT_SiegeOperator"))

(event Collision|EventActorBeginOverlap
  (params (OtherActor :type Actor%20Object%20Reference))
  (Utilities|Casting|CastToBP_Siege OtherActor))

(event EventTick
  (params (DeltaSeconds :type Float%20%28single-precision%29))
  ;[1 1 1] Important For Animation
  (|CallParentFunction DeltaSeconds)
  (bind _asabp_soldier_unit (Utilities|Casting|CastToABP_SoldierUnit (Components|SkeletalMesh|GetAnimInstance (Variables|Character|GetMesh))))
  (Variables|/Game/Vive/Blueprints/AI/SoldierAI/ABP_SoldierUnit.ABP_SoldierUnit_C|SetEnemyState _asabp_soldier_unit (Variables|Default|GetCurrentState)))

(fn ConstructionScript
  (|CallParentFunction))