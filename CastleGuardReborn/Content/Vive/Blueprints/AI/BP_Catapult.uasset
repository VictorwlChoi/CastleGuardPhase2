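; AI siege catapult that soldiers crew and push toward an attack position in a VR battle.
; Overlapping soldiers snap to two handle sockets, and crew count sets speed as it heads for FirstPos, then a free FinalLocation.
; Tick aligns it to ground and target, turns its health bar to the headset and drains health once flaming arrows ignite it.
; Death removes catapult and crew from the Overlord's units; destruction frees any held position.
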(event OnComponentBeginOverlap(SoldierOverlapCheck)
  (params (OverlappedComponent :type Primitive%20Component%20Object%20Reference) (OtherActor :type Actor%20Object%20Reference) (OtherComp :type Primitive%20Component%20Object%20Reference) (OtherBodyIndex :type Integer) (bFromSweep :type Boolean) (SweepResult :type Hit%20Result%20Structure%20%28by%20ref%29))
  (bind _handlestring2 (Variables|Default|GetHandleString2))
  (bind _handlestring1 (Variables|Default|GetHandleString1))
  ;[1 1 1] Checking for someone manning Catapult & Attach Soldier if there isn't
  (bind _asbp_soldier_ai (Utilities|Casting|CastToBP_SoldierAI OtherActor))
  (Variables|/Game/Vive/Blueprints/AI/SoldierAIHeavy/BP_SoldierAI.BP_SoldierAI_C|SetCatapult _asbp_soldier_ai (Variables|Default|GetNextCatapult))
  (if (not (Variables|Default|GetHandleBool2))
    (if (Variables|Default|GetHandleBool1)
      (Variables|Default|SetHandleBool2 true)
      (Development|PrintString _handlestring2)
      (Transformation|AttachComponentToComponent OtherActor (Variables|Default|GetStaticMesh) (Utilities|String|StringToName _handlestring2) "SnapToTarget" "SnapToTarget" "KeepWorld" false)
      (Variables|Default|SetIsFull? true)
      (Collision|SetActorEnableCollision OtherActor false)
      (bind _asbp_soldier_ai_2 (Utilities|Casting|CastToBP_SoldierAI OtherActor))
      (Variables|Default|SetSoldier2 _asbp_soldier_ai_2)
      (else
        (Variables|Default|SetHandleBool1 true)
        (Development|PrintString _handlestring1)
        (Transformation|AttachComponentToComponent OtherActor (Variables|Default|GetStaticMesh) (Utilities|String|StringToName _handlestring1) "SnapToTarget" "SnapToTarget" "KeepWorld" false)
        (Collision|SetActorEnableCollision OtherActor false)
        (bind _asbp_soldier_ai_3 (Utilities|Casting|CastToBP_SoldierAI OtherActor))
        (Variables|Default|SetSoldier1 _asbp_soldier_ai_3)))))

(event OnComponentHit(StaticMesh)
  (params (HitComponent :type Primitive%20Component%20Object%20Reference) (OtherActor :type Actor%20Object%20Reference) (OtherComp :type Primitive%20Component%20Object%20Reference) (NormalImpulse :type Vector :default "0, 0, 0") (Hit :type Hit%20Result%20Structure%20%28by%20ref%29))
  (bind _asbp_heavy_arrow (Utilities|Casting|CastToBP_HeavyArrow OtherActor)
    (:then
      (if (Variables|/Game/Vive/Blueprints/BP_HeavyArrow.BP_HeavyArrow_C|GetOnFire _asbp_heavy_arrow)
        (Variables|Default|SetIsOnFire true)))
    (:CastFailed
      (bind _asbp_light_arrow (Utilities|Casting|CastToBP_LightArrow OtherActor))
      (if (Variables|/Game/Vive/Blueprints/BP_LightArrow.BP_LightArrow_C|GetOnFire _asbp_light_arrow)
        (Variables|Default|SetIsOnFire true)))))

(event OnComponentBeginOverlap(CapsuleComponent)
  (params (OverlappedComponent :type Primitive%20Component%20Object%20Reference) (OtherActor :type Actor%20Object%20Reference) (OtherComp :type Primitive%20Component%20Object%20Reference) (OtherBodyIndex :type Integer) (bFromSweep :type Boolean) (SweepResult :type Hit%20Result%20Structure%20%28by%20ref%29))
  ;[1 1 1] Moving AI
  (Utilities|Casting|CastToBP_CatapultAttackPositions OtherActor)
  (Variables|Default|SetHasPosition true))

(event Custom|Tick
  ;[1 1 1] Checking for someone manning Catapult & Attach Soldier if there isn't
  (if (Variables|Default|GetHandleBool1)
    (if (Variables|Default|GetHandleBool2)
      (Variables|/Script/Engine.CharacterMovementComponent|SetMaxWalkSpeed (Variables|Character|GetCharacterMovement) 4e+02)
      (AI|AIMoveTo self "0, 0, 0" (Variables|Default|GetFirstPos) 5.0 false)
      (else
        (Variables|/Script/Engine.CharacterMovementComponent|SetMaxWalkSpeed (Variables|Character|GetCharacterMovement) 2e+02)
        (AI|AIMoveTo self "0, 0, 0" (Variables|Default|GetFirstPos) 5.0 false)))))

(event EventTick
  (params (DeltaSeconds :type Float%20%28single-precision%29))
  (bind _capsulecomponent (Variables|Collision|GetCapsuleComponent))
  (bind _firstpos (Variables|Default|GetFirstPos))
  (bind _returnvalue (Transformation|GetActorTransform _firstpos))
  (bind _returnvalue_2 (Transformation|GetWorldLocation _capsulecomponent))
  (bind _location (Math|Transform|BreakTransform _returnvalue))
  (bind _returnvalue_3 (Math|Rotator|FindLookatRotation _returnvalue_2 _location))
  (bind (_roll _pitch _yaw) (Math|Rotator|BreakRotator _returnvalue_3))
  (bind _outhit (Collision|LineTraceByChannel _returnvalue_2 (+ _returnvalue_2 "0, 0,-100.000000") "TraceTypeQuery1" true 0 "None"))
  (if (Variables|/Game/Vive/Blueprints/AI/BP_SiegePathStops.BP_SiegePathStops_C|GetCatapultLastStop (Variables|Default|GetFirstPos))
    (Transformation|SetActorRotation (Math|Rotator|MakeRotator (.Roll (Math|Rotator|BreakRotator (Math|Rotator|FindLookatRotation _returnvalue_2 (.Location (Math|Transform|BreakTransform (Transformation|GetActorTransform (Variables|Default|GetFinalLocation))))))) (.Pitch (Math|Rotator|BreakRotator (Math|Rotator|MakeRotfromY (.Normal (Collision|BreakHitResult _outhit))))) (.Yaw (Math|Rotator|BreakRotator (Math|Rotator|FindLookatRotation _returnvalue_2 (.Location (Math|Transform|BreakTransform (Transformation|GetActorTransform (Variables|Default|GetFinalLocation)))))))) true)
    (else
      (Transformation|SetActorRotation (Math|Rotator|MakeRotator _roll (.Pitch (Math|Rotator|BreakRotator (Math|Rotator|MakeRotfromY (.Normal (Collision|BreakHitResult _outhit))))) _yaw) true)))
  ;[1 1 1] UpdateHealth (Using Tick Event)
  (CallFunction|Tick)
  (if (<= (Variables|Default|GetHealth) 0.0)
    (bind _outactors (Actor|GetAllActorsOfClass "/Game/Vive/Blueprints/Overlords/BP_Overlord_Master.BP_Overlord_Master_C"))
    (Utilities|Array|RemoveItem (Variables|/Game/Vive/Blueprints/Overlords/BP_Overlord_Master.BP_Overlord_Master_C|GetUnitArray (Utilities|Array|Get(acopy) _outactors)) (Variables|Default|GetSoldier1))
    (Actor|DestroyActor (Variables|Default|GetSoldier1))
    (Utilities|Array|RemoveItem (Variables|/Game/Vive/Blueprints/Overlords/BP_Overlord_Master.BP_Overlord_Master_C|GetUnitArray (Utilities|Array|Get(acopy) _outactors)) (Variables|Default|GetSoldier2))
    (Actor|DestroyActor (Variables|Default|GetSoldier2))
    (Utilities|Array|RemoveItem (Variables|/Game/Vive/Blueprints/Overlords/BP_Overlord_Master.BP_Overlord_Master_C|GetUnitArray (Utilities|Array|Get(acopy) _outactors)) self)
    (Audio|PlaySoundatLocation 0 (Transformation|GetActorLocation))
    (Actor|DestroyActor)
    (else
      (bind _ascatapult_health_bar (Utilities|Casting|CastToCatapultHealthBar (UserInterface|GetUserWidgetObject (Variables|Default|GetCatapultHealthBarComponent))))
      (Transformation|SetWorldRotation (Variables|Default|GetCatapultHealthBarComponent) (Math|Rotator|FindLookatRotation (Transformation|GetWorldLocation (Variables|Default|GetCatapultHealthBarComponent)) (.DevicePosition (Class|HeadMountedDisplayFunctionLibrary|GetOrientationandPosition))) false false)
      (Progress|SetPercent (Variables|/Game/Vive/Blueprints/WidgetUI/CatapultHealthBar.CatapultHealthBar_C|GetProgressBar_143 _ascatapult_health_bar) (/ (Variables|Default|GetHealth) 1e+02))
      (if (Variables|Default|GetIsOnFire)
        (Variables|Default|SetHealth (- (Variables|Default|GetHealth) 0.1)))
      ;[1 1 1] Moving AI
      (if (Variables|Default|GetIsFull?)
        (if (Variables|Default|GetHasPosition)
          (Variables|/Script/Engine.CharacterMovementComponent|SetMaxWalkSpeed (Variables|Character|GetCharacterMovement) 0.0)
          (elif (Variables|/Game/Vive/Blueprints/AI/BP_SiegePathStops.BP_SiegePathStops_C|GetCatapultLastStop (Variables|Default|GetFirstPos))
            (if (Variables|/Game/Vive/Blueprints/AI/BP_CatapultAttackPositions.BP_CatapultAttackPositions_C|GetPositionTaken (Variables|Default|GetFinalLocation))
              (AI|AIMoveTo self "0, 0, 0" (Variables|/Game/Vive/Blueprints/AI/BP_CatapultAttackPositions.BP_CatapultAttackPositions_C|GetNextPosition (Variables|Default|GetFinalLocation)) 5.0 true
                (:then
                  (Development|PrintString "Position is taken, cycle through next")
                  (Variables|Default|SetFinalLocation (Variables|/Game/Vive/Blueprints/AI/BP_CatapultAttackPositions.BP_CatapultAttackPositions_C|GetNextPosition (Variables|Default|GetFinalLocation)))))
              (else
                (AI|AIMoveTo self "0, 0, 0" (Variables|Default|GetFinalLocation) 5.0 true)))))))))

(event EventDestroyed
  (bind _finallocation (Variables|Default|GetFinalLocation))
  ;[1 1 1] Moving AI
  (if (Variables|Default|GetHasPosition)
    (Variables|/Game/Vive/Blueprints/AI/BP_CatapultAttackPositions.BP_CatapultAttackPositions_C|SetPositionTaken _finallocation false)
    (Variables|/Game/Vive/Blueprints/AI/BP_CatapultAttackPositions.BP_CatapultAttackPositions_C|SetTimer _finallocation 0.0)))

(fn ConstructionScript
  (Variables|Default|SetHandleBool1 false)
  (Variables|Default|SetHandleString1 "Handle1")
  (Variables|Default|SetHandleString2 "Handle2")
  (Variables|Default|SetHandleBool2 false))

(fn ReturnCatapultBools
  (return (Variables|Default|GetHasPosition) (Variables|Default|GetHandleBool1) (Variables|Default|GetHandleBool2)))

(fn PrinttoVive
  (params (String%20In :type String))
  (Development|PrintString String%20In)
  (Development|PrintString String%20In)
  (Development|PrintString String%20In)
  (Development|PrintString String%20In)
  (Development|PrintString String%20In)
  (Development|PrintString String%20In)
  (Development|PrintString String%20In)
  (Development|PrintString String%20In)
  (Development|PrintString String%20In)
  (Development|PrintString String%20In)
  (Development|PrintString String%20In)
  (Development|PrintString String%20In)
  (Development|PrintString String%20In)
  (Development|PrintString String%20In)
  (Development|PrintString String%20In)
  (Development|PrintString String%20In))

(fn CatapultChainAudio
  (params (CatapultPositionIn :type Vector))
  (bind _returnvalue (Math|Random|RandomInteger 0))
  (if (== _returnvalue 0)
    (Audio|SpawnSoundAttached 0 (Variables|Default|GetChainAudio1) "None" CatapultPositionIn)
    (elif (== _returnvalue 0)
      _)))