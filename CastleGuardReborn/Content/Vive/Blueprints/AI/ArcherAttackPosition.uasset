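; Attack position marker for archer AI that fires arrows while an archer stands inside its box.
; An ArcherAi entering the box gets its HasPosition flag set and marks the spot taken; leaving frees the spot and resets the timer.
; While taken, Tick spawns an ArcherAIArrow every two seconds above the marker, aimed by the marker's own rotation rather than the archer's.
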(event OnComponentBeginOverlap(Box)
  (params (OverlappedComponent :type Primitive%20Component%20Object%20Reference) (OtherActor :type Actor%20Object%20Reference) (OtherComp :type Primitive%20Component%20Object%20Reference) (OtherBodyIndex :type Integer) (bFromSweep :type Boolean) (SweepResult :type Hit%20Result%20Structure%20%28by%20ref%29))
  (bind _asarcher_ai (Utilities|Casting|CastToArcherAi OtherActor))
  (Variables|/Game/Vive/Blueprints/AI/ArcherAi.ArcherAi_C|SetHasPosition _asarcher_ai true)
  (Variables|Default|SetPositionTaken true))

(event OnComponentEndOverlap(Box)
  (params (OverlappedComponent :type Primitive%20Component%20Object%20Reference) (OtherActor :type Actor%20Object%20Reference) (OtherComp :type Primitive%20Component%20Object%20Reference) (OtherBodyIndex :type Integer))
  (Utilities|Casting|CastToArcherAi OtherActor)
  (Development|PrintString "End Overlap")
  (Variables|Default|SetPositionTaken false)
  (Variables|Default|SetTimer 0.0))

(event EventTick
  (params (DeltaSeconds :type Float%20%28single-precision%29))
  (if (Variables|Default|GetPositionTaken)
    (Variables|Default|SetTimer (+ DeltaSeconds (Variables|Default|GetTimer)))
    (if (>= (Variables|Default|GetTimer) 2.0)
      (Variables|Default|SetTimer 0.0)
      (Game|SpawnActorfromClass "/Game/Vive/Blueprints/AI/ArcherAIArrow.ArcherAIArrow_C" (Math|Transform|MakeTransform (+ (Transformation|GetActorLocation) "0, 0,200.000000") (Transformation|GetActorRotation)) "Undefined" 0 0))))

(fn ConstructionScript)