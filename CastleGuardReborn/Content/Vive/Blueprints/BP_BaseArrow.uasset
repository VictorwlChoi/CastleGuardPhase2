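; BP_BaseArrow is the base arrow projectile for a Vive VR game with AI targets.
; In flight, Tick points the mesh along its velocity and scales it by distance from the Vive pawn, then starts a short lifespan once motion stops.
; Overlapping a brazier's fire collision flags it as on fire.
; Hits on AI characters notify them, attach the arrow and halt it, while landscape hits play a random impact sound.
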(event Collision|EventHit
  (params (MyComp :type Primitive%20Component%20Object%20Reference) (Other :type Actor%20Object%20Reference) (OtherComp :type Primitive%20Component%20Object%20Reference) (bSelfMoved :type Boolean) (HitLocation :type Vector :default "0, 0, 0") (HitNormal :type Vector :default "0, 0, 0") (NormalImpulse :type Vector :default "0, 0, 0") (Hit :type Hit%20Result%20Structure%20%28by%20ref%29))
  (bind _groundimpactsounds (Variables|Default|GetGroundImpactSounds))
  (bind _projectilemovement (Variables|Default|GetProjectileMovement))
  ;[0.622 0 1] Handle Collision
  (bind _asai_character (Utilities|Casting|CastToAiCharacter Other)
    (:then
      (Class|IAttackable|HitUnitwithArrow(Message) _asai_character self HitLocation OtherComp)
      (Transformation|AttachComponentToComponent (Variables|Default|GetScene) (Variables|/Script/Engine.Actor|GetRootComponent Other) "None" "KeepWorld" "KeepWorld" "KeepWorld" true)
      (Components|Movement|StopMovementImmediately _projectilemovement)
      (Variables|/Script/Engine.ProjectileMovementComponent|SetMaxSpeed _projectilemovement 0.0)
      (Variables|/Script/Engine.ProjectileMovementComponent|SetProjectileGravityScale _projectilemovement 0.0))
    (:CastFailed
      (Utilities|Casting|CastToLandscape Other)
      (Audio|PlaySoundatLocation (Utilities|Array|Get(acopy) _groundimpactsounds (Math|Random|RandomInteger (Utilities|Array|Length _groundimpactsounds))) (Variables|Default|GetArrowHitLocation)))))

(event EventDestroyed)

(event Collision|EventActorBeginOverlap
  (params (OtherActor :type Actor%20Object%20Reference))
  ;[1 0.2942 0] Light Arrow on Fire
  (bind _asbrazier (Utilities|Casting|CastToBrazier OtherActor))
  (if (Class|PrimitiveComponent|IsOverlappingComponent (Variables|/Game/Vive/Blueprints/Brazier.Brazier_C|GetFireCollision _asbrazier) (Variables|Default|GetStaticMesh))
    (Variables|Default|SetOnFire true)))

(event EventTick
  (params (DeltaSeconds :type Float%20%28single-precision%29))
  (bind _maxscale (Variables|Default|GetMaxScale))
  (bind _projectilemovement (Variables|Default|GetProjectileMovement))
  (bind _velocity (Variables|/Script/Engine.MovementComponent|GetVelocity _projectilemovement))
  (bind _returnvalue (Math|Vector|Normalize _velocity))
  (bind _returnvalue_2 (Math|Conversions|RotationFromXVector _returnvalue))
  (bind (_roll _pitch _yaw) (Math|Rotator|BreakRotator _returnvalue_2))
  ;[0 0.6874 1] Tick
  (Transformation|SetWorldRotation (Variables|Default|GetScene1) "0, 0, 0" false false)
  (if (Variables|Default|GetInFlight)
    (bind _output_get (Variables|Default|SetInFlight (Math|Vector|NotEqual(Vector) _velocity "0, 0, 0" 0.0001)))
    (if _output_get
      (Transformation|SetWorldRotation (Variables|Default|GetStaticMesh) (Math|Rotator|MakeRotator _roll (+ _pitch 9e+01) _yaw) false false)
      (bind _outactors (Actor|GetAllActorsOfClass "/Game/Vive/Blueprints/BP_Vive_Pawn.BP_Vive_Pawn_C"))
      (if (> (Utilities|Array|Length _outactors) 0)
        (Transformation|SetWorldScale3D (Variables|Default|GetStaticMesh) (Math|Vector|Lerp(Vector) "1.000000,1.000000,1.000000" (Math|Vector|MakeVector _maxscale _maxscale _maxscale) (/ (Math|Vector|VectorLength (- (Transformation|GetActorLocation (Utilities|Array|Get(acopy) _outactors)) (Transformation|GetActorLocation))) (Variables|Default|GetMaxDistance)))))
      (else
        (Actor|SetLifeSpan 1.0)))))

(event EventBeginPlay
  ;[0 0.6927 0.05965] Initialize
  (Components|Movement|SetUpdatedComponent (Variables|Default|GetProjectileMovement) (Variables|Default|GetStaticMesh))
  (Variables|Default|SetInFlight false)
  (Variables|Default|SetHit false)
  (Variables|Default|SetSocketFlame "Flame")
  (Variables|Default|SetSocketTrail "Trail"))

(fn ConstructionScript)

(fn PrinttoVive
  (params (String%20In :type String))
  (Development|PrintString String%20In)
  (Development|PrintString String%20In)
  (Development|PrintString String%20In)
  (Development|PrintString String%20In)
  (Development|PrintString String%20In)
  (Development|PrintString String%20In)
  (Development|PrintString String%20In)
  (Development|PrintString String%20In)
  (Development|PrintString String%20In)
  (Development|PrintString String%20In)
  (Development|PrintString String%20In)
  (Development|PrintString String%20In)
  (Development|PrintString String%20In)
  (Development|PrintString String%20In)
  (Development|PrintString String%20In)
  (Development|PrintString String%20In))