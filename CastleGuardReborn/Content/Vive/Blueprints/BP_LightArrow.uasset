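; BP_LightArrow is an arrow Blueprint whose only hit-response logic is marked deprecated and never runs.
; That disconnected graph casts an unconnected object to siege engines, unit AIs or Landscape.
; Its branches would set rams and catapults on fire, remove light soldiers and archers from UnitArray, or play sounds.
; The construction script is empty, so the Blueprint has no active graph behavior.
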(fn ConstructionScript)