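; Wave overlord that spawns enemy soldiers, archers, battering rams and catapults along two attack paths.
; Once UnitArray is empty, Tick waits out a timer, then reads the next WaveData row and calls per-unit spawn functions with each path's counts and points.
; Siege weapons spawn with light soldier escorts, and TempCatapult and TempRam link heavy soldiers to them.
; Several spawn loops mishandle their counts, and the CustomEvents spawners are marked useless.
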(event EventBeginPlay)

(event Collision|EventActorBeginOverlap
  (params (OtherActor :type Actor%20Object%20Reference)))

(event EventTick
  (params (DeltaSeconds :type Float%20%28single-precision%29))
  (if (Variables|Default|GetIsWaveComplete)
    (bind _output_get (Variables|Default|SetWaveTimer (+ DeltaSeconds (Variables|Default|GetWaveTimer))))
    (if (>= _output_get 15.0)
      (Variables|Default|SetIsWaveComplete false)
      (Variables|Default|SetCurrentWave (+ (Variables|Default|GetCurrentWave) 1))
      (bind _outrownames (DataTable|GetDataTableRowNames (Variables|Default|GetWaveData)))
      (bind _output_get_2 (Variables|Default|SetWaveNames _outrownames))
      (bind _returnvalue (Utilities|GetDataTableRow (Variables|Default|GetWaveData) (Utilities|Array|Get(acopy) _output_get_2 (Variables|Default|GetCurrentWave)))
        (:then
          (CallFunction|SpawnLightSoldier (.Path1LightSoldierCount (Utilities|Struct|BreakWaveInfo _returnvalue)) (Variables|Default|GetSoldierAttackPosition1) (Variables|Default|GetSoldierSpawnpoint1) (Variables|Default|GetSoldierStartPoint1))
          (CallFunction|SpawnSoldier (.Path1HeavySoldierCount (Utilities|Struct|BreakWaveInfo _returnvalue)) (Variables|Default|GetSoldierSpawnpoint1) (Variables|Default|GetSoldierStartPoint1) (Variables|Default|GetSoldierAttackPosition1))
          (CallFunction|SpawnRam (.Path1BatteringRamCount (Utilities|Struct|BreakWaveInfo _returnvalue)) (Variables|Default|GetTempRam) (Variables|Default|GetSiegeStartPoint1) (Variables|Default|GetSiegeSpawnpoint1) (Variables|Default|GetRamAttackPosition1) (Variables|Default|GetSoldierAttackPosition1) (Variables|Default|GetSoldierSpawnpoint1) (Variables|Default|GetSoldierStartPoint1))
          (CallFunction|SpawnCatapult (.Path1CatapultCount (Utilities|Struct|BreakWaveInfo _returnvalue)) (Variables|Default|GetTempCatapult) (Variables|Default|GetSiegeStartPoint1) (Variables|Default|GetSiegeSpawnpoint1) (Variables|Default|GetCatapultAttackPosition1) (Variables|Default|GetSoldierAttackPosition1) (Variables|Default|GetSoldierSpawnpoint1) (Variables|Default|GetSoldierStartPoint1))
          (CallFunction|SpawnArcher (.Path1ArcherCount (Utilities|Struct|BreakWaveInfo _returnvalue)) (Variables|Default|GetArcherSpawnPoint1) (Variables|Default|GetArcherStartPoint1) (Variables|Default|GetArcherAttackPosition1))
          (CallFunction|SpawnLightSoldier (.Path2LightSoldierCount (Utilities|Struct|BreakWaveInfo _returnvalue)) (Variables|Default|GetSoldierAttackPosition2) (Variables|Default|GetSoldierSpawnpoint2) (Variables|Default|GetSoldierStartPoint2))
          (CallFunction|SpawnSoldier (.Path2HeavySoldierCount (Utilities|Struct|BreakWaveInfo _returnvalue)) (Variables|Default|GetSoldierSpawnpoint2) (Variables|Default|GetSoldierStartPoint2) (Variables|Default|GetSoldierAttackPosition2))
          (CallFunction|SpawnRam (.Path2BatteringRamCount (Utilities|Struct|BreakWaveInfo _returnvalue)) (Variables|Default|GetTempRam) (Variables|Default|GetSiegeStartPoint2) (Variables|Default|GetSiegeSpawnpoint2) (Variables|Default|GetRamAttackPosition2) (Variables|Default|GetSoldierAttackPosition2) (Variables|Default|GetSoldierSpawnpoint2) (Variables|Default|GetSoldierStartPoint2))
          (CallFunction|SpawnCatapult (.Path2CatapultCount (Utilities|Struct|BreakWaveInfo _returnvalue)) (Variables|Default|GetTempCatapult) (Variables|Default|GetSiegeStartPoint2) (Variables|Default|GetSiegeSpawnpoint2) (Variables|Default|GetCatapultAttackPosition2))
          (CallFunction|SpawnArcher (.Path2ArcherCount (Utilities|Struct|BreakWaveInfo _returnvalue))))))
    (elif (== (Utilities|Array|Length (Variables|Default|GetUnitArray)) 0)
      (Variables|Default|SetIsWaveComplete true)
      (Variables|Default|SetWaveTimer 0.0))))

(event Custom|SpawnRamUnit
  (params (FirstPositionIn :type BP%20Siege%20Path%20Stops%20Object%20Reference) (SpawnPointIn :type Actor%20Object%20Reference) (AttackPositionIn :type BP%20Battering%20Ram%20Attack%20Position%20Object%20Reference) (NextRamIn :type BP%20Battering%20Ram%20Old%20Object%20Reference))
  ;[1 1 1] All these are useless
  ;;[1 1 1] Spawn a Battering Ram
  (bind _returnvalue (Game|SpawnActorfromClass "/Game/Vive/Blueprints/AI/BP_BatteringRamOld.BP_BatteringRamOld_C" (Transformation|GetActorTransform SpawnPointIn) "Undefined" 0 0))
  (Utilities|Array|Add (Variables|Default|GetUnitArray) _returnvalue)
  (Variables|/Game/Vive/Blueprints/AI/BP_BatteringRamOld.BP_BatteringRamOld_C|SetAttackPos _returnvalue AttackPositionIn)
  (Variables|/Game/Vive/Blueprints/AI/BP_BatteringRamOld.BP_BatteringRamOld_C|SetFirstPos _returnvalue FirstPositionIn)
  (Variables|Default|SetTempRam _returnvalue)
  (if (Utilities|IsValid NextRamIn)
    (Variables|/Game/Vive/Blueprints/AI/BP_BatteringRamOld.BP_BatteringRamOld_C|SetNextRam _returnvalue NextRamIn)))

(event Custom|SpawnHeavySoldierUnit
  (params (SpawnPointIn :type Actor%20Object%20Reference) (FirstStopIn :type BP%20Soldier%20Path%20Stops%20Object%20Reference) (AttackPositionIn :type BP%20Soldier%20Attack%20Position%20Object%20Reference))
  ;[1 1 1] All these are useless
  ;;[1 1 1] Spawn Heavy Soldier and Check for a Siege weapon
  (bind _returnvalue (Game|SpawnActorfromClass "/Game/Vive/Blueprints/AI/SoldierAIHeavy/BP_SoldierAI.BP_SoldierAI_C" (Transformation|GetActorTransform SpawnPointIn) "Undefined" 0 0))
  (Utilities|Array|Add (Variables|Default|GetUnitArray) _returnvalue)
  (Variables|/Game/Vive/Blueprints/AI/SoldierAIHeavy/BP_SoldierAI.BP_SoldierAI_C|SetFirstStop _returnvalue FirstStopIn)
  (Variables|/Game/Vive/Blueprints/AI/SoldierAIHeavy/BP_SoldierAI.BP_SoldierAI_C|SetAttackPos _returnvalue AttackPositionIn)
  (if (Utilities|IsValid (Variables|Default|GetTempCatapult))
    (bind _output_get (Variables|/Game/Vive/Blueprints/AI/SoldierAIHeavy/BP_SoldierAI.BP_SoldierAI_C|SetCatapult _returnvalue (Variables|Default|GetTempCatapult)))
    (if (Variables|/Game/Vive/Blueprints/AI/BP_Catapult.BP_Catapult_C|GetIsFull? _output_get)
      (Variables|Default|SetTempCatapult 0))
    (elif (Utilities|IsValid (Variables|Default|GetTempRam))
      (bind _output_get_2 (Variables|/Game/Vive/Blueprints/AI/SoldierAIHeavy/BP_SoldierAI.BP_SoldierAI_C|SetBatteringRam _returnvalue (Variables|Default|GetTempRam)))
      (if (Variables|/Game/Vive/Blueprints/AI/BP_BatteringRamOld.BP_BatteringRamOld_C|GetIsFull? _output_get_2)
        (Variables|Default|SetTempRam 0)))))

(event Custom|SpawnArcherUnit
  (params (FirstStopIn :type BP%20Archer%20Path%20Stops%20Object%20Reference) (SpawnPointIn :type Actor%20Object%20Reference) (AttackPositionIn :type BP%20Archer%20Attack%20Position%20Object%20Reference))
  ;[1 1 1] All these are useless
  ;;[1 1 1] Spawn Archer
  (bind _returnvalue (Game|SpawnActorfromClass "/Game/Vive/Blueprints/AI/ArcherAI/BP_ArcherAi.BP_ArcherAi_C" (Transformation|GetActorTransform SpawnPointIn) "Undefined" 0 0))
  (Utilities|Array|Add (Variables|Default|GetUnitArray) _returnvalue)
  (Variables|/Game/Vive/Blueprints/AI/ArcherAI/BP_ArcherAi.BP_ArcherAi_C|SetFirstStop _returnvalue FirstStopIn)
  (Variables|/Game/Vive/Blueprints/AI/ArcherAI/BP_ArcherAi.BP_ArcherAi_C|SetAttackPosition _returnvalue AttackPositionIn))

(event Custom|SpawnLightSoldierUnit
  (params (AttackPositionIn :type BP%20Soldier%20Attack%20Position%20Object%20Reference) (SpawnpointIn :type Actor%20Object%20Reference) (FirstStopIn :type BP%20Soldier%20Path%20Stops%20Object%20Reference))
  ;[1 1 1] All these are useless
  ;;[1 1 1] Spawn Light Soldier Unit
  (bind _returnvalue (Game|SpawnActorfromClass "/Game/Vive/Blueprints/AI/SoldierAILight/BP_LightSoldierAI.BP_LightSoldierAI_C" (Transformation|GetActorTransform SpawnpointIn) "Undefined" 0 0))
  (Utilities|Array|Add (Variables|Default|GetUnitArray) _returnvalue)
  (Variables|/Game/Vive/Blueprints/AI/SoldierAILight/BP_LightSoldierAI.BP_LightSoldierAI_C|SetFirstStop _returnvalue FirstStopIn)
  (Variables|/Game/Vive/Blueprints/AI/SoldierAILight/BP_LightSoldierAI.BP_LightSoldierAI_C|SetAttackPos _returnvalue AttackPositionIn))

(event Custom|SpawnCatapultUnit
  (params (NextCatapultIn :type BP%20Catapult%20Object%20Reference) (FirstLocationIn :type BP%20Siege%20Path%20Stops%20Object%20Reference) (SpawnPointIn :type Actor%20Object%20Reference) (AttackPositionIn :type BP%20Catapult%20Attack%20Positions%20Object%20Reference))
  ;[1 1 1] All these are useless
  ;;[1 1 1] Spawn Catapult
  (bind _returnvalue (Game|SpawnActorfromClass "/Game/Vive/Blueprints/AI/BP_Catapult.BP_Catapult_C" (Transformation|GetActorTransform SpawnPointIn) "Undefined" 0 0))
  (Utilities|Array|Add (Variables|Default|GetUnitArray) _returnvalue)
  (Variables|/Game/Vive/Blueprints/AI/BP_Catapult.BP_Catapult_C|SetFinalLocation _returnvalue AttackPositionIn)
  (Variables|/Game/Vive/Blueprints/AI/BP_Catapult.BP_Catapult_C|SetFirstPos _returnvalue FirstLocationIn)
  (Variables|Default|SetTempCatapult _returnvalue)
  (if (Utilities|IsValid NextCatapultIn)
    (Variables|/Game/Vive/Blueprints/AI/BP_Catapult.BP_Catapult_C|SetNextCatapult _returnvalue NextCatapultIn)))

(fn ConstructionScript)

(fn SpawnSoldier
  (params (SpawnCountIn :type Integer) (SpawnPoint :type Actor%20Object%20Reference) (FirstStopIn :type BP%20Soldier%20Path%20Stops%20Object%20Reference) (AttackPositionIn :type BP%20Soldier%20Attack%20Position%20Object%20Reference))
  (Variables|Default|SetHeavySoldierNumberOfSpawnsLeft SpawnCountIn)
  (bind _returnvalue (Game|SpawnActorfromClass "/Game/Vive/Blueprints/AI/SoldierAIHeavy/BP_SoldierAI.BP_SoldierAI_C" (Transformation|GetActorTransform SpawnPoint) "Undefined" 0 0 :!label _label))
  (Utilities|Array|Add (Variables|Default|GetUnitArray) _returnvalue)
  (Variables|/Game/Vive/Blueprints/AI/SoldierAIHeavy/BP_SoldierAI.BP_SoldierAI_C|SetFirstStop _returnvalue FirstStopIn)
  (Variables|/Game/Vive/Blueprints/AI/SoldierAIHeavy/BP_SoldierAI.BP_SoldierAI_C|SetAttackPos _returnvalue AttackPositionIn)
  (if (Utilities|IsValid (Variables|Default|GetTempCatapult))
    (bind _output_get (Variables|/Game/Vive/Blueprints/AI/SoldierAIHeavy/BP_SoldierAI.BP_SoldierAI_C|SetCatapult _returnvalue (Variables|Default|GetTempCatapult)))
    (if (Variables|/Game/Vive/Blueprints/AI/BP_Catapult.BP_Catapult_C|GetIsFull? _output_get)
      (Variables|Default|SetTempCatapult 0))
    (elif (Utilities|IsValid (Variables|Default|GetTempRam))
      (bind _output_get_2 (Variables|/Game/Vive/Blueprints/AI/SoldierAIHeavy/BP_SoldierAI.BP_SoldierAI_C|SetBatteringRam _returnvalue (Variables|Default|GetTempRam)))
      (if (Variables|/Game/Vive/Blueprints/AI/BP_BatteringRamOld.BP_BatteringRamOld_C|GetIsFull? _output_get_2)
        (Variables|Default|SetTempRam 0))))
  (bind _output_get_3 (Variables|Default|SetHeavySoldierNumberOfSpawnsLeft (- (Variables|Default|GetHeavySoldierNumberOfSpawnsLeft) 1)))
  (if (> _output_get_3 0)
    (goto _label)
    (else
      (return))))

(fn SpawnArcher
  (params (WaveCountIn :type Integer) (SpawnpointIn :type Actor%20Object%20Reference) (FirstStopIn :type BP%20Archer%20Path%20Stops%20Object%20Reference) (AttackPositionIn :type BP%20Archer%20Attack%20Position%20Object%20Reference))
  (bind _returnvalue (Game|SpawnActorfromClass "/Game/Vive/Blueprints/AI/ArcherAI/BP_ArcherAi.BP_ArcherAi_C" (Transformation|GetActorTransform SpawnpointIn) "Undefined" 0 0 :!label _label))
  (Utilities|Array|Add (Variables|Default|GetUnitArray) _returnvalue)
  (Variables|/Game/Vive/Blueprints/AI/ArcherAI/BP_ArcherAi.BP_ArcherAi_C|SetFirstStop _returnvalue FirstStopIn)
  (Variables|/Game/Vive/Blueprints/AI/ArcherAI/BP_ArcherAi.BP_ArcherAi_C|SetAttackPosition _returnvalue AttackPositionIn)
  (if (> WaveCountIn 0)
    (goto _label)))

(fn SpawnLightSoldier
  (params (WaveCountIn :type Integer) (AttackPositionIn :type BP%20Soldier%20Attack%20Position%20Object%20Reference) (SpawnPointIn :type Actor%20Object%20Reference) (FirstStopIn :type BP%20Soldier%20Path%20Stops%20Object%20Reference))
  (bind _returnvalue (Game|SpawnActorfromClass "/Game/Vive/Blueprints/AI/SoldierAILight/BP_LightSoldierAI.BP_LightSoldierAI_C" (Transformation|GetActorTransform SpawnPointIn) "Undefined" 0 0 :!label _label))
  (Utilities|Array|Add (Variables|Default|GetUnitArray) _returnvalue)
  (Variables|/Game/Vive/Blueprints/AI/SoldierAILight/BP_LightSoldierAI.BP_LightSoldierAI_C|SetFirstStop _returnvalue FirstStopIn)
  (Variables|/Game/Vive/Blueprints/AI/SoldierAILight/BP_LightSoldierAI.BP_LightSoldierAI_C|SetAttackPos _returnvalue AttackPositionIn)
  (if (> 0 WaveCountIn)
    (goto _label)))

(fn SpawnCatapult
  (params (SpawnCountIn :type Integer) (NextCatapultIn :type BP%20Catapult%20Object%20Reference) (CatapultFirstLocationIn :type BP%20Siege%20Path%20Stops%20Object%20Reference) (CatapultSpawnPointIn :type Actor%20Object%20Reference) (CatapultAttackPositionIn :type BP%20Catapult%20Attack%20Positions%20Object%20Reference) (Soldier%20AttackPositionIn :type BP%20Soldier%20Attack%20Position%20Object%20Reference) (SoldierSpawnLocationIn :type Actor%20Object%20Reference) (SoldierFirstLocationIn :type BP%20Soldier%20Path%20Stops%20Object%20Reference))
  (Variables|Default|SetCatapultNumberOfSpawnsLeft SpawnCountIn)
  (bind _returnvalue (Game|SpawnActorfromClass "/Game/Vive/Blueprints/AI/BP_Catapult.BP_Catapult_C" (Transformation|GetActorTransform CatapultSpawnPointIn) "Undefined" 0 0 :!label _label))
  (Utilities|Array|Add (Variables|Default|GetUnitArray) _returnvalue)
  (Variables|/Game/Vive/Blueprints/AI/BP_Catapult.BP_Catapult_C|SetFinalLocation _returnvalue CatapultAttackPositionIn)
  (Variables|/Game/Vive/Blueprints/AI/BP_Catapult.BP_Catapult_C|SetFirstPos _returnvalue CatapultFirstLocationIn)
  (Variables|Default|SetTempCatapult _returnvalue)
  (if (Utilities|IsValid NextCatapultIn)
    (Variables|/Game/Vive/Blueprints/AI/BP_Catapult.BP_Catapult_C|SetNextCatapult _returnvalue NextCatapultIn))
  (bind _returnvalue_2 (Game|SpawnActorfromClass "/Game/Vive/Blueprints/AI/SoldierAILight/BP_LightSoldierAI.BP_LightSoldierAI_C" (Transformation|GetActorTransform SoldierSpawnLocationIn) "Undefined" 0 0))
  (Utilities|Array|Add (Variables|Default|GetUnitArray) _returnvalue_2)
  (Variables|/Game/Vive/Blueprints/AI/SoldierAILight/BP_LightSoldierAI.BP_LightSoldierAI_C|SetFirstStop _returnvalue_2 SoldierFirstLocationIn)
  (Variables|/Game/Vive/Blueprints/AI/SoldierAILight/BP_LightSoldierAI.BP_LightSoldierAI_C|SetAttackPos _returnvalue_2 Soldier%20AttackPositionIn)
  (bind _returnvalue_3 (Game|SpawnActorfromClass "/Game/Vive/Blueprints/AI/SoldierAILight/BP_LightSoldierAI.BP_LightSoldierAI_C" (Transformation|GetActorTransform SoldierSpawnLocationIn) "Undefined" 0 0))
  (Utilities|Array|Add (Variables|Default|GetUnitArray) _returnvalue_3)
  (Variables|/Game/Vive/Blueprints/AI/SoldierAILight/BP_LightSoldierAI.BP_LightSoldierAI_C|SetFirstStop _returnvalue_3 SoldierFirstLocationIn)
  (Variables|/Game/Vive/Blueprints/AI/SoldierAILight/BP_LightSoldierAI.BP_LightSoldierAI_C|SetAttackPos _returnvalue_3 Soldier%20AttackPositionIn)
  (bind _returnvalue_4 (Game|SpawnActorfromClass "/Game/Vive/Blueprints/AI/SoldierAILight/BP_LightSoldierAI.BP_LightSoldierAI_C" (Transformation|GetActorTransform SoldierSpawnLocationIn) "Undefined" 0 0))
  (Utilities|Array|Add (Variables|Default|GetUnitArray) _returnvalue_4)
  (Variables|/Game/Vive/Blueprints/AI/SoldierAILight/BP_LightSoldierAI.BP_LightSoldierAI_C|SetFirstStop _returnvalue_4 SoldierFirstLocationIn)
  (Variables|/Game/Vive/Blueprints/AI/SoldierAILight/BP_LightSoldierAI.BP_LightSoldierAI_C|SetAttackPos _returnvalue_4 Soldier%20AttackPositionIn)
  (bind _output_get (Variables|Default|SetCatapultNumberOfSpawnsLeft (- (Variables|Default|GetCatapultNumberOfSpawnsLeft) 1)))
  (if (< _output_get 0)
    (goto _label)
    (else
      (return))))

(fn SpawnRam
  (params (WaveCount :type Integer) (NextRam :type BP%20Battering%20Ram%20Old%20Object%20Reference) (FirstPositionIn :type BP%20Siege%20Path%20Stops%20Object%20Reference) (SpawnPointIn :type Actor%20Object%20Reference) (AttackPositionIn :type BP%20Battering%20Ram%20Attack%20Position%20Object%20Reference) (SoldierAttackPositionIn :type BP%20Soldier%20Attack%20Position%20Object%20Reference) (SoldierSpawnPointIn :type Actor%20Object%20Reference) (SoldierPathStopIn :type BP%20Soldier%20Path%20Stops%20Object%20Reference))
  (Variables|Default|SetRamNumberOfSpawnsLeft WaveCount)
  (bind _returnvalue (Game|SpawnActorfromClass "/Game/Vive/Blueprints/AI/BP_BatteringRamOld.BP_BatteringRamOld_C" (Transformation|GetActorTransform SpawnPointIn) "Undefined" 0 0 :!label _label))
  (Utilities|Array|Add (Variables|Default|GetUnitArray) _returnvalue)
  (Variables|/Game/Vive/Blueprints/AI/BP_BatteringRamOld.BP_BatteringRamOld_C|SetAttackPos _returnvalue AttackPositionIn)
  (Variables|/Game/Vive/Blueprints/AI/BP_BatteringRamOld.BP_BatteringRamOld_C|SetFirstPos _returnvalue FirstPositionIn)
  (Variables|Default|SetTempRam _returnvalue)
  (if (Utilities|IsValid NextRam)
    (Variables|/Game/Vive/Blueprints/AI/BP_BatteringRamOld.BP_BatteringRamOld_C|SetNextRam _returnvalue NextRam))
  (bind _returnvalue_2 (Game|SpawnActorfromClass "/Game/Vive/Blueprints/AI/SoldierAILight/BP_LightSoldierAI.BP_LightSoldierAI_C" (Transformation|GetActorTransform SoldierSpawnPointIn) "Undefined" 0 0))
  (Utilities|Array|Add (Variables|Default|GetUnitArray) _returnvalue_2)
  (Variables|/Game/Vive/Blueprints/AI/SoldierAILight/BP_LightSoldierAI.BP_LightSoldierAI_C|SetFirstStop _returnvalue_2 SoldierPathStopIn)
  (Variables|/Game/Vive/Blueprints/AI/SoldierAILight/BP_LightSoldierAI.BP_LightSoldierAI_C|SetAttackPos _returnvalue_2 SoldierAttackPositionIn)
  (bind _returnvalue_3 (Game|SpawnActorfromClass "/Game/Vive/Blueprints/AI/SoldierAILight/BP_LightSoldierAI.BP_LightSoldierAI_C" (Transformation|GetActorTransform SoldierSpawnPointIn) "Undefined" 0 0))
  (Utilities|Array|Add (Variables|Default|GetUnitArray) _returnvalue_3)
  (Variables|/Game/Vive/Blueprints/AI/SoldierAILight/BP_LightSoldierAI.BP_LightSoldierAI_C|SetFirstStop _returnvalue_3 SoldierPathStopIn)
  (Variables|/Game/Vive/Blueprints/AI/SoldierAILight/BP_LightSoldierAI.BP_LightSoldierAI_C|SetAttackPos _returnvalue_3 SoldierAttackPositionIn)
  (bind _returnvalue_4 (Game|SpawnActorfromClass "/Game/Vive/Blueprints/AI/SoldierAILight/BP_LightSoldierAI.BP_LightSoldierAI_C" (Transformation|GetActorTransform SoldierSpawnPointIn) "Undefined" 0 0))
  (Utilities|Array|Add (Variables|Default|GetUnitArray) _returnvalue_4)
  (Variables|/Game/Vive/Blueprints/AI/SoldierAILight/BP_LightSoldierAI.BP_LightSoldierAI_C|SetFirstStop _returnvalue_4 SoldierPathStopIn)
  (Variables|/Game/Vive/Blueprints/AI/SoldierAILight/BP_LightSoldierAI.BP_LightSoldierAI_C|SetAttackPos _returnvalue_4 SoldierAttackPositionIn)
  (bind _output_get (Variables|Default|SetRamNumberOfSpawnsLeft (- (Variables|Default|GetRamNumberOfSpawnsLeft) 1)))
  (if (< _output_get 0)
    (goto _label)
    (else
      (return))))

(fn CheckUnitCount
  (if (== (Utilities|Array|Length (Variables|Default|GetUnitArray)) 0)
    (Variables|Default|SetIsWaveComplete true)))