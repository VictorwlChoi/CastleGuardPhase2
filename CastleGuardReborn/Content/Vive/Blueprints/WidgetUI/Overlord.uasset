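; Overlord is a wave manager that spawns AI soldiers, archers, light soldiers, catapults and battering rams, giving each its route and attack positions.
; Spawned units go into UnitArray, and CheckUnitCount_0 flags the wave complete when that array is empty.
; The latest catapult or ram is held as a temporary reference and assigned to new soldiers, catapult first, until full.
; Tick loops over the units without acting on them.
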(event EventBeginPlay)

(event Collision|EventActorBeginOverlap
  (params (OtherActor :type Actor%20Object%20Reference)))

(event EventTick
  (params (DeltaSeconds :type Float%20%28single-precision%29))
  (for _array_element (Variables|Default|GetUnitArray)
    _))

(fn ConstructionScript)

(fn SpawnSoldier
  (params (SpawnPoint :type Actor%20Object%20Reference) (FirstStopIn :type BP%20Soldier%20Path%20Stops%20Object%20Reference) (AttackPositionIn :type BP%20Soldier%20Attack%20Position%20Object%20Reference))
  (bind _returnvalue (Game|SpawnActorfromClass "/Game/Vive/Blueprints/AI/SoldierAIHeavy/BP_SoldierAI.BP_SoldierAI_C" (Transformation|GetActorTransform SpawnPoint) "Undefined" 0 0))
  (Utilities|Array|Add (Variables|Default|GetUnitArray) _returnvalue)
  (Variables|/Game/Vive/Blueprints/AI/SoldierAIHeavy/BP_SoldierAI.BP_SoldierAI_C|SetFirstStop _returnvalue FirstStopIn)
  (Variables|/Game/Vive/Blueprints/AI/SoldierAIHeavy/BP_SoldierAI.BP_SoldierAI_C|SetAttackPos _returnvalue AttackPositionIn)
  (if (Utilities|IsValid (Variables|Default|GetTempCatapult))
    (bind _output_get (Variables|/Game/Vive/Blueprints/AI/SoldierAIHeavy/BP_SoldierAI.BP_SoldierAI_C|SetCatapult _returnvalue (Variables|Default|GetTempCatapult)))
    (if (Variables|/Game/Vive/Blueprints/AI/BP_Catapult.BP_Catapult_C|GetIsFull? _output_get)
      (Variables|Default|SetTempCatapult 0))
    (elif (Utilities|IsValid (Variables|Default|GetTempRam))
      (bind _output_get_2 (Variables|/Game/Vive/Blueprints/AI/SoldierAIHeavy/BP_SoldierAI.BP_SoldierAI_C|SetBatteringRam _returnvalue (Variables|Default|GetTempRam)))
      (if (Variables|/Game/Vive/Blueprints/AI/BP_BatteringRamOld.BP_BatteringRamOld_C|GetIsFull? _output_get_2)
        (Variables|Default|SetTempRam 0))))
  (return))

(fn SpawnArcher
  (params (FirstStopIn :type BP%20Archer%20Path%20Stops%20Object%20Reference) (SpawnpointIn :type Actor%20Object%20Reference) (AttackPositionIn :type BP%20Archer%20Attack%20Position%20Object%20Reference))
  (bind _returnvalue (Game|SpawnActorfromClass "/Game/Vive/Blueprints/AI/ArcherAI/BP_ArcherAi.BP_ArcherAi_C" (Transformation|GetActorTransform SpawnpointIn) "Undefined" 0 0))
  (Utilities|Array|Add (Variables|Default|GetUnitArray) _returnvalue)
  (Variables|/Game/Vive/Blueprints/AI/ArcherAI/BP_ArcherAi.BP_ArcherAi_C|SetFirstStop _returnvalue FirstStopIn)
  (Variables|/Game/Vive/Blueprints/AI/ArcherAI/BP_ArcherAi.BP_ArcherAi_C|SetAttackPosition _returnvalue AttackPositionIn)
  (return))

(fn SpawnLightSoldier
  (params (AttackPositionIn :type BP%20Soldier%20Attack%20Position%20Object%20Reference) (SpawnPointIn :type Actor%20Object%20Reference) (FirstStopIn :type BP%20Soldier%20Path%20Stops%20Object%20Reference))
  (bind _returnvalue (Game|SpawnActorfromClass "/Game/Vive/Blueprints/AI/SoldierAILight/BP_LightSoldierAI.BP_LightSoldierAI_C" (Transformation|GetActorTransform SpawnPointIn) "Undefined" 0 0))
  (Utilities|Array|Add (Variables|Default|GetUnitArray) _returnvalue)
  (Variables|/Game/Vive/Blueprints/AI/SoldierAILight/BP_LightSoldierAI.BP_LightSoldierAI_C|SetFirstStop _returnvalue FirstStopIn)
  (Variables|/Game/Vive/Blueprints/AI/SoldierAILight/BP_LightSoldierAI.BP_LightSoldierAI_C|SetAttackPos _returnvalue AttackPositionIn)
  (return))

(fn CheckUnitCount0
  (if (== (Utilities|Array|Length (Variables|Default|GetUnitArray)) 0)
    (Variables|Default|SetIsWaveComplete true)))

(fn SpawnCatapult
  (params (SpawnPointIn :type Actor%20Object%20Reference) (FirstLocationIn :type BP%20Siege%20Path%20Stops%20Object%20Reference) (AttackPositionIn :type BP%20Catapult%20Attack%20Positions%20Object%20Reference) (NextCatapultIn :type BP%20Catapult%20Object%20Reference))
  (bind _returnvalue (Game|SpawnActorfromClass "/Game/Vive/Blueprints/AI/BP_Catapult.BP_Catapult_C" (Transformation|GetActorTransform SpawnPointIn) "Undefined" 0 0))
  (Utilities|Array|Add (Variables|Default|GetUnitArray) _returnvalue)
  (Variables|/Game/Vive/Blueprints/AI/BP_Catapult.BP_Catapult_C|SetFinalLocation _returnvalue AttackPositionIn)
  (Variables|/Game/Vive/Blueprints/AI/BP_Catapult.BP_Catapult_C|SetFirstPos _returnvalue FirstLocationIn)
  (Variables|Default|SetTempCatapult _returnvalue)
  (if (Utilities|IsValid NextCatapultIn)
    (Variables|/Game/Vive/Blueprints/AI/BP_Catapult.BP_Catapult_C|SetNextCatapult _returnvalue NextCatapultIn))
  (return))

(fn SpawnRam
  (params (FirstPositionIn :type BP%20Siege%20Path%20Stops%20Object%20Reference) (SpawnPointIn :type Actor%20Object%20Reference) (AttackPositionIn :type BP%20Battering%20Ram%20Attack%20Position%20Object%20Reference) (NextRam :type BP%20Battering%20Ram%20Old%20Object%20Reference))
  (bind _returnvalue (Game|SpawnActorfromClass "/Game/Vive/Blueprints/AI/BP_BatteringRamOld.BP_BatteringRamOld_C" (Transformation|GetActorTransform SpawnPointIn) "Undefined" 0 0))
  (Utilities|Array|Add (Variables|Default|GetUnitArray) _returnvalue)
  (Variables|/Game/Vive/Blueprints/AI/BP_BatteringRamOld.BP_BatteringRamOld_C|SetAttackPos _returnvalue AttackPositionIn)
  (Variables|/Game/Vive/Blueprints/AI/BP_BatteringRamOld.BP_BatteringRamOld_C|SetFirstPos _returnvalue FirstPositionIn)
  (Variables|Default|SetTempRam _returnvalue)
  (if (Utilities|IsValid NextRam)
    (Variables|/Game/Vive/Blueprints/AI/BP_BatteringRamOld.BP_BatteringRamOld_C|SetNextRam _returnvalue NextRam))
  (return))