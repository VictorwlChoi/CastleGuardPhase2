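; BP_PlayerCollision is the VR player's hit volume, which turns AI arrow hits into damage on the Vive pawn.
; Its construction script caches the first BP_Vive_Pawn, and Tick moves the actor to just below that pawn's headset position.
; When a BP_AI_Arrows overlaps the capsule, it subtracts a fixed amount from the pawn's Health and destroys the arrow.
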(event OnComponentBeginOverlap(Capsule)
  (params (OverlappedComponent :type Primitive%20Component%20Object%20Reference) (OtherActor :type Actor%20Object%20Reference) (OtherComp :type Primitive%20Component%20Object%20Reference) (OtherBodyIndex :type Integer) (bFromSweep :type Boolean) (SweepResult :type Hit%20Result%20Structure%20%28by%20ref%29))
  (bind _asbp_ai_arrows (Utilities|Casting|CastToBP_AI_Arrows OtherActor))
  (bind _outactors (Actor|GetAllActorsOfClass "/Game/Vive/Blueprints/BP_Vive_Pawn.BP_Vive_Pawn_C"))
  (Variables|/Game/Vive/Blueprints/BP_Vive_Pawn.BP_Vive_Pawn_C|SetHealth (Utilities|Array|Get(acopy) _outactors) (- (Variables|/Game/Vive/Blueprints/BP_Vive_Pawn.BP_Vive_Pawn_C|GetHealth (Utilities|Array|Get(acopy) _outactors)) 25.0))
  (if (Utilities|IsValid _asbp_ai_arrows)
    (Actor|DestroyActor _asbp_ai_arrows)))

(event Collision|EventActorBeginOverlap
  (params (OtherActor :type Actor%20Object%20Reference)))

(event EventTick
  (params (DeltaSeconds :type Float%20%28single-precision%29))
  (bind _vive (Variables|Default|GetVive))
  (bind _headsetsceneactor (Variables|/Game/Vive/Blueprints/BP_Vive_Pawn.BP_Vive_Pawn_C|GetHeadsetSceneActor _vive))
  (if (Utilities|IsValid _headsetsceneactor)
    (Transformation|SetActorLocation (+ (Transformation|GetWorldLocation _headsetsceneactor) "0, 0,-34.000000") false false)
    (else
      (Development|PrintString "Headset Collision is Invalid"))))

(fn ConstructionScript
  (bind _outactors (Actor|GetAllActorsOfClass "/Game/Vive/Blueprints/BP_Vive_Pawn.BP_Vive_Pawn_C"))
  (Variables|Default|SetVive (Utilities|Array|Get(acopy) _outactors)))

(fn PrinttoVive
  (params (String%20In :type String))
  (Development|PrintString String%20In)
  (Development|PrintString String%20In)
  (Development|PrintString String%20In)
  (Development|PrintString String%20In)
  (Development|PrintString String%20In)
  (Development|PrintString String%20In)
  (Development|PrintString String%20In)
  (Development|PrintString String%20In)
  (Development|PrintString String%20In)
  (Development|PrintString String%20In)
  (Development|PrintString String%20In)
  (Development|PrintString String%20In)
  (Development|PrintString String%20In)
  (Development|PrintString String%20In)
  (Development|PrintString String%20In)
  (Development|PrintString String%20In))