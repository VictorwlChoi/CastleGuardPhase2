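; BP_HeavyArrow is a heavy arrow actor whose only graph logic is marked deprecated and never runs.
; That disconnected cast chain would remove soldier, light soldier or archer AI from a UnitArray, play a sound, then destroy both unit and arrow.
; Its battering ram and catapult branches would set IsOnFire, but constant false conditions block them.
; The construction script is empty.
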(fn ConstructionScript)