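; Test AI pawn that walks along a referenced spline path's points.
; From BeginPlay it chains AI Move To calls, advancing one point per success until the last.
; SwitchPaths adopts a new path and selects its nearest point by squared distance, reusing CurrentDistance0 as scratch without issuing a move.
; Older distance-along-spline movement (MoveActor, UpdateDistance) remains, marked deprecated and unused here.
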(event Custom|Update%20Distance
  (bind _pathref_0 (Variables|Default|GetPathRef_0))
  (bind _spline (Variables|/Game/Nathan/BP_SplinePath.BP_SplinePath_C|GetSpline _pathref_0))
  (bind _returnvalue (Spline|GetSplineLength _spline))
  ;[1 1 1] Update Distance - Deprecated
  (if (< (+ (Variables|Default|GetCurrentDistance_0) (Variables|Default|GetSpeed_0)) _returnvalue)
    (Variables|Default|SetCurrentDistance_0 (+ (Variables|Default|GetCurrentDistance_0) (Variables|Default|GetSpeed_0)))
    (else
      (Variables|Default|SetCurrentDistance_0 _returnvalue))))

(event Custom|SwitchPaths
  (params (NewPath :type BP%20Spline%20Path%20Object%20Reference))
  ;[1 0 0.673] Switch Paths - In Test Mode Right Now & Will Later Have An Input Parameter Of Type BP_SplinePath
  (Variables|Default|SetCurrentDistance_0 1e+16)
  (bind _output_get (Variables|Default|SetPathRef_0 NewPath))
  (for (_array_element _array_index) (Variables|/Game/Nathan/BP_SplinePath.BP_SplinePath_C|GetPoints _output_get)
    (if (< (Math|Vector|VectorLengthSquared (- _array_element (Transformation|GetActorLocation))) (Variables|Default|GetCurrentDistance_0))
      (Variables|Default|SetCurrentDistance_0 (Math|Vector|VectorLengthSquared (- _array_element (Transformation|GetActorLocation))))
      (Variables|Default|SetCurrentPoint_0 _array_index))))

(event Custom|MoveActorToNextPoint
  ;[1 0 0.8477] Move Actor To Next Point
  (AI|AIMoveTo self (Utilities|Array|Get(acopy) (Variables|/Game/Nathan/BP_SplinePath.BP_SplinePath_C|GetPoints (Variables|Default|GetPathRef_0)) (Variables|Default|GetCurrentPoint_0)) 0 5.0 false
    (:OnSuccess
      (Math|Integer|IncrementInt (Variables|Default|GetCurrentPoint_0)
        (:%20%20
          (if (not (>= (Variables|Default|GetCurrentPoint_0) (Utilities|Array|Length (Variables|/Game/Nathan/BP_SplinePath.BP_SplinePath_C|GetPoints (Variables|Default|GetPathRef_0)))))
            (CallFunction|MoveActortoNextPoint)))))))

(event EventBeginPlay
  (CallFunction|MoveActortoNextPoint))

(fn ConstructionScript)

(fn GetPathLocationOfCurrentDistance
  ;[1 1 1] Location at Path Distance
  (return (Spline|GetLocationatDistanceAlongSpline (Variables|/Game/Nathan/BP_SplinePath.BP_SplinePath_C|GetSpline (Variables|Default|GetPathRef_0)) (Variables|Default|GetCurrentDistance_0) "World")))

(fn GetPathRotationOfCurrentDistance
  ;[1 1 1] Rotation at Path Distance
  (return (Spline|GetRotationatDistanceAlongSpline (Variables|/Game/Nathan/BP_SplinePath.BP_SplinePath_C|GetSpline (Variables|Default|GetPathRef_0)) (Variables|Default|GetCurrentDistance_0) "World")))

(fn MoveActor
  (params (Actor :type Actor%20Object%20Reference))
  ;[1 1 1] Move Actor - Deprecated
  (bind _pathlocation (CallFunction|GetPathLocationOfCurrentDistance))
  (Transformation|SetActorLocation Actor _pathlocation true false)
  (bind _pathrotation (CallFunction|GetPathRotationOfCurrentDistance))
  (Transformation|SetActorRotation Actor _pathrotation)
  (CallFunction|UpdateDistance))