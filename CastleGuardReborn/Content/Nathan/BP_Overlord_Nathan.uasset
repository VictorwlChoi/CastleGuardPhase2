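; Wave director for a siege defense game: runs the between-wave countdown, refills arrow piles, plays wave sounds and returns to MainMenu after the last wave.
; Each wave reads one DataTable row per path and spawns soldiers, archers and crewed siege units at a staging area, queuing them in SpawnInfoArray.
; A delayed spawn system, optionally shuffled, teleports queued units to path starts, rotating between sides.
; A wave completes when UnitArray empties.
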(event Custom|RemoveUnit
  (params (Unit :type Ai%20Character%20Object%20Reference))
  (Utilities|Array|RemoveItem (Variables|Default|GetUnitArray) Unit))

(event Custom|PlayWaveEndSound
  (params (Index :type Integer))
  (if (< Index (Utilities|Array|Length (Variables|Default|GetWaveEndSounds)))
    (Audio|PlaySound2D self (Utilities|Array|Get(acopy) (Variables|Default|GetWaveEndSounds) Index))))

(event Custom|ResetAmountOfPaths
  (bind _wavedata (Variables|Default|GetWaveData))
  (bind _paths (Variables|Default|GetPaths))
  (bind _returnvalue (Utilities|Array|Length _wavedata))
  (bind _returnvalue_2 (Utilities|Array|Length _paths))
  (if (< _returnvalue _returnvalue_2)
    (Variables|Default|SetAmountOfPathsBeingUsed _returnvalue)
    (else
      (Variables|Default|SetAmountOfPathsBeingUsed _returnvalue_2))))

(event Custom|RemovePath
  (params (PathToRemove :type BP%20Spline%20Path%20Object%20Reference) (PathToReplace :type BP%20Spline%20Path%20Object%20Reference))
  (bind (_array_element _array_index) (Utilities|Array|ForEachLoopwithBreak (Variables|Default|GetPaths))
    (:LoopBody
      (if (== _array_element PathToRemove)
        (Utilities|Array|SetArrayElem (Variables|Default|GetPaths) _array_index PathToReplace)))))

(event Custom|ClearUnits
  (bind _unitarray (Variables|Default|GetUnitArray))
  (while (> (Utilities|Array|Length _unitarray) 0)
    (Default|Seppuku (Utilities|Array|Get(acopy) _unitarray)))
  (Utilities|Array|Clear _unitarray))

(event Custom|AddToQuivers
  (params (HeavyArrowsIncrease :type Integer) (LightArrowsIncrease :type Integer))
  (bind _outactors (Actor|GetAllActorsOfClass "/Game/Vive/Blueprints/WorldObjects/BP_HeavyArrowsPile.BP_HeavyArrowsPile_C"))
  (if (> (Utilities|Array|Length _outactors) 0)
    (Variables|/Game/Vive/Blueprints/WorldObjects/BP_HeavyArrowsPile.BP_HeavyArrowsPile_C|SetQuiverCount (Utilities|Array|Get(acopy) _outactors) (+ HeavyArrowsIncrease (Variables|/Game/Vive/Blueprints/WorldObjects/BP_HeavyArrowsPile.BP_HeavyArrowsPile_C|GetQuiverCount (Utilities|Array|Get(acopy) _outactors))))
    (Default|UpdateCountDisplay (Utilities|Array|Get(acopy) _outactors))
    (bind _outactors_2 (Actor|GetAllActorsOfClass "/Game/Vive/Blueprints/WorldObjects/BP_LightArrowsPile.BP_LightArrowsPile_C"))
    (if (> (Utilities|Array|Length _outactors_2) 0)
      (Variables|/Game/Vive/Blueprints/WorldObjects/BP_LightArrowsPile.BP_LightArrowsPile_C|SetQuiverCount (Utilities|Array|Get(acopy) _outactors_2) (+ LightArrowsIncrease (Variables|/Game/Vive/Blueprints/WorldObjects/BP_LightArrowsPile.BP_LightArrowsPile_C|GetQuiverCount (Utilities|Array|Get(acopy) _outactors_2))))
      (Default|UpdateCountDisplay (Utilities|Array|Get(acopy) _outactors_2))
      (else
        (Development|PrintString "No Light Arrow Pile")))
    (else
      (Development|PrintString "No Heavy Arrow Pile"))))

(event Custom|SetWaveTimerText
  (bind _outactors (Actor|GetAllActorsOfClass "/Game/Vive/Blueprints/WorldObjects/BP_WaveTimer.BP_WaveTimer_C"))
  (if (> (Utilities|Array|Length _outactors) 0)
    (Rendering|Components|TextRender|SetText (Variables|/Game/Vive/Blueprints/WorldObjects/BP_WaveTimer.BP_WaveTimer_C|GetTextRender (Utilities|Array|Get(acopy) _outactors)) (Utilities|Text|ToText(Integer) (- (Variables|Default|GetSecondsBetweenNextWave) (Math|Float|Truncate (Variables|Default|GetWaveTimer)))))
    (else
      (Development|PrintString "No Wave Timer in Map"))))

(event Custom|ChangeWaveTimerVisibility
  (params (Visibility :type Boolean))
  (bind _outactors (Actor|GetAllActorsOfClass "/Game/Vive/Blueprints/WorldObjects/BP_WaveTimer.BP_WaveTimer_C"))
  (if (> (Utilities|Array|Length _outactors) 0)
    (Rendering|SetVisibility (Variables|/Game/Vive/Blueprints/WorldObjects/BP_WaveTimer.BP_WaveTimer_C|GetTextRender (Utilities|Array|Get(acopy) _outactors)) Visibility false)
    (else
      (Development|PrintString "No Wave Timer in Map"))))

(event Custom|PlayWaveStartSound
  (params (Index :type Integer))
  (if (< Index (Utilities|Array|Length (Variables|Default|GetWaveStartSounds)))
    (Audio|PlaySound2D self (Utilities|Array|Get(acopy) (Variables|Default|GetWaveStartSounds) Index))))

(event EventTick
  (params (DeltaSeconds :type Float%20%28single-precision%29))
  (if (not (Variables|Default|GetbGameIsOver))
    (if true
      (CallFunction|SpawnSystem DeltaSeconds)
      (CallFunction|SetWaveTimerText)
      (if (Variables|Default|GetIsWaveComplete)
        (if (< (Variables|Default|GetCurrentWave) (Utilities|Array|Length (Variables|Default|GetWaveEndSounds)))
          (CallFunction|ChangeWaveTimerVisibility true)
          (bind _output_get (Variables|Default|SetWaveTimer (+ DeltaSeconds (Variables|Default|GetWaveTimer))))
          (if (>= _output_get (Math|Conversions|ToFloat(Integer) (Variables|Default|GetSecondsBetweenNextWave)))
            (CallFunction|ChangeWaveTimerVisibility false)
            (if (Variables|Default|GetbCanTickAgain)
              (Variables|Default|SetbCanTickAgain false)
              (Variables|Default|SetSpawnSystemTimer 0.0)
              (bind _output_get_2 (Variables|Default|SetCurrentWave (+ (Variables|Default|GetCurrentWave) 1)))
              (CallFunction|PlayWaveStartSound _output_get_2)
              (for (_array_element _array_index) (Variables|Default|GetWaveData)
                (bind _outrownames (DataTable|GetDataTableRowNames _array_element))
                (bind _output_get_3 (Variables|Default|SetWaveNames _outrownames))
                (bind _returnvalue (Utilities|GetDataTableRow _array_element (Utilities|Array|Get(acopy) _output_get_3 (Variables|Default|GetCurrentWave)))
                  (:then
                    (if (== _array_index 0)
                      (Variables|Default|SetSecondsBetweenNextWave (.SecondsBetweenNextWave (Utilities|Struct|BreakS_WaveInfo _returnvalue)))
                      ;[1 1 1] SpawnCatapult1
                      (CallFunction|AddtoQuivers (.HeavyArrowCountIncrease (Utilities|Struct|BreakS_WaveInfo _returnvalue)) (.LightArrowCountIncrease (Utilities|Struct|BreakS_WaveInfo _returnvalue))))
                    (if (!= (.CatapultCount (Utilities|Struct|BreakS_WaveInfo _returnvalue)) 0)
                      (Variables|Default|SetIsWaveComplete false)
                      (CallFunction|SpawnCatapultUnit (.CatapultCount (Utilities|Struct|BreakS_WaveInfo _returnvalue)) (Variables|Default|GetTempCatapult) _array_index))
                    ;[1 1 1] SpawnRam1
                    (if (!= (.BatteringRamCount (Utilities|Struct|BreakS_WaveInfo _returnvalue)) 0)
                      (Variables|Default|SetIsWaveComplete false)
                      (CallFunction|SpawnRamUnit (.BatteringRamCount (Utilities|Struct|BreakS_WaveInfo _returnvalue)) (Variables|Default|GetTempRam) _array_index))
                    ;[1 1 1] SpawnLightSoldier1
                    (if (!= (.LightSoldierCount (Utilities|Struct|BreakS_WaveInfo _returnvalue)) 0)
                      (Variables|Default|SetIsWaveComplete false)
                      (CallFunction|SpawnLightSoldierUnit (.LightSoldierCount (Utilities|Struct|BreakS_WaveInfo _returnvalue)) _array_index))
                    ;[1 1 1] Reserve Space (MediumSoldier1)
                    (if (!= (.MediumSoldierCount (Utilities|Struct|BreakS_WaveInfo _returnvalue)) 0)
                      (Variables|Default|SetIsWaveComplete false)
                      (CallFunction|SpawnMediumSoldier (.MediumSoldierCount (Utilities|Struct|BreakS_WaveInfo _returnvalue)) _array_index))
                    ;[1 1 1] SpawnHeavySoldier1
                    (if (!= (.HeavySoldierCount (Utilities|Struct|BreakS_WaveInfo _returnvalue)) 0)
                      (Variables|Default|SetIsWaveComplete false)
                      (CallFunction|SpawnHeavySoldierUnit (.HeavySoldierCount (Utilities|Struct|BreakS_WaveInfo _returnvalue)) _array_index))
                    ;[1 1 1] SpawnArcher1
                    (if (!= (.ArcherCount (Utilities|Struct|BreakS_WaveInfo _returnvalue)) 0)
                      (Variables|Default|SetIsWaveComplete false)
                      (CallFunction|SpawnArcherUnit (.ArcherCount (Utilities|Struct|BreakS_WaveInfo _returnvalue)) _array_index))
                    (Variables|Default|SetbCanTickAgain true))))))
          (else
            (Variables|Default|SetEndTimer (+ DeltaSeconds (Variables|Default|GetEndTimer)))
            (if (>= (Variables|Default|GetEndTimer) (Variables|Default|GetEndTimerMax))
              (Game|OpenLevel(byName) "MainMenu"))))
        (elif (== (Utilities|Array|Length (Variables|Default|GetUnitArray)) 0)
          (Variables|Default|SetIsWaveComplete true)
          (Variables|Default|SetWaveTimer 0.0)
          (CallFunction|PlayWaveEndSound (Variables|Default|GetCurrentWave))
          (if (>= (Variables|Default|GetCurrentWave) (Utilities|Array|Length (Variables|Default|GetWaveEndSounds)))
            (Audio|PlaySound2D (Variables|Default|GetEndGameSound))))))))

(event EventBeginPlay
  (for _array_element (Variables|Default|GetWaves)
    (Utilities|Array|Add (Variables|Default|GetWaveData) (.WaveData (Utilities|Struct|BreakS_Wave _array_element)))
    (Utilities|Array|Add (Variables|Default|GetPaths) (.WavePath (Utilities|Struct|BreakS_Wave _array_element))))
  (CallFunction|ResetAmountOfPaths))

(event Custom|SpawnLightSoldierUnit
  (params (WaveCountIn :type Integer) (SpawnSide :type Integer))
  ;[1 1 1] Spawn light Soldier Unit - Done with the new system
  (Variables|Default|SetLightSoldierNumberOfSpawnsLeft WaveCountIn)
  (bind _returnvalue (Game|SpawnActorfromClass "/Game/Vive/Blueprints/AI/SoldierAI/SoldierAILight/BP_LightSoldierAI.BP_LightSoldierAI_C" (Variables|Default|GetStartingArea) "AlwaysSpawn" 0 0 :!label _label))
  (CallFunction|AddtoSpawnInfoArray SpawnSide _returnvalue (Utilities|Array|MakeArray))
  (Utilities|Array|Add (Variables|Default|GetUnitArray) _returnvalue)
  (Variables|Default|SetLightSoldierNumberOfSpawnsLeft (- (Variables|Default|GetLightSoldierNumberOfSpawnsLeft) 1))
  (if (> (Variables|Default|GetLightSoldierNumberOfSpawnsLeft) 0)
    (goto _label)))

(event Custom|SpawnSystem
  (params (DeltaTime :type Float%20%28single-precision%29))
  (bind _spawninfoarray (Variables|Default|GetSpawnInfoArray))
  ;[1 0 0.6645] SpawnSystem - Does all the logic for choosing enemy spawning
  (if (> (Variables|Default|GetSpawnSystemTimer) (Variables|Default|GetSpawnSystemStartDelay))
    (if (> (Utilities|Array|Length _spawninfoarray) 0)
      (Utilities|FlowControl|Delay (Variables|Default|GetSpawnDelay))
      (CallFunction|PickEnemytoMove "NewEnumerator6"))
    (else
      (Variables|Default|SetSpawnSystemTimer (+ DeltaTime (Variables|Default|GetSpawnSystemTimer)))
      (if (Variables|Default|GetUseRandomSpawning)
        (Utilities|Array|Shuffle _spawninfoarray)))))

(event Custom|SpawnHeavySoldierUnit
  (params (WaveCountIn :type Integer) (SpawnSide :type Integer))
  ;[1 1 1] Spawn Heavy Soldier - Done with the new system
  (Variables|Default|SetHeavySoldierNumberOfSpawnsLeft WaveCountIn)
  (bind _returnvalue (Game|SpawnActorfromClass "/Game/Vive/Blueprints/AI/SoldierAI/BP_SoldierAI.BP_SoldierAI_C" (Variables|Default|GetStartingArea) "AlwaysSpawn" 0 0 :!label _label))
  (CallFunction|AddtoSpawnInfoArray SpawnSide _returnvalue (Utilities|Array|MakeArray))
  (Utilities|Array|Add (Variables|Default|GetUnitArray) _returnvalue)
  (bind _output_get (Variables|Default|SetHeavySoldierNumberOfSpawnsLeft (- (Variables|Default|GetHeavySoldierNumberOfSpawnsLeft) 1)))
  (if (> _output_get 0)
    (goto _label)))

(event Custom|MoveLeftOverEnemy
  (bind _spawninfoarray (Variables|Default|GetSpawnInfoArray))
  ;[1 0 0.768] MoveLeftOverEnemy - Called when pick enemy to move doesn't get a valid ai input
  (if (> (Utilities|Array|Length (Variables|Default|GetSpawnInfoArray)) 0)
    (CallFunction|MoveEnemy (Utilities|Array|Get(acopy) _spawninfoarray))
    (Utilities|Array|RemoveIndex _spawninfoarray)))

(event Custom|SpawnArcherUnit
  (params (WaveCountIn :type Integer) (SpawnSide :type Integer))
  ;[1 1 1] Spawn Archer Unit - Done with the new System
  (Variables|Default|SetArcherNumberOfSpawnsLeft WaveCountIn)
  (bind _returnvalue (Game|SpawnActorfromClass "/Game/Vive/Blueprints/AI/ArcherAI/BP_ArcherAi.BP_ArcherAi_C" (Variables|Default|GetStartingArea) "AlwaysSpawn" 0 0 :!label _label))
  (Utilities|Array|Add (Variables|Default|GetUnitArray) _returnvalue)
  (CallFunction|AddtoSpawnInfoArray SpawnSide _returnvalue (Utilities|Array|MakeArray))
  (Variables|Default|SetArcherNumberOfSpawnsLeft (- (Variables|Default|GetArcherNumberOfSpawnsLeft) 1))
  (if (> (Variables|Default|GetArcherNumberOfSpawnsLeft) 0)
    (goto _label)))

(event Custom|MoveEnemy
  (params (Spawn%20Info :type S%20Spawn%20Info%20Structure))
  (bind (_pathindex _actortomove _childrentomove) (Utilities|Struct|BreakS_SpawnInfo Spawn%20Info))
  ;[1 0 0.9199] MoveEnemy - Move the enemy to its starting path point
  (bind (_worldlocation _direction) (CallFunction|GetFirstPointTransformOfPath _pathindex))
  (Transformation|SetActorTransform _actortomove (Math|Conversions|ToTransform(Vector) (Math|Vector|MakeVector (.X (Math|Vector|BreakVector _worldlocation)) (.Y (Math|Vector|BreakVector _worldlocation)) (+ (.Z (Math|Vector|BreakVector _worldlocation)) (Variables|Default|GetSpawnHeightOffset)))) false true)
  (bind _asai_character (Utilities|Casting|CastToAiCharacter _actortomove))
  (Default|Initialize _asai_character (Utilities|Array|Get(acopy) (Variables|Default|GetPaths) _pathindex))
  (for (_array_element _array_index) _childrentomove
    (bind _spawnlocation (CallFunction|GetSiegeOperatorRelativeSpawnLocation (Math|Vector|MakeVector (.X (Math|Vector|BreakVector _worldlocation)) (.Y (Math|Vector|BreakVector _worldlocation)) (+ (.Z (Math|Vector|BreakVector _worldlocation)) (Variables|Default|GetSpawnHeightOffset))) _array_index _direction))
    (Transformation|SetActorTransform _array_element (Math|Conversions|ToTransform(Vector) (Math|Vector|MakeVector (.X (Math|Vector|BreakVector _worldlocation)) (.Y (Math|Vector|BreakVector _worldlocation)) (+ (.Z (Math|Vector|BreakVector _worldlocation)) (Variables|Default|GetSpawnHeightOffset)))) false true)
    (bind _asai_character_2 (Utilities|Casting|CastToAiCharacter _array_element))
    (Default|Initialize _asai_character_2 (Utilities|Array|Get(acopy) (Variables|Default|GetPaths) _pathindex))))

(event Custom|PickEnemyToMove
  (params (Enemy%20Type :type EnemyType%20Enum :default "NewEnumerator6"))
  (bind _spawninfoarray (Variables|Default|GetSpawnInfoArray))
  ;[1 0 0.8136] PickEnemyToMove - This event does the logic to determine which enemy from the spawninfo list should be moved to their path start. If None the type doesnt matter
  (bind (_array_element _array_index) (Utilities|Array|ForEachLoopwithBreak _spawninfoarray :!label _label)
    (:LoopBody
      (if (and (== (.PathIndex (Utilities|Struct|BreakS_SpawnInfo _array_element)) (Variables|Default|GetCurrentSide)) (Math|Conversions|ToBoolean(Integer) (Class|KismetMathLibrary|OrIntInt (Math|Conversions|ToInteger(Boolean) (Utilities|Enum|Equal(Enum) (.EnemyType (Utilities|Struct|BreakS_SpawnInfo _array_element)) Enemy%20Type)) (Math|Conversions|ToInteger(Boolean) (Utilities|Enum|Equal(Enum) Enemy%20Type "NewEnumerator6")))))
        (Variables|Default|SetEnemyMoveIndex _array_index)
        (CallFunction|MoveEnemy _array_element)
        (goto _label Break)))
    (:Completed
      (if (!= (Variables|Default|GetEnemyMoveIndex) -1)
        (Utilities|Array|RemoveIndex _spawninfoarray (Variables|Default|GetEnemyMoveIndex))
        (Variables|Default|SetEnemyMoveIndex -1)
        (CallFunction|AdvanceCurrentSideCounter)
        (else
          (CallFunction|MoveLeftOverEnemy))))))

(event Custom|SpawnMediumSoldier
  (params (WaveCountIn :type Integer) (SpawnSide :type Integer))
  ;[1 1 1] Spawn light Soldier Unit - Done with the new system
  (Variables|Default|SetLightSoldierNumberOfSpawnsLeft WaveCountIn)
  (bind _returnvalue (Game|SpawnActorfromClass "/Game/Vive/Blueprints/AI/SoldierAI/SoldierAILight/BP_LightSoldierAI.BP_LightSoldierAI_C" (Variables|Default|GetStartingArea) "AlwaysSpawn" 0 0 :!label _label))
  (Default|SetupShield _returnvalue)
  (CallFunction|AddtoSpawnInfoArray SpawnSide _returnvalue (Utilities|Array|MakeArray))
  (Utilities|Array|Add (Variables|Default|GetUnitArray) _returnvalue)
  (Variables|Default|SetLightSoldierNumberOfSpawnsLeft (- (Variables|Default|GetLightSoldierNumberOfSpawnsLeft) 1))
  (if (> (Variables|Default|GetLightSoldierNumberOfSpawnsLeft) 0)
    (goto _label)))

(event Custom|AdvanceCurrentSideCounter
  ;[1 0 0.7437] AdvanceCurrentSideCounter - This event cycles through the current side to spawn an enemy on
  (bind _output_get (Variables|Default|SetCurrentSide (+ (Variables|Default|GetCurrentSide) 1)))
  (if (>= _output_get (Variables|Default|GetAmountOfPathsBeingUsed))
    (Variables|Default|SetCurrentSide 0)))

(event Custom|Add%20To%20Spawn%20Info%20Array
  (params (Spawn%20Side :type Integer) (Actor%20To%20Move :type Actor%20Object%20Reference) (Children%20Of%20Actor :type Array%20of%20Actor%20Object%20References))
  ;[1 0 0.7779] AddToSpawnInfoArray - Adds a spawninfo element to the array SpawnInfo
  (bind _asai_character (Utilities|Casting|CastToAiCharacter Actor%20To%20Move))
  (Utilities|Array|Add (Variables|Default|GetSpawnInfoArray) (Utilities|Struct|MakeS_SpawnInfo Spawn%20Side Actor%20To%20Move Children%20Of%20Actor (Variables|/Game/Vive/Blueprints/AI/AiCharacter.AiCharacter_C|GetEnemyType _asai_character))))

(event Custom|SpawnCatapultUnit
  (params (WaveCountIn :type Integer) (NextCatapultIn :type BP%20Catapult%20Object%20Reference) (SpawnSide :type Integer))
  ;[1 1 1] Spawn Catapult and Soldier to man it
  (Variables|Default|SetCatapultNumberOfSpawnsLeft WaveCountIn)
  (bind _returnvalue (Game|SpawnActorfromClass "/Game/Vive/Blueprints/AI/SiegeAI/BP_Catapult.BP_Catapult_C" (Variables|Default|GetStartingArea) "AlwaysSpawn" 0 0 :!label _label))
  (Utilities|Array|Add (Variables|Default|GetUnitArray) _returnvalue)
  (Variables|Default|SetTempCatapult _returnvalue)
  (if (Utilities|IsValid NextCatapultIn)
    _
    (else
      _))
  (bind _returnvalue_2 (Game|SpawnActorfromClass "/Game/Vive/Blueprints/AI/SoldierAI/BP_SoldierAI.BP_SoldierAI_C" (Variables|Default|GetStartingArea) "AlwaysSpawn" 0 0))
  (Utilities|Array|Add (Variables|Default|GetUnitArray) _returnvalue_2)
  (bind _returnvalue_3 (Game|SpawnActorfromClass "/Game/Vive/Blueprints/AI/SoldierAI/BP_SoldierAI.BP_SoldierAI_C" (Variables|Default|GetStartingArea) "AlwaysSpawn" 0 0))
  (Utilities|Array|Add (Variables|Default|GetUnitArray) _returnvalue_3)
  (CallFunction|AddtoSpawnInfoArray SpawnSide _returnvalue (Utilities|Array|MakeArray _returnvalue_2 _returnvalue_3))
  (bind _output_get (Variables|Default|SetCatapultNumberOfSpawnsLeft (- (Variables|Default|GetCatapultNumberOfSpawnsLeft) 1)))
  (if (> _output_get 0)
    (goto _label)))

(event Custom|SpawnRamUnit
  (params (WaveCountIn :type Integer) (NextRamIn :type BP%20Battering%20Ram%20Old%20Object%20Reference) (SpawnSide :type Integer))
  ;[1 1 1] Spawn Ram and Soldiers to Man it - Done with the new System
  (Variables|Default|SetRamNumberOfSpawnsLeft WaveCountIn)
  (bind _returnvalue (Game|SpawnActorfromClass "/Game/Vive/Blueprints/AI/SiegeAI/BP_BatteringRamOld.BP_BatteringRamOld_C" (Variables|Default|GetStartingArea) "AlwaysSpawn" 0 0 :!label _label))
  (Utilities|Array|Add (Variables|Default|GetUnitArray) _returnvalue)
  (if (Utilities|IsValid NextRamIn)
    _
    (else
      _))
  (bind _returnvalue_2 (Game|SpawnActorfromClass "/Game/Vive/Blueprints/AI/SoldierAI/BP_SoldierAI.BP_SoldierAI_C" (Variables|Default|GetStartingArea) "AlwaysSpawn" 0 0))
  (Utilities|Array|Add (Variables|Default|GetUnitArray) _returnvalue_2)
  (bind _returnvalue_3 (Game|SpawnActorfromClass "/Game/Vive/Blueprints/AI/SoldierAI/BP_SoldierAI.BP_SoldierAI_C" (Variables|Default|GetStartingArea) "AlwaysSpawn" 0 0))
  (Utilities|Array|Add (Variables|Default|GetUnitArray) _returnvalue_3)
  (CallFunction|AddtoSpawnInfoArray SpawnSide _returnvalue (Utilities|Array|MakeArray _returnvalue_2 _returnvalue_3))
  (bind _output_get (Variables|Default|SetRamNumberOfSpawnsLeft (- (Variables|Default|GetRamNumberOfSpawnsLeft) 1)))
  (if (> _output_get 0)
    (goto _label)))

(fn ConstructionScript)

(fn CheckUnitCount
  (if (== (Utilities|Array|Length (Variables|Default|GetUnitArray)) 0)
    (Variables|Default|SetIsWaveComplete true)))

(fn EnemyTypetoSpawnSide
  (params (Enemy%20Type :type EnemyType%20Enum :default "NewEnumerator6") (Spawn%20Side :type SpawnSide%20Enum :default "NewEnumerator4"))
  ;[1 0 0.9426] EnemyTypeToSpawnSide - Converts EnemyType and SpawnSide enums to their respective spawn location actors
  (switch Utilities|FlowControl|Switch|SwitchonEnemyType Enemy%20Type
    (:NewEnumerator0
      _)
    (:NewEnumerator1
      (switch Utilities|FlowControl|Switch|SwitchonSpawnSide Spawn%20Side
        (:NewEnumerator0
          (return 0))
        (:NewEnumerator1
          (return 0))
        (:NewEnumerator2
          (return 0))
        (:NewEnumerator3
          (return 0))))
    (:NewEnumerator2
      _)
    (:NewEnumerator4
      (switch Utilities|FlowControl|Switch|SwitchonSpawnSide Spawn%20Side :!label _label
        (:NewEnumerator0
          (return 0))
        (:NewEnumerator1
          (return 0))
        (:NewEnumerator2
          (return 0))
        (:NewEnumerator3
          (return 0))))
    (:NewEnumerator5
      (goto _label)))
  (switch Utilities|FlowControl|Switch|SwitchonSpawnSide Spawn%20Side
    (:NewEnumerator0
      (return 0))
    (:NewEnumerator1
      (return 0))
    (:NewEnumerator2
      (return 0))
    (:NewEnumerator3
      (return 0))))

(fn GetFirstPointTransformOfPath
  (params (Index :type Integer))
  (bind _paths (Variables|Default|GetPaths))
  (bind _output (Utilities|Array|Get(acopy) _paths Index))
  (bind _points (Variables|/Game/Nathan/BP_SplinePath.BP_SplinePath_C|GetPoints _output))
  (bind _output_2 (Utilities|Array|Get(acopy) _points))
  (if (< Index (Utilities|Array|Length _paths))
    (return _output_2 (Math|Vector|Normalize (- (Utilities|Array|Get(acopy) _points 1) _output_2)))
    (else
      (Development|PrintString "Overlord::Invalid Index")
      (return "0, 0, 0" "0, 0, 0"))))

(fn GetSiegeOperatorRelativeSpawnLocation
  (params (WorldLocation :type Vector) (OperatorNumber :type Integer) (UnitMovementDirection :type Vector))
  (return (+ WorldLocation (* UnitMovementDirection (* (+ OperatorNumber 1) (* (LocalVariables|GetSpaceCushion) -1.0))))))