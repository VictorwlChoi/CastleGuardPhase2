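; BP_PathEvent is an event actor that, when activated, closes a spline path and reroutes the AI units on it.
; It stops the path spawning enemies, then switches units not yet past its sphere to a redirect spline.
; Progress is compared by distance along the spline, interpolated between points from the closest input key.
; The construction script finds the Overlord, which supplies the unit list and removes the closed path.
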(event Custom|Activate
  ;[1 1 1] Stop Path From Spawning New Enemies
  (Variables|/Game/Nathan/BP_SplinePath.BP_SplinePath_C|SetSpawnEnemiesHere (Variables|Default|GetSplinePath) false)
  ;[1 1 1] Check Which Units Need To Be Alerted
  (for _array_element (Variables|/Game/Nathan/BP_Overlord_Nathan.BP_Overlord_Nathan_C|GetUnitArray (Variables|Default|GetOverlordRef))
    (bind _asai_character (Utilities|Casting|CastToAiCharacter _array_element))
    ;[1 1 1] Is the AI on the path that caused the event
    (if (== (Variables|/Game/Vive/Blueprints/AI/AiCharacter.AiCharacter_C|GetPathRef _asai_character) (Variables|Default|GetSplinePath))
      ;[1 1 1] Check If the AI is not already past the event location
      (bind _distance (CallFunction|FindDistanceAlongSplineClosesttoWorldLocation (Variables|Default|GetSplinePath) (Transformation|GetWorldLocation (Variables|Default|GetSphere))))
      (bind _distance_2 (CallFunction|FindDistanceAlongSplineClosesttoWorldLocation (Variables|Default|GetSplinePath) (Transformation|GetActorLocation _array_element)))
      (if (< _distance_2 _distance)
        (Default|SwitchPaths _asai_character (Variables|Default|GetSplinePathToRedirectUnitsTo)))))
  (Default|RemovePath (Variables|Default|GetOverlordRef) (Variables|Default|GetSplinePath)))

(fn ConstructionScript
  (bind _outactors (Actor|GetAllActorsOfClass "/Game/Nathan/BP_Overlord_Nathan.BP_Overlord_Nathan_C"))
  (if (> (Utilities|Array|Length _outactors) 0)
    (Variables|Default|SetOverlordRef (Utilities|Array|Get(acopy) _outactors))
    (else
      (Development|PrintString "PathEvent::No Overlord In Scene"))))

(fn FindDistanceAlongSplineClosesttoWorldLocation
  (params (Spline :type BP%20Spline%20Path%20Object%20Reference) (WorldLocation :type Vector))
  (bind _returnvalue (Class|SplineComponent|FindInputKeyClosesttoWorldLocation (Variables|/Game/Nathan/BP_SplinePath.BP_SplinePath_C|GetSpline Spline) WorldLocation))
  (bind _returnvalue_2 (Math|Float|Truncate _returnvalue))
  (bind _returnvalue_3 (Spline|GetDistanceAlongSplineatSplinePoint (Variables|/Game/Nathan/BP_SplinePath.BP_SplinePath_C|GetSpline Spline) _returnvalue_2))
  (return (+ _returnvalue_3 (* (- (Spline|GetDistanceAlongSplineatSplinePoint (Variables|/Game/Nathan/BP_SplinePath.BP_SplinePath_C|GetSpline Spline) (Math|Float|Truncate (+ _returnvalue 1.0))) _returnvalue_3) (- _returnvalue (Math|Conversions|ToFloat(Integer) _returnvalue_2))))))