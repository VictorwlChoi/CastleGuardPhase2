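; BP_SplinePath is a path actor that converts its Spline component into an array of world-space Points.
; SetupPoints runs from the construction script, clearing the array and sampling the spline at DistancePiece intervals, then appending the spline's end location.
; BeginPlay only prints a warning if Points is empty.
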(event Custom|SetupPoints
  (bind _spline (Variables|Default|GetSpline))
  (Utilities|Array|Clear (Variables|Default|GetPoints))
  (for _index (range 0 (Math|Float|Truncate (/ (Spline|GetSplineLength (Variables|Default|GetSpline)) (Variables|Default|GetDistancePiece))))
    (Utilities|Array|Add (Variables|Default|GetPoints) (Spline|GetLocationatDistanceAlongSpline (Variables|Default|GetSpline) (* _index (Variables|Default|GetDistancePiece)) "World")))
  (Utilities|Array|Add (Variables|Default|GetPoints) (Spline|GetLocationatDistanceAlongSpline _spline (Spline|GetSplineLength _spline) "World")))

(event EventBeginPlay
  (if (== (Utilities|Array|Length (Variables|Default|GetPoints)) 0)
    (Development|PrintString "SETUP POINTS!!!!!")))

(event Collision|EventActorBeginOverlap
  (params (OtherActor :type Actor%20Object%20Reference)))

(fn ConstructionScript
  (CallFunction|SetupPoints))